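; Player fighter aircraft for Player One or Two on a twin rig, with blasters, boost, brake and barrel rolls.
; Axis inputs move and tilt it within depth-scaled limits, with rolls modifying horizontal speed.
; Looping timers fire projectiles through an input gate and run a 60 Hz pulse for energy, depth recentering, ailerons, reticles and HUD.
; InitializeAircraft sets up per-player stats, color, HUD, offsets and hull hitpoints.
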(event Custom|InitializeAircraft
  (bind _twinaircraftrig (Variables|Core|GetTwinAircraftRig))
  (bind _distancefromcentre (Variables|/Game/Gameplay/Blueprints/BP_TwinAircraftRig.BP_TwinAircraftRig_C|GetDistanceFromCentre _twinaircraftrig))
  ;[1 1 1] Initialize Aircraft at the start of the level from the game mode
  (CallFunction|StartPulse)
  (Utilities|FlowControl|Sequence
    (:then_0
      ;[1 1 1] Create HUD for Aircraft and Populate with data
      (switch Utilities|FlowControl|Switch|SwitchonENUM_PlayerNumber (Variables|Core|GetPlayer)
        (:NewEnumerator0
          (Variables|Core|SetAircraftData (Utilities|Struct|MakeSTRUCT_AicraftData 20 20 3 12 (Utilities|Struct|MakeSlateColor "(R=0.106985,G=0.655000,B=0.000000,A=1.000000)"))))
        (:NewEnumerator1
          (Variables|Core|SetAircraftData (Utilities|Struct|MakeSTRUCT_AicraftData 9 15 4 6 (Utilities|Struct|MakeSlateColor "(R=0.825000,G=0.600217,B=0.000000,A=1.000000)")))))
      (bind _returnvalue (UserInterface|CreateWidget "/Game/Players/Widgets/WID_AircraftHUD.WID_AircraftHUD_C"))
      (Default|InitializeAircraftHUD _returnvalue (Variables|Core|GetPlayer) (Variables|Core|GetAircraftData))
      (bind _output_get (Variables|Core|SetAircraftHUD _returnvalue))
      (UserInterface|Viewport|AddtoViewport _output_get 0))
    (:then_1
      ;[1 1 1] Get the offset amount from the Twin Rig for horizontal movement
      (switch Utilities|FlowControl|Switch|SwitchonENUM_PlayerNumber (Variables|Core|GetPlayer)
        (:NewEnumerator0
          (Variables|HorizontalMovement|SetHorizontalOffsetMax (* _distancefromcentre 2.0))
          (Variables|HorizontalMovement|SetHorizontalOffsetMin 0.0))
        (:NewEnumerator1
          (Variables|HorizontalMovement|SetHorizontalOffsetMin (* _distancefromcentre -2.0))
          (Variables|HorizontalMovement|SetHorizontalOffsetMax 0.0))))
    (:then_2
      ;[1 1 1] Set Aircraft Color
      (CallFunction|SetAircraftColor))
    (:then_3
      ;[1 1 1] Set Energy Bar to Full
      (Variables|Health|SetCurrentHealth (.TotalNumberOfHitPoints (Utilities|Struct|BreakSTRUCT_AicraftData (Variables|Core|GetAircraftData))))
      (Variables|Energy|SetCurrentEnergyAmount (Math|Conversions|ToFloat(Integer) (.TotalNumberOfEnergyTanks (Utilities|Struct|BreakSTRUCT_AicraftData (Variables|Core|GetAircraftData))))))
    (:then_4
      ;[1 1 1] Set total hitpoints on the Hull Component and set it as player owned
      (bind _asbp_hull_component_player (Utilities|Casting|CastToBP_HullComponentPlayer (Variables|/Script/Engine.ChildActorComponent|GetChildActor (Variables|Default|GetHullComponent))))
      (Default|SetPlayerComponentHitpoints _asbp_hull_component_player (.TotalNumberOfHitPoints (Utilities|Struct|BreakSTRUCT_AicraftData (Variables|Core|GetAircraftData)))))))

(event Custom|StartPulse
  ;[1 1 1] Tick Pulse
  (bind _returnvalue (Utilities|Time|SetTimerbyEvent (delegate Custom|Pulse) (/ 1.0 6e+01) true))
  (Variables|Energy|SetBoostRechargeTimer _returnvalue))

(event Custom|Pulse
  (bind _maxboostposition (Variables|Boosting|GetMaxBoostPosition))
  (bind _maxbrakeposition (Variables|Braking|GetMaxBrakePosition))
  ;[1 1 1] Tick Pulse
  (Utilities|FlowControl|Sequence
    (:then_0
      ;[1 1 1] Set the current hit points on the UI
      (bind _asbp_hull_component (Utilities|Casting|CastToBP_HullComponent (Variables|/Script/Engine.ChildActorComponent|GetChildActor (Variables|Default|GetHullComponent))))
      (Default|UpdateHitPointBar (Variables|Core|GetAircraftHUD) (Variables|/Game/Units/Blueprints/BP_HullComponent.BP_HullComponent_C|GetCurrentHitpoints _asbp_hull_component)))
    (:then_1
      ;[1 1 1] Charge Energy Bar
      (Utilities|FlowControl|Sequence
        (:then_0
          (if (Variables|Energy|GetEnergyAvailable)
            (goto _label Open)
            (else
              (goto _label Close))))
        (:then_1
          (Utilities|FlowControl|Gate false :!label _label
            (:Exit
              (Math|Float|CompareFloat (Variables|Energy|GetCurrentEnergyAmount) 0.0
                (:>
                  _)
                (:==
                  _)
                (:<
                  (Variables|Energy|SetEnergyAvailable false)
                  (Variables|Boosting|SetBoosting false)
                  (Variables|Energy|SetBraking false)
                  (Utilities|FlowControl|Delay 1.0)
                  (Variables|Energy|SetEnergyAvailable true)))
              (bind _output_get (Variables|Energy|SetCurrentEnergyAmount (Math|Float|Clamp(Float) (+ (Variables|Energy|GetCurrentEnergyAmount) 0.06) -0.5 (Math|Conversions|ToFloat(Integer) (Utilities|Struct|BreakSTRUCT_AicraftData (Variables|Core|GetAircraftData))))))
              (Default|UpdateEnergyBar (Variables|Core|GetAircraftHUD) _output_get))))))
    (:then_2
      ;[1 1 1] Adjust the Ailerons
      (CallFunction|PivotAilerons))
    (:then_3
      ;[1 1 1] Boost Brake
      (Utilities|FlowControl|Sequence
        (:then_0
          (if (Variables|Energy|GetEnergyAvailable)
            (Utilities|FlowControl|Gate true
              (:Exit
                (Utilities|CheckEnergyUsage 0.07
                  (:Proceed
                    (Variables|Boosting|SetBoosting true)
                    (Variables|DepthMovement|SetCurrentDepthPosition (Math|Float|Clamp(Float) (+ (Variables|DepthMovement|GetCurrentDepthPosition) (Variables|Boosting|GetBoostSpeed)) _maxbrakeposition _maxboostposition))))))))
        (:then_1
          (if (Variables|Energy|GetEnergyAvailable)
            (Utilities|FlowControl|Gate true
              (:Exit
                (Utilities|CheckEnergyUsage 0.05
                  (:Proceed
                    (Variables|Energy|SetBraking true)
                    (Variables|DepthMovement|SetCurrentDepthPosition (Math|Float|Clamp(Float) (- (Variables|DepthMovement|GetCurrentDepthPosition) (Variables|Braking|GetBrakeSpeed)) _maxbrakeposition _maxboostposition))))))))))
    (:then_4
      ;[1 1 1] Pull aircraft back to the middle when not boosting or braking
      (Math|Float|CompareFloat (Variables|DepthMovement|GetCurrentDepthPosition) 0.0
        (:>
          (if (not (Variables|Boosting|GetBoosting))
            (Variables|DepthMovement|SetCurrentDepthPosition (Math|Float|Clamp(Float) (- (Variables|DepthMovement|GetCurrentDepthPosition) 2.5) 0.0 (Variables|Boosting|GetMaxBoostPosition)))))
        (:==
          (Variables|DepthMovement|SetCurrentDepthPosition 0.0))
        (:<
          (if (not (Variables|Energy|GetBraking))
            (Variables|DepthMovement|SetCurrentDepthPosition (Math|Float|Clamp(Float) (+ (Variables|DepthMovement|GetCurrentDepthPosition) 2.5) (Variables|Braking|GetMaxBrakePosition) 0.0))))))
    (:then_5
      ;[1 1 1] Rotate Targeting Guides and position the inner one
      (Transformation|SetWorldRotation (Variables|Default|GetWidgetLaserTargeting) (Math|Rotator|MakeRotfromX (Math|Vector|Normalize (* (- (Transformation|GetActorLocation (Game|GetPlayerCameraManager 0)) (Transformation|GetWorldLocation (Variables|Default|GetWidgetLaserTargeting))) "1.000000,1.000000,0.000000"))) false false)
      (Transformation|SetWorldLocation (Variables|Default|GetWidgetLaserTargetingGuide) (Math|Vector|Lerp(Vector) (Transformation|GetWorldLocation (Variables|Default|GetBlasterOrigin)) (Transformation|GetWorldLocation (Variables|Default|GetLaserTargeting)) 0.666) false true))))

(event Custom|FireBlaster
  (bind _aircraftdata (Variables|Core|GetAircraftData))
  (bind (_totalnumberofhitpoints _totalnumberofenergytanks _primaryweapongrade _totalnumberofmissiles _aircraftcolor) (Utilities|Struct|BreakSTRUCT_AicraftData _aircraftdata))
  ;[1 1 1] Fire Lasers
  (Utilities|FlowControl|Gate true
    (:Exit
      (bind _returnvalue (Game|SpawnActorfromClass "/Game/Weaponry/Master/Blueprints/BP_WeaponProjectile.BP_WeaponProjectile_C" (Math|Transform|MakeTransform (Transformation|GetWorldLocation (Variables|Default|GetBlasterOrigin)) (Math|Conversions|RotationFromXVector (Math|Vector|GetForwardVector (Variables|Default|GetBlasterOrigin)))) "Undefined" 0 0))
      (Default|ProjectileSetHitInfo _returnvalue _primaryweapongrade (Utilities|Struct|MakeSTRUCT_Factions true false true true))
      (bind _returnvalue_2 (Rendering|Material|CreateDynamicMaterialInstance (Variables|/Game/Weaponry/Master/Blueprints/BP_WeaponProjectile.BP_WeaponProjectile_C|GetSM_BlasterBoltSingle _returnvalue) 0 "/Game/Weaponry/Blasters/Materials/M_BlasterBoltMaterial.M_BlasterBoltMaterial" :!class /Script/Engine.PrimitiveComponent))
      (Rendering|Material|SetVectorParameterValue _returnvalue_2 "Color" (.SpecifiedColor (Utilities|Struct|BreakSlateColor _aircraftcolor)) :!class /Script/Engine.MaterialInstanceDynamic))))

(event EventBeginPlay
  ;[1 1 1] Fire Lasers
  (Utilities|Time|SetTimerbyEvent (delegate Custom|FireBlaster) 0.06 true))

(event Input|ActionEvents|InputActionBarrelRollLeft
  (params (Key :type Key%20Structure :default "AnyKey"))
  (bind _barrelrollcontrol (Variables|Default|GetBarrelRollControl))
  ;[1 1 1] Barrel Rolls
  (:Pressed
    (Utilities|FlowControl|Sequence
      (:then_0
        (Utilities|FlowControl|Gate false :!label _label
          (:Exit
            (Variables|BarrelRolling|SetBarrelRollingLeft true)
            (bind _barrelrollleft (Timeline|BarrelRollLeft PlayFromStart)
              (:Update
                (Transformation|SetRelativeRotation _barrelrollcontrol (Math|Rotator|MakeRotator _barrelrollleft 0.0 0.0) false false))
              (:Finished
                (Variables|BarrelRolling|SetBarrelRollingLeft false))))))
      (:then_1
        (Utilities|FlowControl|Sequence
          (:then_0
            (goto _label Close))
          (:then_1
            (Utilities|FlowControl|Gate false) ; enters at Close
          )))
      (:then_2
        (Utilities|FlowControl|Delay 0.76)
        (Utilities|FlowControl|Sequence
          (:then_0
            (goto _label Open))
          (:then_1
            (Utilities|FlowControl|Gate false) ; enters at Open
          ))))))

(event Input|ActionEvents|InputActionBarrelRollRight
  (params (Key :type Key%20Structure :default "AnyKey"))
  (bind _barrelrollcontrol (Variables|Default|GetBarrelRollControl))
  ;[1 1 1] Barrel Rolls
  (:Pressed
    (Utilities|FlowControl|Sequence
      (:then_0
        (Utilities|FlowControl|Gate false :!label _label
          (:Exit
            (Variables|BarrelRolling|SetBarrelRollingRight true)
            (bind _barrelrollright (Timeline|BarrelRollRight PlayFromStart)
              (:Update
                (Transformation|SetRelativeRotation _barrelrollcontrol (Math|Rotator|MakeRotator _barrelrollright 0.0 0.0) false false))
              (:Finished
                (Variables|BarrelRolling|SetBarrelRollingRight false))))))
      (:then_1
        (Utilities|FlowControl|Sequence
          (:then_0
            (Utilities|FlowControl|Gate false) ; enters at Close
          )
          (:then_1
            (goto _label Close))))
      (:then_2
        (Utilities|FlowControl|Delay 0.76)
        (Utilities|FlowControl|Sequence
          (:then_0
            (Utilities|FlowControl|Gate false) ; enters at Open
          )
          (:then_1
            (goto _label Open)))))))

(event Input|ActionEvents|InputActionFireBlasters
  (params (Key :type Key%20Structure :default "AnyKey"))
  (bind _aircraftdata (Variables|Core|GetAircraftData))
  (bind (_totalnumberofhitpoints _totalnumberofenergytanks _primaryweapongrade _totalnumberofmissiles _aircraftcolor) (Utilities|Struct|BreakSTRUCT_AicraftData _aircraftdata))
  ;[1 1 1] Fire Lasers
  (:Pressed
    (Utilities|FlowControl|Gate true) ; enters at Open
  )
  (:Released
    (Utilities|FlowControl|Gate true) ; enters at Close
  ))

(event Input|ActionEvents|InputActionBoost
  (params (Key :type Key%20Structure :default "AnyKey"))
  ;[1 1 1] Boost Brake
  (:Pressed
    (if (not (Variables|Energy|GetBraking))
      (Utilities|FlowControl|Gate true) ; enters at Open
    ))
  (:Released
    (Variables|Boosting|SetBoosting false)
    (Utilities|FlowControl|Gate true) ; enters at Close
  ))

(event Input|ActionEvents|InputActionBrake
  (params (Key :type Key%20Structure :default "AnyKey"))
  ;[1 1 1] Boost Brake
  (:Pressed
    (if (not (Variables|Boosting|GetBoosting))
      (Utilities|FlowControl|Gate true) ; enters at Open
    ))
  (:Released
    (Variables|Energy|SetBraking false)
    (Utilities|FlowControl|Gate true) ; enters at Close
  ))

(event Input|AxisEvents|InputAxisAircraftVertical
  (params (AxisValue :type Float%20%28single-precision%29))
  (Variables|VerticalMovement|SetInputAxisVertical AxisValue)
  ;[1 1 1] Calculate the Depth Scale
  (Variables|DepthMovement|SetDepthScale (Math|Float|NormalizetoRange (Variables|DepthMovement|GetCurrentDepthPosition) (Variables|Braking|GetMaxBrakePosition) (Variables|Boosting|GetMaxBoostPosition)))
  ;[1 1 1] Tilt Control
  (Utilities|FlowControl|Sequence
    (:then_0
      ;[1 1 1] Get the Aircrafts current position along its clamped vertical axis
      (Variables|VerticalMovement|SetCurrentVerticalPosition (Math|Float|Clamp(Float) (+ (Variables|VerticalMovement|GetCurrentVerticalPosition) (* (Variables|VerticalMovement|GetInputAxisVertical) (Variables|VerticalMovement|GetVerticalMovementSpeed))) (* (Math|Float|Lerp (Variables|VerticalMovement|GetVerticalPositionLimitMin) (Variables|VerticalMovement|GetVerticalPositionLimitMax) (Variables|DepthMovement|GetDepthScale)) -1.0) (Math|Float|Lerp (Variables|VerticalMovement|GetVerticalPositionLimitMin) (Variables|VerticalMovement|GetVerticalPositionLimitMax) (Variables|DepthMovement|GetDepthScale))))
      ;[1 1 1] Set final Aircraft Position
      (Transformation|SetRelativeLocation (Variables|Default|GetAircraftControl) (Math|Vector|MakeVector (Variables|DepthMovement|GetCurrentDepthPosition) (Variables|HorizontalMovement|GetCurrentHorizontalPosition) (Variables|VerticalMovement|GetCurrentVerticalPosition)) true false))
    (:then_1
      (Utilities|TiltAircraft (Variables|VerticalMovement|GetInputAxisVertical) (Variables|HorizontalMovement|GetInputAxisHorizontal)))))

(event Input|AxisEvents|InputAxisAircraftHorizontal
  (params (AxisValue :type Float%20%28single-precision%29))
  (bind _horizontalpositionlimitmax (Variables|HorizontalMovement|GetHorizontalPositionLimitMax))
  (bind _depthscale (Variables|DepthMovement|GetDepthScale))
  (bind _horizontalpositionlimitmin (Variables|HorizontalMovement|GetHorizontalPositionLimitMin))
  (bind _returnvalue (Math|Float|Lerp _horizontalpositionlimitmin _horizontalpositionlimitmax _depthscale))
  (Variables|HorizontalMovement|SetInputAxisHorizontal AxisValue)
  ;[1 1 1] Calculate what Barrel Roll Horizontal Speed Multiplier should be applied
  (Math|Float|CompareFloat (Variables|HorizontalMovement|GetInputAxisHorizontal) 0.0
    (:>
      (if (Variables|BarrelRolling|GetBarrelRollingRight)
        (Variables|BarrelRolling|SetBarrelRollHorizontalBoost (Math|Float|Lerp 1.5 3.0 (Variables|DepthMovement|GetDepthScale)) :!label _label)
        (elif (Variables|BarrelRolling|GetBarrelRollingLeft)
          (Variables|BarrelRolling|SetBarrelRollHorizontalBoost 0.5 :!label _label_2)
          (else
            (Variables|BarrelRolling|SetBarrelRollHorizontalBoost 1.0 :!label _label_3)))))
    (:==
      (goto _label_3))
    (:<
      (if (Variables|BarrelRolling|GetBarrelRollingLeft)
        (goto _label)
        (elif (Variables|BarrelRolling|GetBarrelRollingRight)
          (goto _label_2)
          (else
            (goto _label_3))))))
  (Variables|HorizontalMovement|SetCurrentHorizontalPosition (Math|Float|Clamp(Float) (+ (Variables|HorizontalMovement|GetCurrentHorizontalPosition) (* (Variables|HorizontalMovement|GetInputAxisHorizontal) (Variables|HorizontalMovement|GetHorizontalMovementSpeed) (Variables|BarrelRolling|GetBarrelRollHorizontalBoost))) (+ (* _returnvalue -1.0) (Variables|HorizontalMovement|GetHorizontalOffsetMin)) (+ _returnvalue (Variables|HorizontalMovement|GetHorizontalOffsetMax)))))

(event Input|GamepadEvents|GamepadSpecialRight
  (params (Key :type Key%20Structure :default "AnyKey"))
  ;[1 1 1] Pause and Unpause
  (:Pressed
    (Utilities|FlowControl|FlipFlop
      (:A
        (Game|SetGamePaused true))
      (:B
        (Game|SetGamePaused false)))))

(fn ConstructionScript)

(fn SetAircraftColor
  (bind _aircraftdata (Variables|Core|GetAircraftData))
  (bind _aircraftcolor (Utilities|Struct|BreakSTRUCT_AicraftData _aircraftdata))
  (bind _specifiedcolor (Utilities|Struct|BreakSlateColor _aircraftcolor))
  (bind _asbp_hull_component_player (Utilities|Casting|CastToBP_HullComponentPlayer (Variables|/Script/Engine.ChildActorComponent|GetChildActor (Variables|Default|GetHullComponent))))
  (Default|SetEngineColor _asbp_hull_component_player _aircraftdata)
  (bind _aswid_laser_targeting (Utilities|Casting|CastToWID_LaserTargeting (UserInterface|GetUserWidgetObject (Variables|Default|GetWidgetLaserTargeting))))
  (Default|SetReticleColor _aswid_laser_targeting _specifiedcolor false)
  (bind _aswid_laser_targeting_2 (Utilities|Casting|CastToWID_LaserTargeting (UserInterface|GetUserWidgetObject (Variables|Default|GetWidgetLaserTargetingGuide))))
  (Default|SetReticleColor _aswid_laser_targeting_2 _specifiedcolor true))

(fn PivotAilerons
  (bind _depthscale (Variables|DepthMovement|GetDepthScale))
  (bind _returnvalue (Math|Float|Lerp 6e+01 0.0 _depthscale))
  (Utilities|FlowControl|Sequence
    (:then_0
      (Transformation|SetRelativeRotation (Variables|Default|GetAileronTopLeftControl) (Math|Rotator|MakeRotator 0.0 _returnvalue 0.0) false false))
    (:then_1
      (Transformation|SetRelativeRotation (Variables|Default|GetAileronBottomLeftControl) (Math|Rotator|MakeRotator 0.0 (* _returnvalue -1.0) 0.0) false false))))
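; Causeway bridge actor for the coastal environment, posed in the construction script from a single BridgeAngle value.
; The angle, clamped between flat and a quarter turn, sets the pitch of the Hinge component.
; The same clamped angle, normalized, blends ControlEndpiece's world location from the EndpieceOut marker to EndpieceIn, keeping it in step with the hinge.
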(fn ConstructionScript
  (bind _bridgeangle (Variables|Default|GetBridgeAngle))
  (bind _returnvalue (Math|Float|Clamp(Float) _bridgeangle 0.0 9e+01))
  (Transformation|SetRelativeRotation (Variables|Default|GetHinge) (Math|Rotator|MakeRotator 0.0 _returnvalue 0.0) false false)
  (Transformation|SetWorldLocation (Variables|Default|GetControlEndpiece) (Math|Vector|Lerp(Vector) (Transformation|GetWorldLocation (Variables|Default|GetEndpieceOut)) (Transformation|GetWorldLocation (Variables|Default|GetEndpieceIn)) (/ _returnvalue 9e+01)) false false))
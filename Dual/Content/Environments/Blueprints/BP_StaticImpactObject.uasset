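; BP_StaticImpactObject is an environment object that damages player ships on contact.
; The construction script applies a configurable mesh to its static mesh component.
; When that component begins overlapping a BP_Playership, it deals damage to the ship and plays a collision sound at the object's location.
; It also sends hit force feedback to player controller 0 or 1, chosen by the ship's Player enum.
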(event OnComponentBeginOverlap(StaticMesh)
  (params (OverlappedComponent :type Primitive%20Component%20Object%20Reference) (OtherActor :type Actor%20Object%20Reference) (OtherComp :type Primitive%20Component%20Object%20Reference) (OtherBodyIndex :type Integer) (bFromSweep :type Boolean) (SweepResult :type Hit%20Result%20Structure%20%28by%20ref%29))
  (bind _asbp_playership (Utilities|Casting|CastToBP_Playership OtherActor))
  (Default|TakeDamage _asbp_playership (Variables|Default|GetDamage))
  (Audio|PlaySoundatLocation (Variables|Default|GetCollisionSoundEffect) (Transformation|GetActorLocation self))
  (if (Utilities|Enum|Equal(Enum) (Variables|/Game/Players/Blueprints/BP_Playership.BP_Playership_C|GetPlayer _asbp_playership) "NewEnumerator0")
    (Game|Feedback|ClientPlayForceFeedback (Game|GetPlayerController 0) (Variables|Default|GetForceFeedbackHitGeometry) false false "None")
    (else
      (Game|Feedback|ClientPlayForceFeedback (Game|GetPlayerController 1) (Variables|Default|GetForceFeedbackHitGeometry) false false "None"))))

(fn ConstructionScript
  (Components|StaticMesh|SetStaticMesh (Variables|Default|GetStaticMesh) (Variables|Default|GetMesh)))
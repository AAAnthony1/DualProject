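; Starscape backdrop for interstellar travel that endlessly scrolls five groups of seven meshes along negative X, each group at its own speed.
; Each Tick, the Scrolling macro offsets the meshes, wraps those past the far end back to the start, and computes a position-based fade at both ends.
; That value scrubs a per-group timeline, whose curve sets StarBrightness on an M_Starscape dynamic material instance created at each update.
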(event EventTick
  (params (DeltaSeconds :type Float%20%28single-precision%29))
  (Utilities|FlowControl|Sequence
    (:then_0
      (bind (_mesh _starbrightness) (Utilities|Scrolling (Variables|Default|GetSpeedGroupA) (Utilities|Array|MakeArray (Variables|Default|Get1A) (Variables|Default|Get2A) (Variables|Default|Get3A) (Variables|Default|Get4A) (Variables|Default|Get5A) (Variables|Default|Get6A) (Variables|Default|Get7A)))
        (:OpacitySet
          (bind _starbrightnesscurve (Timeline|Timeline_Starbrightness SetNewTime)
            (:Update
              (bind _returnvalue (Rendering|Material|CreateDynamicMaterialInstance _mesh 0 "/Game/Environments/InterstellarTravel/M_Starscape.M_Starscape" :!class /Script/Engine.PrimitiveComponent))
              (Rendering|Material|SetScalarParameterValue _returnvalue "StarBrightness" _starbrightnesscurve :!class /Script/Engine.MaterialInstanceDynamic))))))
    (:then_1
      (bind (_mesh_2 _starbrightness_2) (Utilities|Scrolling (Variables|Default|GetSpeedGroupB) (Utilities|Array|MakeArray (Variables|Default|Get1B) (Variables|Default|Get2B) (Variables|Default|Get3B) (Variables|Default|Get4B) (Variables|Default|Get5B) (Variables|Default|Get6B) (Variables|Default|Get7B)))
        (:OpacitySet
          (bind _starbrightnesscurve_2 (Timeline|Timeline_0 SetNewTime)
            (:Update
              (bind _returnvalue_2 (Rendering|Material|CreateDynamicMaterialInstance _mesh_2 0 "/Game/Environments/InterstellarTravel/M_Starscape.M_Starscape" :!class /Script/Engine.PrimitiveComponent))
              (Rendering|Material|SetScalarParameterValue _returnvalue_2 "StarBrightness" _starbrightnesscurve_2 :!class /Script/Engine.MaterialInstanceDynamic))))))
    (:then_2
      (bind (_mesh_3 _starbrightness_3) (Utilities|Scrolling (Variables|Default|GetSpeedGroupC) (Utilities|Array|MakeArray (Variables|Default|Get1C) (Variables|Default|Get2C) (Variables|Default|Get3C) (Variables|Default|Get4C) (Variables|Default|Get5C) (Variables|Default|Get6C) (Variables|Default|Get7C)))
        (:OpacitySet
          (bind _starbrightnesscurve_3 (Timeline|Timeline_1 SetNewTime)
            (:Update
              (bind _returnvalue_3 (Rendering|Material|CreateDynamicMaterialInstance _mesh_3 0 "/Game/Environments/InterstellarTravel/M_Starscape.M_Starscape" :!class /Script/Engine.PrimitiveComponent))
              (Rendering|Material|SetScalarParameterValue _returnvalue_3 "StarBrightness" _starbrightnesscurve_3 :!class /Script/Engine.MaterialInstanceDynamic))))))
    (:then_3
      (bind (_mesh_4 _starbrightness_4) (Utilities|Scrolling (Variables|Default|GetSpeedGroupD) (Utilities|Array|MakeArray (Variables|Default|Get1D) (Variables|Default|Get2D) (Variables|Default|Get3D) (Variables|Default|Get4D) (Variables|Default|Get5D) (Variables|Default|Get6D) (Variables|Default|Get7D)))
        (:OpacitySet
          (bind _starbrightnesscurve_4 (Timeline|Timeline_2 SetNewTime)
            (:Update
              (bind _returnvalue_4 (Rendering|Material|CreateDynamicMaterialInstance _mesh_4 0 "/Game/Environments/InterstellarTravel/M_Starscape.M_Starscape" :!class /Script/Engine.PrimitiveComponent))
              (Rendering|Material|SetScalarParameterValue _returnvalue_4 "StarBrightness" _starbrightnesscurve_4 :!class /Script/Engine.MaterialInstanceDynamic))))))
    (:then_4
      (bind (_mesh_5 _starbrightness_5) (Utilities|Scrolling (Variables|Default|GetSpeedGroupE) (Utilities|Array|MakeArray (Variables|Default|Get1E) (Variables|Default|Get2E) (Variables|Default|Get3E) (Variables|Default|Get4E) (Variables|Default|Get5E) (Variables|Default|Get6E) (Variables|Default|Get7E)))
        (:OpacitySet
          (bind _starbrightnesscurve_5 (Timeline|Timeline_3 SetNewTime)
            (:Update
              (bind _returnvalue_5 (Rendering|Material|CreateDynamicMaterialInstance _mesh_5 0 "/Game/Environments/InterstellarTravel/M_Starscape.M_Starscape" :!class /Script/Engine.PrimitiveComponent))
              (Rendering|Material|SetScalarParameterValue _returnvalue_5 "StarBrightness" _starbrightnesscurve_5 :!class /Script/Engine.MaterialInstanceDynamic))))))))

(fn ConstructionScript)
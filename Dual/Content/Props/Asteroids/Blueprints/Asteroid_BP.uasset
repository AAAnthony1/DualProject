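; Asteroid prop that shows one of several rock meshes and tumbles in place.
; The construction script picks a random or chosen mesh from the RockMesh array, resetting out-of-range indices to the first.
; A looping timer at UpdateFrequency, rather than Tick, adds a small local rotation, either randomized at BeginPlay or a clamped manual override.
; Each step is not time-scaled, so spin speed follows the update frequency.
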(event Custom|RotateAsteroid
  (if (Variables|Asteroid|GetRotRateOverride)
    (Transformation|AddLocalRotation (Variables|Default|GetStaticMesh) (Math|Rotator|MakeRotator (Math|Float|Clamp(Float) (Variables|Asteroid|GetRoll) -1.0) (Math|Float|Clamp(Float) (Variables|Asteroid|GetPitch) -1.0) (Math|Float|Clamp(Float) (Variables|Asteroid|GetYaw) -1.0)) false false)
    (else
      (Transformation|AddLocalRotation (Variables|Default|GetStaticMesh) (Variables|Default|GetRotation) false false))))

(event EventBeginPlay
  (|CallParentFunction)
  (Variables|Default|SetRotation (Math|Rotator|MakeRotator (Math|Random|RandomFloatinRange -1.0 1.0) (Math|Random|RandomFloatinRange -1.0 1.0) (Math|Random|RandomFloatinRange -1.0 1.0)))
  (Utilities|Time|SetTimerbyEvent (delegate Custom|RotateAsteroid) (/ 1.0 (Variables|Asteroid|GetUpdateFrequency)) true))

(fn ConstructionScript
  (|CallParentFunction)
  (if (Variables|Asteroid|GetRandomRockMesh)
    (Variables|Asteroid|SetRockType (Math|Random|RandomInteger (Utilities|Array|Length (Variables|Default|GetRockMesh))))
    (Components|StaticMesh|SetStaticMesh (Variables|Default|GetStaticMesh) (Utilities|Array|Get(acopy) (Variables|Default|GetRockMesh) (Variables|Asteroid|GetRockType)) :!label _label)
    (elif (> (Variables|Asteroid|GetRockType) (- (Utilities|Array|Length (Variables|Default|GetRockMesh)) 1))
      (bind _output_get (Variables|Asteroid|SetRockType 0))
      (Components|StaticMesh|SetStaticMesh (Variables|Default|GetStaticMesh) (Utilities|Array|Get(acopy) (Variables|Default|GetRockMesh) _output_get))
      (else
        (goto _label)))))
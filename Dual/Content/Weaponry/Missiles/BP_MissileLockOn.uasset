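; Missile lock-on marker actor whose widget component shows a reticle in a color set through SetColor, which also stores the Player.
; A looping 30 Hz timer destroys it when its attached BP_DamageableComponent parent runs out of hitpoints or its position projects outside player 0's viewport.
; It otherwise expires seven seconds after BeginPlay.
; Despite its name, the WidgetFacePlayers timer event performs only these checks and never rotates the widget.
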(event Custom|WidgetFacePlayers
  (bind _returnvalue (Actor|GetAttachParentActor))
  (bind _returnvalue_2 (Game|GetPlayerController 0))
  (bind _returnvalue_3 (Viewport|GetViewportSize))
  (bind _self self)
  (bind _returnvalue_4 (Transformation|GetActorLocation _self))
  (bind (_x _y) (Math|Vector2D|BreakVector2D _returnvalue_3))
  (bind _screenlocation (Class|PlayerController|ProjectWorldLocationtoScreen _returnvalue_2 _returnvalue_4 false))
  (bind (_x_2 _y_2) (Math|Vector2D|BreakVector2D _screenlocation))
  (Utilities|FlowControl|Sequence
    (:then_0
      (Utilities|IsValid _returnvalue
        (:Is%20Valid
          (bind _asbp_damageable_component (Utilities|Casting|CastToBP_DamageableComponent _returnvalue))
          (Math|Integer|CompareInt (Variables|/Game/Units/Blueprints/BP_DamageableComponent.BP_DamageableComponent_C|GetCurrentHitpoints _asbp_damageable_component) 0
            (:==
              _)
            (:<
              _))
          (Utilities|FlowControl|DoOnce false
            (:Completed
              (Actor|DestroyActor))))))
    (:then_1
      (if (not (Math|Boolean|ANDBoolean (> _x_2 0.0) (> _y_2 0.0) (< _x_2 _x) (< _y_2 _y)))
        (Actor|DestroyActor)))))

(event Custom|SetColor
  (params (Color :type Linear%20Color%20Structure) (Player :type ENUM_PlayerNumber%20Enum :default "NewEnumerator0"))
  (bind _aswid_missile_lock_on (Utilities|Casting|CastToWID_MissileLockOn (UserInterface|GetUserWidgetObject (Variables|Default|GetWidgetMissileLockOn))))
  (Default|SetReticleColor _aswid_missile_lock_on Color)
  (Variables|Default|SetPlayer Player))

(event EventBeginPlay
  (Utilities|Time|SetTimerbyEvent (delegate Custom|WidgetFacePlayers) (/ 1.0 3e+01) true)
  (Utilities|FlowControl|Delay 7.0)
  (Actor|DestroyActor))

(fn ConstructionScript)
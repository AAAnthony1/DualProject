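; Missile projectile that can home on a target's mesh piece and explodes on impact for area damage.
; Collision switches on shortly after launch, and a missile that hits nothing self-destructs after a timeout with a smaller, damage-free explosion.
; Impacts, except with other weapon projectiles, sphere-overlap BP_DamageableComponent actors and call TakeMissileHit with the supplied AttackPower.
; The valid-targets list is stored and exposed but does not filter damage.
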(event Custom|HomingMissile
  (params (MissileTarget :type BP%20Damageable%20Component%20Object%20Reference))
  (bind _projectilemovement (Variables|Default|GetProjectileMovement))
  (Utilities|IsValid MissileTarget
    (:Is%20Valid
      (Variables|/Script/Engine.ProjectileMovementComponent|SetHomingTargetComponent _projectilemovement (Variables|/Game/Units/Blueprints/BP_DamageableComponent.BP_DamageableComponent_C|GetStaticMeshPiece MissileTarget))
      (Variables|/Script/Engine.ProjectileMovementComponent|SetbIsHomingProjectile _projectilemovement true)
      (Variables|/Script/Engine.ProjectileMovementComponent|SetHomingAccelerationMagnitude _projectilemovement 5e+04))))

(event EventBeginPlay
  (Audio|PlaySound2D "/Game/Audio/SoundEffects/SC_MissileLaunch.SC_MissileLaunch")
  (Utilities|FlowControl|Sequence
    (:then_0
      (Utilities|FlowControl|Delay 0.1)
      (Collision|SetCollisionEnabled (Variables|Default|GetSM_Missile) "QueryAndPhysics"))
    (:then_1
      (Utilities|FlowControl|Delay 5.0)
      (Effects|SpawnEmitteratLocation "/Game/StarterContent/Particles/P_Explosion.P_Explosion" (Transformation|GetActorLocation) "0, 0, 0" "20.000000,20.000000,20.000000")
      (Actor|DestroyActor))))

(event Collision|EventHit
  (params (MyComp :type Primitive%20Component%20Object%20Reference) (Other :type Actor%20Object%20Reference) (OtherComp :type Primitive%20Component%20Object%20Reference) (bSelfMoved :type Boolean) (HitLocation :type Vector :default "0, 0, 0") (HitNormal :type Vector :default "0, 0, 0") (NormalImpulse :type Vector :default "0, 0, 0") (Hit :type Hit%20Result%20Structure%20%28by%20ref%29))
  (Utilities|Casting|CastToBP_WeaponProjectile Other
    (:CastFailed
      (Audio|PlaySoundatLocation "/Game/Audio/SoundEffects/SC_MissileExplodes.SC_MissileExplodes" HitLocation)
      (Utilities|FlowControl|Sequence
        (:then_0
          (Effects|SpawnEmitteratLocation "/Game/StarterContent/Particles/P_Explosion.P_Explosion" HitLocation "0, 0, 0" "80.000000,80.000000,80.000000")
          (Actor|DestroyActor))
        (:then_1
          (bind _outactors (Collision|SphereOverlapActors HitLocation 4e+03 (Variables|Default|GetObjectTypes) "/Game/Units/Blueprints/BP_DamageableComponent.BP_DamageableComponent_C"))
          (for _array_element _outactors
            (bind _asbp_damageable_component (Utilities|Casting|CastToBP_DamageableComponent _array_element))
            (Default|TakeMissileHit _asbp_damageable_component (Variables|Default|GetAttackPower))))))))

(event EventProjectileSetHitInfo
  (params (AttackPower :type Integer) (ValidTargetsList :type STRUCT%20Factions%20Structure))
  (Variables|Default|SetAttackPower AttackPower)
  (Variables|Default|SetValidTargetsList ValidTargetsList))

(fn ConstructionScript)

(fn WeaponGetHitInfo
  (return (Variables|Default|GetAttackPower) (Variables|Default|GetValidTargetsList)))

(fn WeaponSetHitInfo
  (params (AttackPower :type Integer) (ValidTargetsList :type STRUCT%20Factions%20Structure))
  (return))

(fn ProjectileGetHitInfo
  (return (Variables|Default|GetAttackPower) (Variables|Default|GetValidTargetsList)))
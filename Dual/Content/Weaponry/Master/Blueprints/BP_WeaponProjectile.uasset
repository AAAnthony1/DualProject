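; Blaster bolt projectile that carries attack power and a valid-target list, set by an event and exposed through weapon and projectile getters.
; On spawn it plays the firing sound, enables mesh collision after a brief delay and self-destructs after a few seconds.
; Any hit destroys it shortly after, with explosion and sound only if the other actor casts to BP_DamageableComponent.
; It applies no damage itself, and WeaponSetHitInfo is empty.
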(event EventBeginPlay
  (Audio|PlaySound2D "/Game/Audio/SoundEffects/SC_Blaster.SC_Blaster")
  (Utilities|FlowControl|Sequence
    (:then_0
      (Utilities|FlowControl|Delay 0.01)
      (Collision|SetCollisionEnabled (Variables|Default|GetSM_BlasterBoltSingle) "QueryAndPhysics"))
    (:then_1
      (Utilities|FlowControl|Delay 5.0)
      (Actor|DestroyActor))))

(event Collision|EventHit
  (params (MyComp :type Primitive%20Component%20Object%20Reference) (Other :type Actor%20Object%20Reference) (OtherComp :type Primitive%20Component%20Object%20Reference) (bSelfMoved :type Boolean) (HitLocation :type Vector :default "0, 0, 0") (HitNormal :type Vector :default "0, 0, 0") (NormalImpulse :type Vector :default "0, 0, 0") (Hit :type Hit%20Result%20Structure%20%28by%20ref%29))
  (Utilities|FlowControl|Sequence
    (:then_0
      (Utilities|FlowControl|Delay 0.01)
      (Actor|DestroyActor))
    (:then_1
      (Utilities|Casting|CastToBP_DamageableComponent Other)
      (Effects|SpawnEmitteratLocation "/Game/StarterContent/Particles/P_Explosion.P_Explosion" HitLocation)
      (Audio|PlaySoundatLocation "/Game/Audio/SoundEffects/SC_BlasterHit.SC_BlasterHit" HitLocation))))

(event EventProjectileSetHitInfo
  (params (AttackPower :type Integer) (ValidTargetsList :type STRUCT%20Factions%20Structure))
  (Variables|Default|SetAttackPower AttackPower)
  (Variables|Default|SetValidTargetsList ValidTargetsList))

(fn ConstructionScript)

(fn WeaponGetHitInfo
  (return (Variables|Default|GetAttackPower) (Variables|Default|GetValidTargetsList)))

(fn WeaponSetHitInfo
  (params (AttackPower :type Integer) (ValidTargetsList :type STRUCT%20Factions%20Structure))
  (return))

(fn ProjectileGetHitInfo
  (return (Variables|Default|GetAttackPower) (Variables|Default|GetValidTargetsList)))
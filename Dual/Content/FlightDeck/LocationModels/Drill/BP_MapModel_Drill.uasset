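; BP_MapModel_Drill is an animated planet map model for the Drill location on the flight deck.
; The construction script creates dynamic materials giving the halo plane and cloud mesh green tints, with cloud emissive switched off.
; From BeginPlay, SpinMore re-calls itself through a 1/60-second Delay instead of using Tick.
; Each pass rotates the coastal and cloud meshes on different axes and turns the Scene component toward the player camera.
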(event Custom|SpinMore
  (Transformation|AddLocalRotation (Variables|Default|GetSM_MapModelCoastal) (Math|Rotator|MakeRotator 0.0 0.2 0.0) false false)
  (Transformation|AddLocalRotation (Variables|Default|GetSM_MapModel_Clouds) (Math|Rotator|MakeRotator 0.0 0.0 0.1) false false)
  (Utilities|FlowControl|Delay (/ 1.0 6e+01))
  (Transformation|SetWorldRotation (Variables|Default|GetScene) (Math|Rotator|FindLookatRotation (Transformation|GetActorLocation self) (Transformation|GetActorLocation (Game|GetPlayerCameraManager 0))) false false)
  (CallFunction|SpinMore))

(event EventBeginPlay
  (Transformation|AddLocalRotation (Variables|Default|GetSM_MapModelCoastal) (Math|Rotator|MakeRotator 0.0 0.2 0.0) false false)
  (Transformation|AddLocalRotation (Variables|Default|GetSM_MapModel_Clouds) (Math|Rotator|MakeRotator 0.0 0.0 0.1) false false)
  (Utilities|FlowControl|Delay (/ 1.0 6e+01))
  (Transformation|SetWorldRotation (Variables|Default|GetScene) (Math|Rotator|FindLookatRotation (Transformation|GetActorLocation self) (Transformation|GetActorLocation (Game|GetPlayerCameraManager 0))) false false)
  (CallFunction|SpinMore))

(fn ConstructionScript
  (Utilities|FlowControl|Sequence
    (:then_0
      (bind _returnvalue (Rendering|Material|CreateDynamicMaterialInstance (Variables|Default|GetPlaneHalo) 0 "/Game/FlightDeck/LocationModels/Common/M_PlanetHalo.M_PlanetHalo" :!class /Script/Engine.PrimitiveComponent))
      (Rendering|Material|SetScalarParameterValue _returnvalue "HaloEmissivePower" 1.0 :!class /Script/Engine.MaterialInstanceDynamic)
      (Rendering|Material|SetVectorParameterValue _returnvalue "HaloColor" "(R=0.041397,G=0.630208,B=0.411603,A=1.000000)" :!class /Script/Engine.MaterialInstanceDynamic))
    (:then_1
      (bind _returnvalue_2 (Rendering|Material|CreateDynamicMaterialInstance (Variables|Default|GetSM_MapModel_Clouds) 0 "/Game/FlightDeck/LocationModels/Common/M_MapModelClouds.M_MapModelClouds" :!class /Script/Engine.PrimitiveComponent))
      (Rendering|Material|SetScalarParameterValue _returnvalue_2 "CloudEmissivePower" 0.0 :!class /Script/Engine.MaterialInstanceDynamic)
      (Rendering|Material|SetVectorParameterValue _returnvalue_2 "CloudColor" "(R=0.139973,G=0.520833,B=0.138346,A=1.000000)" :!class /Script/Engine.MaterialInstanceDynamic))))
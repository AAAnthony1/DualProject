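; Glacier map model for the flight deck: an animated miniature planet with whales and a glowing halo.
; A self-repeating delay loop, started on BeginPlay and aimed at 60 Hz, counter-rotates the planet mesh and whale group by fixed steps.
; The same loop billboards a scene component toward the player camera.
; The construction script gives the halo plane a dynamic material with its color and emissive power.
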(event Custom|SpinMore
  (Transformation|AddLocalRotation (Variables|Default|GetSM_MapModel_GlacierPlanet) (Math|Rotator|MakeRotator 0.0 0.0 -0.4) false false)
  (Transformation|AddLocalRotation (Variables|Default|GetSceneWhales) (Math|Rotator|MakeRotator 0.0 0.0 0.6) false false)
  (Utilities|FlowControl|Delay (/ 1.0 6e+01))
  (Transformation|SetWorldRotation (Variables|Default|GetScene) (Math|Rotator|FindLookatRotation (Transformation|GetActorLocation self) (Transformation|GetActorLocation (Game|GetPlayerCameraManager 0))) false false)
  (CallFunction|SpinMore))

(event EventBeginPlay
  (Transformation|AddLocalRotation (Variables|Default|GetSM_MapModel_GlacierPlanet) (Math|Rotator|MakeRotator 0.0 0.0 -0.4) false false)
  (Transformation|AddLocalRotation (Variables|Default|GetSceneWhales) (Math|Rotator|MakeRotator 0.0 0.0 0.6) false false)
  (Utilities|FlowControl|Delay (/ 1.0 6e+01))
  (Transformation|SetWorldRotation (Variables|Default|GetScene) (Math|Rotator|FindLookatRotation (Transformation|GetActorLocation self) (Transformation|GetActorLocation (Game|GetPlayerCameraManager 0))) false false)
  (CallFunction|SpinMore))

(fn ConstructionScript
  (bind _returnvalue (Rendering|Material|CreateDynamicMaterialInstance (Variables|Default|GetPlaneHalo) 0 "/Game/FlightDeck/LocationModels/Common/M_PlanetHalo.M_PlanetHalo" :!class /Script/Engine.PrimitiveComponent))
  (Rendering|Material|SetScalarParameterValue _returnvalue "HaloEmissivePower" 1.0 :!class /Script/Engine.MaterialInstanceDynamic)
  (Rendering|Material|SetVectorParameterValue _returnvalue "HaloColor" "(R=1.000000,G=0.967098,B=0.957051,A=1.000000)" :!class /Script/Engine.MaterialInstanceDynamic))
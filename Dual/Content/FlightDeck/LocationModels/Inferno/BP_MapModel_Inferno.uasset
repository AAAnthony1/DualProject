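; Flight deck map model of the Inferno location: a spinning mesh with a glowing orange-red planet halo.
; The construction script builds a dynamic M_PlanetHalo material for PlaneHalo, setting its emissive power, color and texture.
; From BeginPlay, SpinMore re-triggers itself through a 1/60-second Delay instead of Tick, adding yaw to the mesh and turning the Scene component toward the player camera.
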(event Custom|SpinMore
  (Transformation|AddLocalRotation (Variables|Default|GetSM_MapModelInferno) (Math|Rotator|MakeRotator 0.0 0.0 3.0) false false)
  (Utilities|FlowControl|Delay (/ 1.0 6e+01))
  (Transformation|SetWorldRotation (Variables|Default|GetScene) (Math|Rotator|FindLookatRotation (Transformation|GetActorLocation self) (Transformation|GetActorLocation (Game|GetPlayerCameraManager 0))) false false)
  (CallFunction|SpinMore))

(event EventBeginPlay
  (Transformation|AddLocalRotation (Variables|Default|GetSM_MapModelInferno) (Math|Rotator|MakeRotator 0.0 0.0 3.0) false false)
  (Utilities|FlowControl|Delay (/ 1.0 6e+01))
  (Transformation|SetWorldRotation (Variables|Default|GetScene) (Math|Rotator|FindLookatRotation (Transformation|GetActorLocation self) (Transformation|GetActorLocation (Game|GetPlayerCameraManager 0))) false false)
  (CallFunction|SpinMore))

(fn ConstructionScript
  (bind _returnvalue (Rendering|Material|CreateDynamicMaterialInstance (Variables|Default|GetPlaneHalo) 0 "/Game/FlightDeck/LocationModels/Common/M_PlanetHalo.M_PlanetHalo" :!class /Script/Engine.PrimitiveComponent))
  (Rendering|Material|SetScalarParameterValue _returnvalue "HaloEmissivePower" 25.0 :!class /Script/Engine.MaterialInstanceDynamic)
  (Rendering|Material|SetVectorParameterValue _returnvalue "HaloColor" "(R=1.000000,G=0.056943,B=0.000000,A=1.000000)" :!class /Script/Engine.MaterialInstanceDynamic)
  (Rendering|Material|SetTextureParameterValue _returnvalue "HaloTexture" "/Game/FlightDeck/LocationModels/Common/T_PlanetHaloLarge.T_PlanetHaloLarge"))
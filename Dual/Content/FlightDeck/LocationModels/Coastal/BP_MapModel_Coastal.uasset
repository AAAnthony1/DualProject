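; BP_MapModel_Coastal is a flight deck location model that displays an animated coastal map with clouds.
; A self-repeating loop, started on BeginPlay and paced by a 1/60-second Delay instead of Tick, slowly yaws the map and cloud meshes in opposite directions.
; Each pass also turns the Scene component to face the player camera.
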(event Custom|SpinMore
  (Transformation|AddLocalRotation (Variables|Default|GetSM_MapModelCoastal) (Math|Rotator|MakeRotator 0.0 0.0 -0.25) false false)
  (Transformation|AddLocalRotation (Variables|Default|GetSM_MapModel_Clouds) (Math|Rotator|MakeRotator 0.0 0.0 0.05) false false)
  (Utilities|FlowControl|Delay (/ 1.0 6e+01))
  (Transformation|SetWorldRotation (Variables|Default|GetScene) (Math|Rotator|FindLookatRotation (Transformation|GetActorLocation self) (Transformation|GetActorLocation (Game|GetPlayerCameraManager 0))) false false)
  (CallFunction|SpinMore))

(event EventBeginPlay
  (Transformation|AddLocalRotation (Variables|Default|GetSM_MapModelCoastal) (Math|Rotator|MakeRotator 0.0 0.0 -0.25) false false)
  (Transformation|AddLocalRotation (Variables|Default|GetSM_MapModel_Clouds) (Math|Rotator|MakeRotator 0.0 0.0 0.05) false false)
  (Utilities|FlowControl|Delay (/ 1.0 6e+01))
  (Transformation|SetWorldRotation (Variables|Default|GetScene) (Math|Rotator|FindLookatRotation (Transformation|GetActorLocation self) (Transformation|GetActorLocation (Game|GetPlayerCameraManager 0))) false false)
  (CallFunction|SpinMore))

(fn ConstructionScript)
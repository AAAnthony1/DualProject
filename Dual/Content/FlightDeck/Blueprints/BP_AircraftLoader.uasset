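; Aircraft loader that carries a ship model along the spline of its parent BP_AircraftLoaderTrack, starting at a default slot.
; ChangePosition updates a looping slot index and plays a timeline that slides it one-seventh of the spline up or down, wrapping at the ends.
; The construction script sets a Player1 material parameter from the track's player.
; SetShipMesh swaps the displayed mesh and stores its data table index.
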(event Custom|ChangePosition
  (params (Down :type Boolean))
  ;[1 1 1] Move Loaders along track
  (CallFunction|SetLoaderCurrentPosition Down)
  (if Down
    (Variables|Default|SetDirectionMultiplier 1.0)
    (bind _movement (Timeline|AdjustPosition PlayFromStart)
      (:Update
        (Variables|Default|SetAdjustedPositionAlongTrack (/ (* _movement (Variables|Default|GetDirectionMultiplier)) 7.0))
        (CallFunction|SetPositionAlongTrack))
      (:Finished
        (Math|Float|CompareFloat (+ (Variables|Default|GetCurrentPositionOnTrack) (Variables|Default|GetAdjustedPositionAlongTrack)) 1.01
          (:>
            (Variables|Default|SetCurrentPositionOnTrack 0.0))
          (:==
            (Variables|Default|SetCurrentPositionOnTrack (+ (Variables|Default|GetCurrentPositionOnTrack) (Variables|Default|GetAdjustedPositionAlongTrack)) :!label _label))
          (:<
            (Math|Float|CompareFloat (+ (Variables|Default|GetCurrentPositionOnTrack) (Variables|Default|GetAdjustedPositionAlongTrack)) -0.01
              (:>
                (goto _label))
              (:==
                (goto _label))
              (:<
                (Variables|Default|SetCurrentPositionOnTrack 1.0)))))
        (Variables|Default|SetAdjustedPositionAlongTrack 0.0)))
    (else
      (Variables|Default|SetDirectionMultiplier -1.0)
      (Timeline|AdjustPosition PlayFromStart))))

(event Custom|SetShipMesh
  (params (StaticMesh :type Static%20Mesh%20Object%20Reference) (DataTableIndex :type Integer))
  ;[1 1 1] Set Static Mesh
  (Components|StaticMesh|SetStaticMesh (Variables|Default|GetShipModel) StaticMesh)
  (Variables|Default|SetShipDataTableIndex DataTableIndex))

(event Custom|SetPositionAlongTrack
  ;[1 1 1] Set Position Along Track
  (Transformation|SetActorLocationAndRotation (Spline|GetLocationatDistanceAlongSpline (Variables|Default|GetSpline) (* (Spline|GetSplineLength (Variables|Default|GetSpline)) (+ (Variables|Default|GetCurrentPositionOnTrack) (Variables|Default|GetAdjustedPositionAlongTrack))) "World") "0, 0, 0"))

(event EventBeginPlay
  ;[1 1 1] Set starting position along track
  (bind _asbp_aircraft_loader_track (Utilities|Casting|CastToBP_AircraftLoaderTrack (Actor|GetParentActor)))
  (Variables|Default|SetSpline (Variables|/Game/FlightDeck/Blueprints/BP_AircraftLoaderTrack.BP_AircraftLoaderTrack_C|GetSpline _asbp_aircraft_loader_track))
  (bind _output_get (Variables|Default|SetInPosition (Variables|Default|GetDefaultPositionOnTrack)))
  (Variables|Default|SetCurrentPositionOnTrack (/ (Math|Conversions|ToFloat(Integer) _output_get) 7.0))
  (Variables|Default|SetAdjustedPositionAlongTrack 0.0)
  (CallFunction|SetPositionAlongTrack))

(fn ConstructionScript
  (bind _returnvalue (Rendering|Material|CreateDynamicMaterialInstance (Variables|Default|GetShipModel) 2 0 :!class /Script/Engine.PrimitiveComponent))
  (bind _asbp_aircraft_loader_track (Utilities|Casting|CastToBP_AircraftLoaderTrack (Actor|GetParentActor)))
  (if (Utilities|Enum|Equal(Enum) (Variables|/Game/FlightDeck/Blueprints/BP_AircraftLoaderTrack.BP_AircraftLoaderTrack_C|GetPlayer _asbp_aircraft_loader_track) "NewEnumerator0")
    (Rendering|Material|SetScalarParameterValue _returnvalue "Player1" 1.0 :!class /Script/Engine.MaterialInstanceDynamic)
    (else
      (Rendering|Material|SetScalarParameterValue _returnvalue "Player1" 0.0 :!class /Script/Engine.MaterialInstanceDynamic))))

(fn SetLoaderCurrentPosition
  (params (Down :type Boolean))
  (if Down
    (Math|Integer|IncrementInt (Variables|Default|GetInPosition)
      (:%20%20
        _))
    (else
      (Math|Integer|DecrementInt (Variables|Default|GetInPosition)
        (:%20%20
          _))))
  (bind _intoutput (CallFunction|SetIntegerWithinLoopingRange (Variables|Default|GetInPosition) 0 7))
  (Variables|Default|SetInPosition _intoutput))
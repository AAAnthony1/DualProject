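; Flight deck ship-selection carousel for one player in the hub, hidden once the campaign has started.
; Eight child loaders shift along the track, with position 5 as the selection and end loaders re-meshed from wrapped DATA_PlayerShipTypes indices for endless scrolling.
; The selected ship feeds the player's GAMEMODE_Hub card and takes rotation input.
; Readying locks selection and saves ship data to the Game Instance; hub state changes trigger launch.
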(event Custom|ChangeSelection
  (params (Down :type Boolean))
  (bind _gamemodehub (Variables|Default|GetGamemodeHub))
  (bind _player (Variables|Default|GetPlayer))
  ;[1 1 1] Set Ship Data from up / down direction provided from Hub Pawn(s)
  (if (Variables|Default|GetAllowShipSelection)
    (Audio|PlaySound2D "/Game/FlightDeck/Audio/SC_ElectricMotorStart.SC_ElectricMotorStart")
    (Variables|Default|SetMoveTrackDown Down)
    (Utilities|FlowControl|Sequence
      (:then_0
        (Utilities|FlowControl|Delay 0.25)
        (for _array_element (Variables|Default|GetLoadersArray)
          (if (== (Variables|/Game/FlightDeck/Blueprints/BP_AircraftLoader.BP_AircraftLoader_C|GetInPosition _array_element) 5)
            (Variables|Default|SetCurrentlySelectedLoader _array_element)
            (bind _outrownames (DataTable|GetDataTableRowNames "/Game/Players/Blueprints/DATA_PlayerShipTypes.DATA_PlayerShipTypes"))
            (bind _returnvalue (Utilities|GetDataTableRow "/Game/Players/Blueprints/DATA_PlayerShipTypes.DATA_PlayerShipTypes" (Utilities|Array|Get(acopy) _outrownames (Variables|/Game/FlightDeck/Blueprints/BP_AircraftLoader.BP_AircraftLoader_C|GetShipDataTableIndex _array_element)))
              (:then
                (Variables|Default|SetShipData (Utilities|Struct|MakeSTRUCT_ShipData (Utilities|Array|Get(acopy) _outrownames (Variables|/Game/FlightDeck/Blueprints/BP_AircraftLoader.BP_AircraftLoader_C|GetShipDataTableIndex _array_element)) (.DisplayName (Utilities|Struct|BreakSTRUCT_PlayerShipTypes _returnvalue)) (.Description (Utilities|Struct|BreakSTRUCT_PlayerShipTypes _returnvalue)) (.Icon (Utilities|Struct|BreakSTRUCT_PlayerShipTypes _returnvalue)) (.StartingArmorLevel (Utilities|Struct|BreakSTRUCT_PlayerShipTypes _returnvalue)) (.StartingThrustLevel (Utilities|Struct|BreakSTRUCT_PlayerShipTypes _returnvalue)) (.StartingBlasterLevel (Utilities|Struct|BreakSTRUCT_PlayerShipTypes _returnvalue)) (.StartingMissileCount (Utilities|Struct|BreakSTRUCT_PlayerShipTypes _returnvalue)) "(SpecifiedColor=(R=1.000000,G=1.000000,B=1.000000,A=1.000000),ColorUseRule=UseColor_Specified)" (.Ability (Utilities|Struct|BreakSTRUCT_PlayerShipTypes _returnvalue)) (.StartingModiifers (Utilities|Struct|BreakSTRUCT_PlayerShipTypes _returnvalue)) (.StartingTotalSpecialItemSlots (Utilities|Struct|BreakSTRUCT_PlayerShipTypes _returnvalue)) (.StartingSpecialItems (Utilities|Struct|BreakSTRUCT_PlayerShipTypes _returnvalue))))
                (if (Utilities|Enum|Equal(Enum) _player "NewEnumerator0")
                  (Default|UpdateShipCardPlayer1 _gamemodehub (Variables|Default|GetShipData))
                  (elif (Utilities|Enum|Equal(Enum) _player "NewEnumerator1")
                    (Default|UpdateShipCardPlayer2 _gamemodehub (Variables|Default|GetShipData)))))))))
      (:then_1
        (for _array_element_2 (Variables|Default|GetLoadersArray)
          (Default|ChangePosition _array_element_2 (Variables|Default|GetMoveTrackDown))
          (Default|ResetShipOrientation _array_element_2))
        (CallFunction|ChangeMeshesonFirstandLastLoader)))))

(event Custom|OrientateShip
  (params (ShipRotateVertical :type Float%20%28single-precision%29) (ShipRotateHorizontal :type Float%20%28single-precision%29))
  ;[1 1 1] Pass Camera Control Input through to selected loader
  (if (Variables|Default|GetAllowShipSelection)
    (Default|OrientateShip (Variables|Default|GetCurrentlySelectedLoader) ShipRotateVertical ShipRotateHorizontal)))

(event Custom|ShipSelectPlayerReady
  (params (Ready :type Boolean))
  (bind _shipdata (Variables|Default|GetShipData))
  (bind _gamemodehub (Variables|Default|GetGamemodeHub))
  (bind _gamemodehub_2 (Variables|Default|GetGamemodeHub))
  ;[1 1 1] Ship Selected
  (if Ready
    (Utilities|FlowControl|Sequence
      (:then_0
        (Utilities|FlowControl|DoOnce false :!label _label
          (:Completed
            (Variables|Default|SetAllowShipSelection false)
            (if (Utilities|Enum|Equal(Enum) (Variables|Default|GetPlayer) "NewEnumerator0")
              (Default|PlayerReady _gamemodehub_2 1 true)
              (else
                (Default|PlayerReady _gamemodehub_2 2 true)))
            (Default|ResetShipOrientation (Variables|Default|GetCurrentlySelectedLoader))
            ;[1 1 1] Save Ship Data to the Game Instance
            (bind _asbp_game_instance_campaign (Utilities|Casting|CastToBP_GameInstance_Campaign (Game|GetGameInstance)))
            (if (Utilities|Enum|Equal(Enum) (Variables|Default|GetPlayer) "NewEnumerator0")
              (Variables|/Game/Gamemodes/BP_GameInstance_Campaign.BP_GameInstance_Campaign_C|SetShipDataPlayer1 _asbp_game_instance_campaign _shipdata)
              (else
                (Variables|/Game/Gamemodes/BP_GameInstance_Campaign.BP_GameInstance_Campaign_C|SetShipDataPlayer2 _asbp_game_instance_campaign _shipdata))))))
      (:then_1
        (goto _label_2 Reset)))
    (else
      (Utilities|FlowControl|Sequence
        (:then_0
          (Utilities|FlowControl|DoOnce false :!label _label_2
            (:Completed
              (Variables|Default|SetAllowShipSelection true)
              (if (Utilities|Enum|Equal(Enum) (Variables|Default|GetPlayer) "NewEnumerator0")
                (Default|PlayerReady _gamemodehub 1 false)
                (else
                  (Default|PlayerReady _gamemodehub 2 false))))))
        (:then_1
          (goto _label Reset))))))

(event Custom|ChangeMeshesOnFirstAndLastLoader
  (bind _loadersarray (Variables|Default|GetLoadersArray))
  (bind _totalselectableships (Variables|Default|GetTotalSelectableShips))
  (bind _returnvalue (- _totalselectableships 1))
  ;[1 1 1] Replace First and last loaders
  (for _array_element (Variables|Default|GetLoadersArray)
    (if (== (Variables|/Game/FlightDeck/Blueprints/BP_AircraftLoader.BP_AircraftLoader_C|GetInPosition _array_element) 0)
      (Variables|Default|SetLoaderInPosition0 _array_element)
      (for _array_element_2 _loadersarray
        (if (== (Variables|/Game/FlightDeck/Blueprints/BP_AircraftLoader.BP_AircraftLoader_C|GetInPosition _array_element_2) 1)
          (bind _output_get (Variables|Default|SetLoaderInPosition1 _array_element_2))
          (bind _intoutput (CallFunction|SetIntegerWithinLoopingRange (+ (Variables|/Game/FlightDeck/Blueprints/BP_AircraftLoader.BP_AircraftLoader_C|GetShipDataTableIndex _output_get) 1) 0 _returnvalue))
          (CallFunction|SetLoaderMesh (Variables|Default|GetLoaderInPosition0) _intoutput)))
      (elif (== (Variables|/Game/FlightDeck/Blueprints/BP_AircraftLoader.BP_AircraftLoader_C|GetInPosition _array_element) 7)
        (Variables|Default|SetLoaderInPosition7 _array_element)
        (for _array_element_3 _loadersarray
          (if (== (Variables|/Game/FlightDeck/Blueprints/BP_AircraftLoader.BP_AircraftLoader_C|GetInPosition _array_element_3) 6)
            (bind _output_get_2 (Variables|Default|SetLoaderInPosition6 _array_element_3))
            (bind _intoutput_2 (CallFunction|SetIntegerWithinLoopingRange (- (Variables|/Game/FlightDeck/Blueprints/BP_AircraftLoader.BP_AircraftLoader_C|GetShipDataTableIndex _output_get_2) 1) 0 _returnvalue))
            (CallFunction|SetLoaderMesh (Variables|Default|GetLoaderInPosition7) _intoutput_2)))))))

(event Custom|PopulateWidgetWithDefault
  (bind _gamemodehub (Variables|Default|GetGamemodeHub))
  (bind _player (Variables|Default|GetPlayer))
  ;[1 1 1] Set Ship Data from up / down direction provided from Hub Pawn(s)
  (for _array_element (Variables|Default|GetLoadersArray)
    (if (== (Variables|/Game/FlightDeck/Blueprints/BP_AircraftLoader.BP_AircraftLoader_C|GetInPosition _array_element) 5)
      (Variables|Default|SetCurrentlySelectedLoader _array_element)
      (bind _outrownames (DataTable|GetDataTableRowNames "/Game/Players/Blueprints/DATA_PlayerShipTypes.DATA_PlayerShipTypes"))
      (bind _returnvalue (Utilities|GetDataTableRow "/Game/Players/Blueprints/DATA_PlayerShipTypes.DATA_PlayerShipTypes" (Utilities|Array|Get(acopy) _outrownames (Variables|/Game/FlightDeck/Blueprints/BP_AircraftLoader.BP_AircraftLoader_C|GetShipDataTableIndex _array_element)))
        (:then
          (Variables|Default|SetShipData (Utilities|Struct|MakeSTRUCT_ShipData (Utilities|Array|Get(acopy) _outrownames (Variables|/Game/FlightDeck/Blueprints/BP_AircraftLoader.BP_AircraftLoader_C|GetShipDataTableIndex _array_element)) (.DisplayName (Utilities|Struct|BreakSTRUCT_PlayerShipTypes _returnvalue)) (.Description (Utilities|Struct|BreakSTRUCT_PlayerShipTypes _returnvalue)) (.Icon (Utilities|Struct|BreakSTRUCT_PlayerShipTypes _returnvalue)) (.StartingArmorLevel (Utilities|Struct|BreakSTRUCT_PlayerShipTypes _returnvalue)) (.StartingThrustLevel (Utilities|Struct|BreakSTRUCT_PlayerShipTypes _returnvalue)) (.StartingBlasterLevel (Utilities|Struct|BreakSTRUCT_PlayerShipTypes _returnvalue)) (.StartingMissileCount (Utilities|Struct|BreakSTRUCT_PlayerShipTypes _returnvalue)) "(SpecifiedColor=(R=1.000000,G=1.000000,B=1.000000,A=1.000000),ColorUseRule=UseColor_Specified)" (.Ability (Utilities|Struct|BreakSTRUCT_PlayerShipTypes _returnvalue)) (.StartingModiifers (Utilities|Struct|BreakSTRUCT_PlayerShipTypes _returnvalue)) (.StartingTotalSpecialItemSlots (Utilities|Struct|BreakSTRUCT_PlayerShipTypes _returnvalue)) (.StartingSpecialItems (Utilities|Struct|BreakSTRUCT_PlayerShipTypes _returnvalue))))
          (if (Utilities|Enum|Equal(Enum) _player "NewEnumerator0")
            (Default|UpdateShipCardPlayer1 _gamemodehub (Variables|Default|GetShipData))
            (elif (Utilities|Enum|Equal(Enum) _player "NewEnumerator1")
              (Default|UpdateShipCardPlayer2 _gamemodehub (Variables|Default|GetShipData)))))))))

(event Custom|HubStateShipSelect
  (params (State :type ENUM_HubState%20Enum :default "NewEnumerator1"))
  ;[1 1 1] Once the Ship Select Widget is created default it to the first ship
  (if (Utilities|Enum|Equal(Enum) State "NewEnumerator2")
    (Variables|Default|SetCurrentShipSelected 0)
    (CallFunction|PopulateWidgetwithDefault)
    (else
      ;[1 1 1] Launch Ship
      (if (Utilities|Enum|Equal(Enum) State "NewEnumerator4")
        (Default|LaunchShip (Variables|Default|GetCurrentlySelectedLoader))
        (for _array_element (Variables|Default|GetLoadersArray)
          (if (<= (Variables|/Game/FlightDeck/Blueprints/BP_AircraftLoader.BP_AircraftLoader_C|GetInPosition _array_element) 4)
            (Default|ClearLoader _array_element)))))))

(event EventBeginPlay
  (bind _loadersarray (Variables|Default|GetLoadersArray))
  (bind _asbp_game_instance_campaign (Utilities|Casting|CastToBP_GameInstance_Campaign (Game|GetGameInstance)))
  (if (Variables|/Game/Gamemodes/BP_GameInstance_Campaign.BP_GameInstance_Campaign_C|GetCampaignStarted _asbp_game_instance_campaign)
    (Development|SetHiddeninGame (Variables|Default|GetDefaultSceneRoot self) true true)
    (else
      (Utilities|FlowControl|Sequence
        (:then_0
          ;[1 1 1] Pack all the Loader Children into an Array
          (for _array_element (Utilities|Array|MakeArray (Variables|Default|GetLoader0) (Variables|Default|GetLoader1) (Variables|Default|GetLoader2) (Variables|Default|GetLoader3) (Variables|Default|GetLoader4) (Variables|Default|GetLoader5) (Variables|Default|GetLoader6) (Variables|Default|GetLoader7))
            (bind _aschild_actor_component (Utilities|Casting|CastToChildActorComponent _array_element))
            (bind _asbp_aircraft_loader (Utilities|Casting|CastToBP_AircraftLoader (Variables|/Script/Engine.ChildActorComponent|GetChildActor _aschild_actor_component)))
            (Utilities|Array|Add (Variables|Default|GetLoadersArray) _asbp_aircraft_loader)))
        (:then_1
          ;[1 1 1] Once the Ship Select Widget is created default it to the first ship
          (bind _asgamemode_hub (Utilities|Casting|CastToGAMEMODE_Hub (Game|GetGameMode)))
          (bind _output_get (Variables|Default|SetGamemodeHub _asgamemode_hub))
          (EventDispatchers|BindEventtoHubStateChanged _output_get (delegate Custom|HubStateShipSelect)))
        (:then_2
          ;[1 1 1] Get Total Selectable Ships and set meshes on loaders
          (bind _totalselectableships (CallFunction|GetTotalSelectableShips))
          (Variables|Default|SetTotalSelectableShips _totalselectableships))
        (:then_3
          ;[1 1 1] Set Initial Loader Ship Meshes
          (CallFunction|SetLoaderMesh (Utilities|Array|Get(acopy) _loadersarray) 5)
          (CallFunction|SetLoaderMesh (Utilities|Array|Get(acopy) _loadersarray 1) 4)
          (CallFunction|SetLoaderMesh (Utilities|Array|Get(acopy) _loadersarray 2) 3)
          (CallFunction|SetLoaderMesh (Utilities|Array|Get(acopy) _loadersarray 3) 2)
          (CallFunction|SetLoaderMesh (Utilities|Array|Get(acopy) _loadersarray 4) 1)
          (CallFunction|SetLoaderMesh (Utilities|Array|Get(acopy) _loadersarray 5))
          (CallFunction|SetLoaderMesh (Utilities|Array|Get(acopy) _loadersarray 6) (- (Variables|Default|GetTotalSelectableShips) 1))
          (CallFunction|SetLoaderMesh (Utilities|Array|Get(acopy) _loadersarray 7) (- (Variables|Default|GetTotalSelectableShips) 2)))))))

(fn ConstructionScript)

(fn GetTotalSelectableShips
  (bind _outrownames (DataTable|GetDataTableRowNames "/Game/Players/Blueprints/DATA_PlayerShipTypes.DATA_PlayerShipTypes"))
  (for _array_element _outrownames
    (bind _returnvalue (Utilities|GetDataTableRow "/Game/Players/Blueprints/DATA_PlayerShipTypes.DATA_PlayerShipTypes" _array_element)
      (:then
        (if (.Selectable (Utilities|Struct|BreakSTRUCT_PlayerShipTypes _returnvalue))
          (Math|Integer|IncrementInt (Variables|Default|GetSelectableShipsTally))))))
  (return (Variables|Default|GetSelectableShipsTally)))

(fn GetShipStaticMesh
  (params (DataTableIndex :type Integer))
  (bind _outrownames (DataTable|GetDataTableRowNames "/Game/Players/Blueprints/DATA_PlayerShipTypes.DATA_PlayerShipTypes"))
  (bind _returnvalue (Utilities|GetDataTableRow "/Game/Players/Blueprints/DATA_PlayerShipTypes.DATA_PlayerShipTypes" (Utilities|Array|Get(acopy) _outrownames DataTableIndex))
    (:then
      (return (Utilities|Struct|BreakSTRUCT_PlayerShipTypes _returnvalue)))))

(fn SetLoaderMesh
  (params (Loader :type BP%20Aircraft%20Loader%20Object%20Reference) (DataTableIndex :type Integer))
  (bind _staticmesh (CallFunction|GetShipStaticMesh DataTableIndex))
  (Default|SetShipMesh Loader _staticmesh DataTableIndex))
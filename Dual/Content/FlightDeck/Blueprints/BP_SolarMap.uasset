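; Campaign solar map that displays mission locations, zooms the hub camera onto the next one and plays its briefing.
; BeginPlay gathers child-actor locations and resolves the current one from the game instance's next mission via DATA_Missions.
; A timeline slides and lerps the camera to just short of that location, hiding labels.
; Briefings are hard-coded dialogue chains for four missions, ending in CallBriefingFinished; most of Coastal1's is disconnected.
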(event Custom|ShowSolarMap
  (params (Show :type Boolean))
  ;[1 1 1] Set Solar Map to Active
  (Variables|Default|SetSolarMapActive Show)
  (for _array_element (Variables|Default|GetLocationsArray)
    (Default|ShowLocation _array_element (Variables|Default|GetSolarMapActive))))

(event Custom|ZoomInCamera
  (params (True :type Boolean))
  (bind _hubcamera (Variables|Default|GetHubCamera))
  (bind _hubcamera_2 (Variables|Default|GetHubCamera))
  ;[1 1 1] Zoom Camera at Location
  (if True
    (Variables|Default|SetHubCameraMapSelectDefaultPosition (Transformation|GetActorLocation _hubcamera))
    (Variables|Default|SetHubCameraMapSelectDefaultRotation (Transformation|GetActorRotation _hubcamera))
    (CallFunction|SetCameraFocusPointLocation)
    (Utilities|FlowControl|Sequence
      (:then_0
        (bind _zoom (Timeline|Zoom PlayFromStart)
          (:Update
            (Default|SlideCameraRight (Variables|Default|GetHubCamera) _zoom)
            (Utilities|FlowControl|Sequence
              (:then_0
                (Transformation|SetActorLocation _hubcamera_2 (Math|Vector|Lerp(Vector) (Variables|Default|GetHubCameraMapSelectDefaultPosition) (Transformation|GetWorldLocation (Variables|Default|GetCameraFocusPoint)) _zoom) false false))
              (:then_1
                (Transformation|SetActorRotation _hubcamera_2 (Math|Rotator|Lerp(Rotator) (Variables|Default|GetHubCameraMapSelectDefaultRotation) (Math|Rotator|FindLookatRotation (Transformation|GetActorLocation (Variables|Default|GetHubCamera)) (Transformation|GetActorLocation (Variables|Default|GetCurrentLocation))) _zoom)))))))
      (:then_1
        (for _array_element (Variables|Default|GetLocationsArray)
          (Default|HideLabel _array_element true))))
    (else
      (Timeline|Zoom ReverseFromEnd))))

(event Custom|SetCameraFocusPointLocation
  (bind _hubcamera (Variables|Default|GetHubCamera))
  (bind _returnvalue (Transformation|GetActorLocation _hubcamera))
  ;[1 1 1] Set Camera Focus Point Location
  (Transformation|SetWorldLocation (Variables|Default|GetCameraFocusPoint) (+ _returnvalue (* (Math|Vector|GetUnitDirection(Vector) _returnvalue (Transformation|GetActorLocation (Variables|Default|GetCurrentLocation))) (- (Transformation|GetDistanceTo (Variables|Default|GetCurrentLocation) (Variables|Default|GetHubCamera)) 3.0))) false false))

(event EventBeginPlay
  ;[1 1 1] Pack Locations Into an Array
  (for _array_element (Utilities|Array|MakeArray (Variables|Default|GetBP_Location_Coastal) (Variables|Default|GetBP_Location_Station) (Variables|Default|GetBP_Location_Glacier) (Variables|Default|GetBP_Location_Facility) (Variables|Default|GetBP_Location_Shipyard) (Variables|Default|GetBP_Location_Skeletons) (Variables|Default|GetBP_Location_Drill) (Variables|Default|GetBP_Location_Inferno) (Variables|Default|GetBP_Location_Fortress) (Variables|Default|GetBP_Location_Experiment) (Variables|Default|GetBP_Location_Ocean) (Variables|Default|GetBP_Location_Capital))
    (bind _asbp_location (Utilities|Casting|CastToBP_Location (Variables|/Script/Engine.ChildActorComponent|GetChildActor _array_element)))
    (Utilities|Array|Add (Variables|Default|GetLocationsArray) _asbp_location))
  ;[1 1 1] Set Current Location
  (bind _currentlocation (CallFunction|GetCurrentLocation))
  (Variables|Default|SetCurrentLocation _currentlocation))

(event Custom|PlayMissionBriefing
  (bind _asbp_game_instance_campaign (Utilities|Casting|CastToBP_GameInstance_Campaign (Game|GetGameInstance)))
  (if (Utilities|Name|Equal(Name) (Variables|/Game/Gamemodes/BP_GameInstance_Campaign.BP_GameInstance_Campaign_C|GetNextMissionDataReference _asbp_game_instance_campaign) "Coastal1")
    (CallFunction|PlayMissionBriefingCoastal1)
    (elif (Utilities|Name|Equal(Name) (Variables|/Game/Gamemodes/BP_GameInstance_Campaign.BP_GameInstance_Campaign_C|GetNextMissionDataReference _asbp_game_instance_campaign) "Glacier1")
      (CallFunction|PlayMissionBriefingGlacier1)
      (elif (Utilities|Name|Equal(Name) (Variables|/Game/Gamemodes/BP_GameInstance_Campaign.BP_GameInstance_Campaign_C|GetNextMissionDataReference _asbp_game_instance_campaign) "Drill1")
        (CallFunction|PlayMissionBriefingDrill1)
        (elif (Utilities|Name|Equal(Name) (Variables|/Game/Gamemodes/BP_GameInstance_Campaign.BP_GameInstance_Campaign_C|GetNextMissionDataReference _asbp_game_instance_campaign) "Shipyard1")
          (CallFunction|PlayMissionBriefingShipyard1))))))

(event Custom|PlayMissionBriefingCoastal1
  (Utilities|PlayDialogue "NewEnumerator0" "NewEnumerator4" "NewEnumerator15" "NewEnumerator6" "This is Captain Jones, are you receiving me?" 3.5 true true "/Game/Audio/VO/Coastal/SC_Briefing_Coastal1_Captain_010.SC_Briefing_Coastal1_Captain_010"
    (:DelayedOut
      (Default|CallBriefingFinished))))

(event Custom|PlayMissionBriefingGlacier1
  (Utilities|PlayDialogue "NewEnumerator0" "NewEnumerator4" "NewEnumerator15" "NewEnumerator6" "I don't know who attacked the colony but we'll make them pay!" 3.5 true false
    (:DelayedOut
      (Utilities|PlayDialogue "NewEnumerator0" "NewEnumerator4" "NewEnumerator15" "NewEnumerator6" "The Aurora is in no shape for a fight though, we need to reach the science output at Arcadia to make repairs" 3.5 false false
        (:DelayedOut
          (Utilities|PlayDialogue "NewEnumerator2" "NewEnumerator4" "NewEnumerator15" "NewEnumerator6" "We'll keep the ship safe Captain" 2.5 false true
            (:DelayedOut
              (Default|CallBriefingFinished))))))))

(event Custom|PlayMissionBriefingShipyard1
  (Utilities|PlayDialogue "NewEnumerator0" "NewEnumerator4" "NewEnumerator15" "NewEnumerator6" "Our next target is a big one.  The Idin Shipyard.  Fly down to the surface and destroy the Reactor" 6.0 true false
    (:DelayedOut
      (Utilities|PlayDialogue "NewEnumerator2" "NewEnumerator4" "NewEnumerator15" "NewEnumerator6" "Will do" 3.0 false true
        (:DelayedOut
          (Default|CallBriefingFinished))))))

(event Custom|PlayMissionBriefingDrill1
  (Utilities|PlayDialogue "NewEnumerator0" "NewEnumerator4" "NewEnumerator15" "NewEnumerator6" "We've recieved communications from the surface, the enemy has overrun the colonial base with a huge force" 4.0 true false
    (:DelayedOut
      (Utilities|PlayDialogue "NewEnumerator3" "NewEnumerator4" "NewEnumerator15" "NewEnumerator6" "The Vale has no strategic value.  What have they got planned here?" 3.0 false false
        (:DelayedOut
          (Utilities|PlayDialogue "NewEnumerator0" "NewEnumerator4" "NewEnumerator15" "NewEnumerator6" "The intelligence we have is that they are drilling deep into the planet.  " 3.0 false false
            (:DelayedOut
              (Utilities|PlayDialogue "NewEnumerator0" "NewEnumerator4" "NewEnumerator15" "NewEnumerator6" "Geological scans of the planet a few decades ago revealed huge deposits of Antimatter but it was too difficult for us to reach.  " 3.0 false false
                (:DelayedOut
                  (Utilities|PlayDialogue "NewEnumerator2" "NewEnumerator4" "NewEnumerator15" "NewEnumerator6" "They could build devastating weapons with that!" 2.0 false false
                    (:DelayedOut
                      (Utilities|PlayDialogue "NewEnumerator0" "NewEnumerator4" "NewEnumerator15" "NewEnumerator6" "Not if the two of you take out those drills.  Strike fast and get out of there." 3.0 false true
                        (:DelayedOut
                          (Default|CallBriefingFinished))))))))))))))

(fn ConstructionScript)

(fn GetCurrentLocation
  (bind _asbp_game_instance_campaign (Utilities|Casting|CastToBP_GameInstance_Campaign (Game|GetGameInstance)))
  (bind _returnvalue (Utilities|GetDataTableRow "/Game/FlightDeck/Blueprints/DATA_Missions.DATA_Missions" (Variables|/Game/Gamemodes/BP_GameInstance_Campaign.BP_GameInstance_Campaign_C|GetNextMissionDataReference _asbp_game_instance_campaign))
    (:then
      (if (Utilities|Enum|Equal(Enum) (Utilities|Struct|BreakSTRUCT_Missions _returnvalue) "NewEnumerator0")
        (Variables|Default|SetLocationChildHandled (Variables|Default|GetBP_Location_Coastal))
        (bind _asbp_location (Utilities|Casting|CastToBP_Location (Variables|/Script/Engine.ChildActorComponent|GetChildActor (Variables|Default|GetLocationChildHandled)) :!label _label))
        (return _asbp_location)
        (elif (Utilities|Enum|Equal(Enum) (Utilities|Struct|BreakSTRUCT_Missions _returnvalue) "NewEnumerator1")
          (Variables|Default|SetLocationChildHandled (Variables|Default|GetBP_Location_Station))
          (goto _label)
          (elif (Utilities|Enum|Equal(Enum) (Utilities|Struct|BreakSTRUCT_Missions _returnvalue) "NewEnumerator2")
            (Variables|Default|SetLocationChildHandled (Variables|Default|GetBP_Location_Glacier))
            (goto _label)
            (elif (Utilities|Enum|Equal(Enum) (Utilities|Struct|BreakSTRUCT_Missions _returnvalue) "NewEnumerator8")
              (Variables|Default|SetLocationChildHandled (Variables|Default|GetBP_Location_Facility))
              (goto _label)
              (elif (Utilities|Enum|Equal(Enum) (Utilities|Struct|BreakSTRUCT_Missions _returnvalue) "NewEnumerator4")
                (Variables|Default|SetLocationChildHandled (Variables|Default|GetBP_Location_Shipyard))
                (goto _label)
                (elif (Utilities|Enum|Equal(Enum) (Utilities|Struct|BreakSTRUCT_Missions _returnvalue) "NewEnumerator5")
                  (Variables|Default|SetLocationChildHandled (Variables|Default|GetBP_Location_Skeletons))
                  (goto _label)
                  (elif (Utilities|Enum|Equal(Enum) (Utilities|Struct|BreakSTRUCT_Missions _returnvalue) "NewEnumerator9")
                    (Variables|Default|SetLocationChildHandled (Variables|Default|GetBP_Location_Drill))
                    (goto _label)
                    (elif (Utilities|Enum|Equal(Enum) (Utilities|Struct|BreakSTRUCT_Missions _returnvalue) "NewEnumerator6")
                      (Variables|Default|SetLocationChildHandled (Variables|Default|GetBP_Location_Inferno))
                      (goto _label)
                      (elif (Utilities|Enum|Equal(Enum) (Utilities|Struct|BreakSTRUCT_Missions _returnvalue) "NewEnumerator7")
                        (Variables|Default|SetLocationChildHandled (Variables|Default|GetBP_Location_Fortress))
                        (goto _label)
                        (elif (Utilities|Enum|Equal(Enum) (Utilities|Struct|BreakSTRUCT_Missions _returnvalue) "NewEnumerator3")
                          (Variables|Default|SetLocationChildHandled (Variables|Default|GetBP_Location_Experiment))
                          (goto _label)
                          (elif (Utilities|Enum|Equal(Enum) (Utilities|Struct|BreakSTRUCT_Missions _returnvalue) "NewEnumerator10")
                            (Variables|Default|SetLocationChildHandled (Variables|Default|GetBP_Location_Ocean))
                            (goto _label)
                            (elif (Utilities|Enum|Equal(Enum) (Utilities|Struct|BreakSTRUCT_Missions _returnvalue) "NewEnumerator11")
                              (Variables|Default|SetLocationChildHandled (Variables|Default|GetBP_Location_Capital))
                              (goto _label))))))))))))))))
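; BP_FlightDeck is the flight deck actor, which slides its left and right control hatches open when play begins.
; A HatchesOpen timeline starts on BeginPlay and uses its track as an alpha to lerp each hatch's world location.
; Both hatches move from a shared closed-position marker component to their own open-position markers, without sweep.
; The construction script is empty.
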(event EventBeginPlay
  (bind _hatchesclosedpos (Variables|Default|GetHatchesClosedPos))
  (bind _newtrack_1 (Timeline|HatchesOpen Play)
    (:Update
      (Utilities|FlowControl|Sequence
        (:then_0
          (Transformation|SetWorldLocation (Variables|Default|GetControlHatchesLeft) (Math|Vector|Lerp(Vector) (Transformation|GetWorldLocation _hatchesclosedpos) (Transformation|GetWorldLocation (Variables|Default|GetHatchesLeftOpenPos)) _newtrack_1) false false))
        (:then_1
          (Transformation|SetWorldLocation (Variables|Default|GetControlHatchesRight) (Math|Vector|Lerp(Vector) (Transformation|GetWorldLocation _hatchesclosedpos) (Transformation|GetWorldLocation (Variables|Default|GetHatchesRightOpenPos)) _newtrack_1) false false))))))

(fn ConstructionScript)
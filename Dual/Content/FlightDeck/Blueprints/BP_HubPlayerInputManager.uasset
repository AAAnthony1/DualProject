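; Possessable player input handler for the hub that drives the main menu, ship select and shop.
; On first possession it binds to GAMEMODE_Hub to set the hub camera view and track hub state.
; State checks route scroll, confirm, back and vertical camera input to the game mode or LoaderTrack, which handles ship selection and rotation.
; Gates with Delays throttle scrolling and alternate confirm and back in ship select and shop.
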(event Custom|ShipSelectAllowInput
  (params (Allow :type Boolean))
  ;[1 1 1] Ship Select Move
  (if Allow
    (Utilities|FlowControl|Sequence
      (:then_0
        (Utilities|FlowControl|Gate false) ; enters at Open
      )
      (:then_1
        (Utilities|FlowControl|Gate false) ; enters at Open
      ))
    (else
      (Utilities|FlowControl|Sequence
        (:then_0
          (Utilities|FlowControl|Gate false) ; enters at Close
        )
        (:then_1
          (Utilities|FlowControl|Gate false) ; enters at Close
        )))))

(event Custom|ShopBack
  (bind _player (Variables|Default|GetPlayer))
  (bind _gamemodehub (Variables|Default|GetGamemodeHub))
  ;[1 1 1] Ship Select Confirm or Cancel
  (Utilities|FlowControl|Sequence
    (:then_0
      (Utilities|FlowControl|Gate true
        (:Exit
          (Default|ShopSelectionEntered _gamemodehub false _player))))
    (:then_1
      (Utilities|FlowControl|Gate false) ; enters at Close
    )
    (:then_2
      (Utilities|FlowControl|Delay 0.5)
      (Utilities|FlowControl|Gate false) ; enters at Open
    )))

(event Custom|MainMenuScrollVertical
  (params (AxisValue :type Float%20%28single-precision%29))
  ;[1 1 1] Main Menu Move
  (Math|Float|CompareFloat AxisValue 0.75
    (:>
      (Utilities|FlowControl|Gate false
        (:Exit
          (CallFunction|MainMenuAllowInput false)
          (Variables|Default|SetMainMenuMoveDown false))))
    (:<
      (Math|Float|CompareFloat AxisValue -0.75
        (:<
          (Utilities|FlowControl|Gate false
            (:Exit
              (CallFunction|MainMenuAllowInput false)
              (Variables|Default|SetMainMenuMoveDown true)))))))
  (bind _asgamemode_hub (Utilities|Casting|CastToGAMEMODE_Hub (Game|GetGameMode)))
  (Default|MainMenuSelectionChanged _asgamemode_hub (Variables|Default|GetMainMenuMoveDown))
  (Utilities|FlowControl|Delay 0.25)
  (CallFunction|MainMenuAllowInput true))

(event Custom|ShipSelectScrollVertical
  (params (AxisValue :type Float%20%28single-precision%29))
  ;[1 1 1] Ship Select Move
  (Math|Float|CompareFloat AxisValue 0.75
    (:>
      (Utilities|FlowControl|Gate false
        (:Exit
          (CallFunction|ShipSelectAllowInput false)
          (Variables|Default|SetShipSelectMoveDown false))))
    (:<
      (Math|Float|CompareFloat AxisValue -0.75
        (:<
          (Utilities|FlowControl|Gate false
            (:Exit
              (CallFunction|ShipSelectAllowInput false)
              (Variables|Default|SetShipSelectMoveDown true)))))))
  (Default|ChangeSelection (Variables|Default|GetLoaderTrack) (Variables|Default|GetShipSelectMoveDown))
  (Utilities|FlowControl|Delay 0.5)
  (CallFunction|ShipSelectAllowInput true))

(event Custom|ShopAllowInput
  (params (Allow :type Boolean))
  ;[1 1 1] Shop Move
  (if Allow
    (Utilities|FlowControl|Sequence
      (:then_0
        (Utilities|FlowControl|Gate false) ; enters at Open
      )
      (:then_1
        (Utilities|FlowControl|Gate false) ; enters at Open
      ))
    (else
      (Utilities|FlowControl|Sequence
        (:then_0
          (Utilities|FlowControl|Gate false) ; enters at Close
        )
        (:then_1
          (Utilities|FlowControl|Gate false) ; enters at Close
        )))))

(event Custom|ShopScrollVertical
  (params (AxisValue :type Float%20%28single-precision%29))
  ;[1 1 1] Shop Move
  (Math|Float|CompareFloat AxisValue 0.75
    (:>
      (Utilities|FlowControl|Gate false
        (:Exit
          (CallFunction|ShopAllowInput false)
          (Variables|Default|SetShopMenuMoveDown false))))
    (:<
      (Math|Float|CompareFloat AxisValue -0.75
        (:<
          (Utilities|FlowControl|Gate false
            (:Exit
              (CallFunction|ShopAllowInput false)
              (Variables|Default|SetShopMenuMoveDown true)))))))
  (bind _asgamemode_hub (Utilities|Casting|CastToGAMEMODE_Hub (Game|GetGameMode)))
  (Default|ShopSelectionChanged _asgamemode_hub (Variables|Default|GetShopMenuMoveDown) (Variables|Default|GetPlayer))
  (Utilities|FlowControl|Delay 0.1)
  (CallFunction|ShopAllowInput true))

(event Custom|MainMenuConfirm
  ;[1 1 1] Main Menu Confirm
  (bind _asgamemode_hub (Utilities|Casting|CastToGAMEMODE_Hub (Game|GetGameMode)))
  (Default|MainMenuButtonClicked _asgamemode_hub))

(event Custom|MainMenuAllowInput
  (params (Allow :type Boolean))
  ;[1 1 1] Main Menu Move
  (if Allow
    (Utilities|FlowControl|Sequence
      (:then_0
        (Utilities|FlowControl|Gate false) ; enters at Open
      )
      (:then_1
        (Utilities|FlowControl|Gate false) ; enters at Open
      ))
    (else
      (Utilities|FlowControl|Sequence
        (:then_0
          (Utilities|FlowControl|Gate false) ; enters at Close
        )
        (:then_1
          (Utilities|FlowControl|Gate false) ; enters at Close
        )))))

(event Custom|ControllersSet
  ;[1 1 1] Set Camera
  (Game|Player|SetViewTargetwithBlend (Game|GetPlayerController 0) (Variables|Default|GetBP_HubCamera) 0.0 "VTBlend_Linear" 0.0 false))

(event Custom|HubStateHasChanged
  (params (State :type ENUM_HubState%20Enum :default "NewEnumerator1"))
  ;[1 1 1] Track Hub State from the Hub Gamemode
  (Variables|Default|SetHubState State))

(event Custom|ShipSelectConfirm
  (bind _loadertrack (Variables|Default|GetLoaderTrack))
  ;[1 1 1] Ship Select Confirm or Cancel
  (Utilities|FlowControl|Sequence
    (:then_0
      (Utilities|FlowControl|Gate false
        (:Exit
          (Default|ShipSelectPlayerReady _loadertrack true))))
    (:then_1
      (Utilities|FlowControl|Gate true) ; enters at Close
    )
    (:then_2
      (Utilities|FlowControl|Delay 0.5)
      (Utilities|FlowControl|Gate true) ; enters at Open
    )))

(event Custom|ShipSelectBack
  (bind _loadertrack (Variables|Default|GetLoaderTrack))
  ;[1 1 1] Ship Select Confirm or Cancel
  (Utilities|FlowControl|Sequence
    (:then_0
      (Utilities|FlowControl|Gate true
        (:Exit
          (Default|ShipSelectPlayerReady _loadertrack false))))
    (:then_1
      (Utilities|FlowControl|Gate false) ; enters at Close
    )
    (:then_2
      (Utilities|FlowControl|Delay 0.5)
      (Utilities|FlowControl|Gate false) ; enters at Open
    )))

(event Custom|ShopConfirm
  (bind _player (Variables|Default|GetPlayer))
  (bind _gamemodehub (Variables|Default|GetGamemodeHub))
  ;[1 1 1] Ship Select Confirm or Cancel
  (Utilities|FlowControl|Sequence
    (:then_0
      (Utilities|FlowControl|Gate false
        (:Exit
          (Default|ShopSelectionEntered _gamemodehub true _player))))
    (:then_1
      (Utilities|FlowControl|Gate true) ; enters at Close
    )
    (:then_2
      (Utilities|FlowControl|Delay 0.5)
      (Utilities|FlowControl|Gate true) ; enters at Open
    )))

(event EventPossessed
  (params (NewController :type Controller%20Object%20Reference))
  ;[1 1 1] Set Camera
  (Utilities|FlowControl|DoOnce false
    (:Completed
      (bind _asgamemode_hub (Utilities|Casting|CastToGAMEMODE_Hub (Game|GetGameMode)))
      (bind _output_get (Variables|Default|SetGamemodeHub _asgamemode_hub))
      (EventDispatchers|BindEventtoHubPlayerControllersSet _output_get (delegate Custom|ControllersSet))
      ;[1 1 1] Track Hub State from the Hub Gamemode
      (EventDispatchers|BindEventtoHubStateChanged (Variables|Default|GetGamemodeHub) (delegate Custom|HubStateHasChanged)))))

(event Input|ActionEvents|InputActionMenuConfirm
  (params (Key :type Key%20Structure))
  ;[1 1 1] Inputs
  (:Pressed
    (Utilities|CheckHubState "NewEnumerator1"
      (:True
        (CallFunction|MainMenuConfirm))
      (:False
        (Utilities|CheckHubState "NewEnumerator2"
          (:True
            (CallFunction|ShipSelectConfirm))
          (:False
            (Utilities|CheckHubState "NewEnumerator5"
              (:True
                (CallFunction|ShopConfirm)))))))))

(event Input|ActionEvents|InputActionMenuBack
  (params (Key :type Key%20Structure))
  ;[1 1 1] Inputs
  (:Pressed
    (Utilities|CheckHubState "NewEnumerator2"
      (:True
        (CallFunction|ShipSelectBack))
      (:False
        (Utilities|CheckHubState "NewEnumerator5"
          (:True
            (CallFunction|ShopBack)))))))

(event Input|AxisEvents|InputAxisMenuScrollVertical
  (params (AxisValue :type Float%20%28single-precision%29))
  ;[1 1 1] Inputs
  (Utilities|CheckHubState "NewEnumerator1"
    (:True
      (CallFunction|MainMenuScrollVertical AxisValue))
    (:False
      (Utilities|CheckHubState "NewEnumerator2"
        (:True
          (CallFunction|ShipSelectScrollVertical AxisValue))
        (:False
          (Utilities|CheckHubState "NewEnumerator5"
            (:True
              (CallFunction|ShopScrollVertical AxisValue))))))))

(event Input|AxisEvents|InputAxisMenuCameraHorizontal
  (params (AxisValue :type Float%20%28single-precision%29))
  ;[1 1 1] Ship Select Camera movement
)

(event Input|AxisEvents|InputAxisMenuCameraVertical
  (params (AxisValue :type Float%20%28single-precision%29))
  ;[1 1 1] Ship Select Camera movement
  (Utilities|CheckHubState "NewEnumerator2"
    (:True
      (Default|OrientateShip (Variables|Default|GetLoaderTrack) AxisValue (stale Input|AxisEvents|InputAxisMenuCameraHorizontal AxisValue)))))

(fn ConstructionScript)
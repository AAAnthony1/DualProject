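; BP_Hub is the flight deck hub Blueprint that runs map selection and travel to the chosen campaign location.
; OpenMapSelect sets the hub state, shows the solar map child actor and opens the map select widget with UI-only input.
; On selection, it removes the widget, restores game input and opens the level named after GAMEMODE_Campaign's CurrentLocation enum.
; Face and special button handlers check HubState but perform no actions.
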(event Custom|OpenMapSelect
  (bind _returnvalue (Game|GetPlayerController 0))
  ;[1 1 1] Map Select
  (Variables|Default|SetHubState "NewEnumerator3")
  (bind _asbp_solar_map (Utilities|Casting|CastToBP_SolarMap (Variables|/Script/Engine.ChildActorComponent|GetChildActor (Variables|Default|GetBP_SolarMap))))
  (Default|ShowSolarMap _asbp_solar_map true)
  (bind _returnvalue_2 (UserInterface|CreateWidget "/Game/FlightDeck/Widgets/WID_MapSelect.WID_MapSelect_C"))
  (bind _output_get (Variables|Default|SetWIDMapSelect _returnvalue_2))
  (UserInterface|Viewport|AddtoViewport _output_get 0)
  (Input|SetInputModeUIOnly _returnvalue (Variables|/Game/FlightDeck/Widgets/WID_MapSelect.WID_MapSelect_C|GetConfirmButton _output_get) "DoNotLock")
  (Variables|/Script/Engine.PlayerController|SetbShowMouseCursor _returnvalue true)
  (EventDispatchers|BindEventtoMapSelected (Variables|Default|GetWIDMapSelect) (delegate Custom|MapSelected)))

(event Custom|LoadMap
  ;[1 1 1] Load Map
  (bind _asgamemode_campaign (Utilities|Casting|CastToGAMEMODE_Campaign (Game|GetGameMode)))
  (Development|PrintString (Utilities|String|EnumtoString (Variables|/Game/Gamemodes/GAMEMODE_Campaign.GAMEMODE_Campaign_C|GetCurrentLocation _asgamemode_campaign)))
  (Input|SetInputModeGameOnly (Game|GetPlayerController 0))
  (Game|OpenLevel(byName) (Utilities|String|StringToName (Utilities|String|EnumtoString (Variables|/Game/Gamemodes/GAMEMODE_Campaign.GAMEMODE_Campaign_C|GetCurrentLocation _asgamemode_campaign)))))

(event Custom|MapSelected
  ;[1 1 1] Map Select
  (Widget|RemovefromParent (Variables|Default|GetWIDMapSelect))
  (CallFunction|LoadMap))

(fn ConstructionScript)
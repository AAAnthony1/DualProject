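; BP_Location is a FlightDeck location marker with a sphere and a widget label showing its display name.
; The construction script swaps the sphere for a child actor when a custom model Blueprint class is set.
; BeginPlay hides the sphere and widget, then passes the name to WID_LocationDetails.
; ShowLocation toggles sphere and widget visibility, and HideLabel drives the widget's text fade.
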(event Custom|ShowLocation
  (params (Show :type Boolean))
  ;[1 1 1] Show Location
  (Rendering|SetVisibility (Variables|Default|GetSphere) Show false))

(event Custom|HideLabel
  (params (True :type Boolean))
  (Default|FadeText (Variables|Default|GetLocationDetailsWidget) True))

(event EventBeginPlay
  ;[1 1 1] Set Location Name
  (Rendering|SetVisibility (Variables|Default|GetSphere) false false)
  (bind _aswid_location_details (Utilities|Casting|CastToWID_LocationDetails (UserInterface|GetUserWidgetObject (Variables|Default|GetWidget))))
  (bind _output_get (Variables|Default|SetLocationDetailsWidget _aswid_location_details))
  (Default|SetDetails _output_get (Variables|Default|GetLocationDisplayName)))

(fn ConstructionScript
  (bind _sphere (Variables|Default|GetSphere))
  (if (Utilities|IsValidClass (Variables|Default|GetLocationModelBlueprint))
    (Rendering|SetVisibility _sphere false false)
    (Development|SetHiddeninGame _sphere true false)
    (ChildActorComponent|SetChildActorClass (Variables|Default|GetLocationBlueprint) (Variables|Default|GetLocationModelBlueprint))))
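; Power Bomb superweapon actor that flies out, soaks up power from projectiles that hit it, then explodes.
; A timeline sweeps it between launch and detonation points while valid hits, filtered through the weapons interface and faction check, add attack power to its charge.
; Charge drives mesh scale plus the color and glow of a dynamic material.
; After a fixed delay, a second timeline expands the mesh by absorbed power, then destroys the actor.
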(event OnComponentHit(PowerbombMesh)
  (params (HitComponent :type Primitive%20Component%20Object%20Reference) (OtherActor :type Actor%20Object%20Reference) (OtherComp :type Primitive%20Component%20Object%20Reference) (NormalImpulse :type Vector :default "0, 0, 0") (Hit :type Hit%20Result%20Structure%20%28by%20ref%29))
  (if (Utilities|DoesObjectImplementInterface OtherActor "/Game/Weaponry/BPI_WeaponsInterface.BPI_WeaponsInterface_C")
    (bind (_attackpower _validtargetslist) (Class|BPIWeaponsInterface|ProjectileGetHitInfo(Message) OtherActor))
    (Utilities|CheckValidTarget (Utilities|Struct|MakeSTRUCT_Factions false false false false true) _validtargetslist
      (:ValidTarget
        (Variables|Default|SetPowerPercentageAbsorbed (Math|Float|Clamp(Float) (+ (* (Math|Conversions|ToFloat(Integer) _attackpower) 0.005) (Variables|Default|GetPowerPercentageAbsorbed))))
        (bind _output_get (Variables|Default|SetChargeScale (Math|Float|Lerp 1e+01 1e+02 (Variables|Default|GetPowerPercentageAbsorbed))))
        (Transformation|SetWorldScale3D (Variables|Default|GetPowerbombMesh) (Math|Vector|MakeVector _output_get _output_get _output_get))
        (Rendering|Material|SetVectorParameterValue (Variables|Default|GetMaterial) "Color" (Math|Color|Lerp(LinearColor) (Variables|Default|GetColorLowPower) (Variables|Default|GetColorHighPower) (Variables|Default|GetPowerPercentageAbsorbed)) :!class /Script/Engine.MaterialInstanceDynamic)
        (Rendering|Material|SetScalarParameterValue (Variables|Default|GetMaterial) "Emissive" (Math|Float|Clamp(Float) (* (Variables|Default|GetPowerPercentageAbsorbed) 1e+03) 1.0 1e+03) :!class /Script/Engine.MaterialInstanceDynamic)))))

(event Custom|Move
  (bind _fly (Timeline|FlyForward PlayFromStart)
    (:Update
      (Transformation|SetActorLocation (Math|Vector|Lerp(Vector) (Transformation|GetWorldLocation (Variables|Default|GetLaunchPoint)) (Transformation|GetWorldLocation (Variables|Default|GetDetonationPoint)) (Math|Float|Clamp(Float) _fly)) true false))))

(event EventBeginPlay
  (Utilities|FlowControl|Sequence
    (:then_0
      (CallFunction|Move)
      (bind _returnvalue (Rendering|Material|CreateDynamicMaterialInstance (Variables|Default|GetPowerbombMesh) 0 "/Game/Superweapons/PowerBomb/M_Powerbomb.M_Powerbomb" :!class /Script/Engine.PrimitiveComponent))
      (bind _output_get (Variables|Default|SetMaterial _returnvalue))
      (Rendering|Material|SetVectorParameterValue _output_get "Color" (Variables|Default|GetColorLowPower) :!class /Script/Engine.MaterialInstanceDynamic)
      (Rendering|Material|SetScalarParameterValue (Variables|Default|GetMaterial) "Emissive" 1.0 :!class /Script/Engine.MaterialInstanceDynamic))
    (:then_1
      (Utilities|FlowControl|Delay 5.0)
      (bind _expand (Timeline|Explode PlayFromStart)
        (:Update
          (Variables|Default|SetExplosionScale (* (Math|Float|Lerp 1.0 5.0 (Variables|Default|GetPowerPercentageAbsorbed)) (Math|Float|Lerp 1e+01 1.5e+02 _expand)))
          (Transformation|SetWorldScale3D (Variables|Default|GetPowerbombMesh) (Math|Vector|MakeVector (Variables|Default|GetExplosionScale) (Variables|Default|GetExplosionScale) (Variables|Default|GetExplosionScale))))
        (:Finished
          (Actor|DestroyActor))))))

(fn ConstructionScript)
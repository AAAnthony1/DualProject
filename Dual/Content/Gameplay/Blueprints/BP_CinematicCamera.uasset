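; BP_CinematicCamera is a cinematic camera actor that plays an intro-style Level Sequence and then hands the view to the twin aircraft rig.
; LookThroughCinematicCamera makes it the player's view target and plays the assigned sequence.
; When the sequence finishes, a timeline lerps its root from the exit transform to the BP_TwinAircraftRig camera, then calls PossessTwinRigCamera for a seamless handoff.
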(event Custom|LookThroughCinematicCamera
  (bind _levelsequence (Variables|Default|GetLevelSequence))
  (bind _sequenceplayer (Variables|/Script/LevelSequence.LevelSequenceActor|GetSequencePlayer _levelsequence))
  (Game|Player|SetViewTargetwithBlend (Game|GetPlayerController 0) self 0.0 "VTBlend_Linear" 0.0 false)
  (Utilities|IsValid _levelsequence
    (:Is%20Valid
      (Sequencer|Player|Play _sequenceplayer :!class /Script/MovieScene.MovieSceneSequencePlayer)
      (EventDispatchers|AssignOnFinished _sequenceplayer (delegate Custom|SequencerFinished)))))

(event Custom|SequencerFinished
  (bind _outactors (Actor|GetAllActorsOfClass "/Game/Gameplay/Blueprints/BP_TwinAircraftRig.BP_TwinAircraftRig_C"))
  (Variables|Default|SetTwinRig (Utilities|Array|Get(acopy) _outactors))
  (Variables|Default|SetCameraSequencerExitTransform (Transformation|GetActorTransform self))
  (bind _lerp (Timeline|Lerp PlayFromStart)
    (:Update
      (Transformation|SetWorldTransform (Variables|Default|GetDefaultSceneRoot self) (Math|Transform|Lerp(Transform) (Variables|Default|GetCameraSequencerExitTransform) (Transformation|GetWorldTransform (Variables|/Game/Gameplay/Blueprints/BP_TwinAircraftRig.BP_TwinAircraftRig_C|GetCamera (Variables|Default|GetTwinRig))) _lerp) false false))
    (:Finished
      (Default|PossessTwinRigCamera (Variables|Default|GetTwinRig)))))

(fn ConstructionScript)
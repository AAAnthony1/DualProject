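; BP_Obstacle is a configurable static mesh obstacle that can register as dynamic collision with the DoN flight navigation manager for flying AI.
; The construction script applies the chosen mesh, if valid, and its scale.
; When flagged dynamic, a looping timer started on BeginPlay schedules collision updates for the mesh with the manager, with optional debug drawing.
; The update result handler is empty.
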(event Custom|DynamicPulseResultHandler
  (params (bTaskSuccessful :type Boolean)))

(event Custom|DynamicCollisionUpdater
  (Class|DonNavigationManager|ScheduleDynamicCollisionUpdate (Variables|Default|GetAI_Flight_Nav_Manager) (Variables|Default|GetStaticMesh) (delegate Custom|DynamicPulseResultHandler) "None" false false false false 1.0 false (Variables|Obstacle|GetDrawDebug)))

(event EventBeginPlay
  (Variables|Default|SetAI_Flight_Nav_Manager (Class|DonNavigationHelper|DonNavigationManager))
  (if (Variables|Obstacle|GetIsDynamic)
    (Utilities|Time|SetTimerbyEvent (delegate Custom|DynamicCollisionUpdater) (Variables|Obstacle|GetDynCollisionPulse) true)))

(fn ConstructionScript
  (Utilities|IsValid (Variables|Obstacle|GetObstacleMesh)
    (:Is%20Valid
      (Components|StaticMesh|SetStaticMesh (Variables|Default|GetStaticMesh) (Variables|Obstacle|GetObstacleMesh)))
    (:Is%20Not%20Valid
      _))
  (Transformation|SetRelativeScale3D (Variables|Default|GetStaticMesh) (Variables|Obstacle|GetMeshScale)))
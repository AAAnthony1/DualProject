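; BP_TwinAircraftRig is a camera rig for two aircraft that rides along BP_Flightpath actors.
; Its construction script offsets the P1 and P2 centre points to opposite sides by DistanceFromCentre.
; On BeginPlay it has the flightpath flagged as starting attach the rig, then makes itself player 0's view target.
; SetPostProcessing swaps the camera between Sky and Underwater post-process settings, applying the default type at start.
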(event EventBeginPlay
  (bind _outactors (Actor|GetAllActorsOfClass "/Game/Gameplay/Blueprints/BP_Flightpath.BP_Flightpath_C"))
  (for _array_element _outactors
    (if (Variables|/Game/Gameplay/Blueprints/BP_Flightpath.BP_Flightpath_C|GetStartingFlightpath _array_element)
      (Default|AttachTwinRig _array_element)
      (Game|Player|SetViewTargetwithBlend (Game|GetPlayerController 0) self 0.0 "VTBlend_Linear" 0.0 false)
      (CallFunction|SetPostProcessing (Variables|Default|GetDefaultPostProcessType)))))

(fn ConstructionScript
  (bind _distancefromcentre (Variables|Default|GetDistanceFromCentre))
  (Utilities|FlowControl|Sequence
    (:then_0
      (Transformation|AddLocalOffset (Variables|Default|GetP1Centrepoint) (Math|Vector|MakeVector 0.0 (* _distancefromcentre -1.0) 0.0) false false))
    (:then_1
      (Transformation|AddLocalOffset (Variables|Default|GetP2Centrepoint) (Math|Vector|MakeVector 0.0 _distancefromcentre 0.0) false false))))

(fn SetPostProcessing
  (params (PostProcessType :type ENUM_PostProcessTypes%20Enum :default "NewEnumerator0"))
  (bind _camera (Variables|Default|GetCamera))
  (switch Utilities|FlowControl|Switch|SwitchonENUM_PostProcessTypes PostProcessType
    (:NewEnumerator0
      (Variables|/Script/Engine.CameraComponent|SetPostProcessSettings _camera (Variables|Default|GetPostProcessSettingsSky)))
    (:NewEnumerator5
      (Variables|/Script/Engine.CameraComponent|SetPostProcessSettings _camera (Variables|Default|GetPostProcessSettingsUnderwater)))))
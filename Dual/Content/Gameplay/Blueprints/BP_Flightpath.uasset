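; BP_Flightpath is a spline path that flies the level's BP_TwinAircraftRig along its length.
; AttachTwinRig finds the rig, resets distance and starts a self-repeating 1/60-second Delay loop that advances by Speed, sweeping the rig to each spline transform.
; At the end, a resettable DoOnce fires the ReachedPathEnd dispatcher once.
; The construction script optionally places evenly spaced static meshes along the spline.
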(event Custom|AttachTwinRig
  (bind _spline (Variables|Default|GetSpline))
  (bind _outactors (Actor|GetAllActorsOfClass "/Game/Gameplay/Blueprints/BP_TwinAircraftRig.BP_TwinAircraftRig_C"))
  (Utilities|IsValid (Utilities|Array|Get(acopy) _outactors)
    (:Is%20Valid
      (Variables|Default|SetTwinRig (Utilities|Array|Get(acopy) _outactors))
      (CallFunction|ResetEndCall)
      (Variables|Default|SetCurrentDistanceAlongSpline 0.0)
      (Transformation|SetActorLocationAndRotation (Variables|Default|GetTwinRig) (Spline|GetLocationatDistanceAlongSpline _spline (Variables|Default|GetCurrentDistanceAlongSpline) "World") (Spline|GetRotationatDistanceAlongSpline _spline (Variables|Default|GetCurrentDistanceAlongSpline) "World") true)
      (Math|Float|CompareFloat (Variables|Default|GetCurrentDistanceAlongSpline) (Spline|GetSplineLength (Variables|Default|GetSpline))
        (:>
          (Utilities|FlowControl|DoOnce false :!label _label
            (:Completed
              (Default|CallReachedPathEnd))))
        (:==
          (goto _label))
        (:<
          (Utilities|FlowControl|Delay (/ 1.0 6e+01))
          (CallFunction|UpdateTwinRigAlongSpline))))))

(event Custom|UpdateTwinRigAlongSpline
  (bind _spline (Variables|Default|GetSpline))
  (Variables|Default|SetCurrentDistanceAlongSpline (+ (Variables|Default|GetCurrentDistanceAlongSpline) (Variables|Default|GetSpeed)))
  (Transformation|SetActorLocationAndRotation (Variables|Default|GetTwinRig) (Spline|GetLocationatDistanceAlongSpline _spline (Variables|Default|GetCurrentDistanceAlongSpline) "World") (Spline|GetRotationatDistanceAlongSpline _spline (Variables|Default|GetCurrentDistanceAlongSpline) "World") true)
  (Math|Float|CompareFloat (Variables|Default|GetCurrentDistanceAlongSpline) (Spline|GetSplineLength (Variables|Default|GetSpline))
    (:>
      (Utilities|FlowControl|DoOnce false :!label _label
        (:Completed
          (Default|CallReachedPathEnd))))
    (:==
      (goto _label))
    (:<
      (Utilities|FlowControl|Delay (/ 1.0 6e+01))
      (CallFunction|UpdateTwinRigAlongSpline))))

(event Custom|ResetEndCall
  (Utilities|FlowControl|DoOnce false) ; enters at Reset
)

(fn ConstructionScript
  (if (Variables|Default|GetSpawnSplineMeshes)
    (for _index (range (Variables|Default|Get0) (.ReturnValue (Math|Float|Division(WholeandRemainder) (Spline|GetSplineLength (Variables|Default|GetSpline)) (Variables|Default|GetSpacing))))
      (bind _returnvalue (AddComponent|AddStaticMeshComponent false (Math|Transform|MakeTransform (Spline|GetLocationatDistanceAlongSpline (Variables|Default|GetSpline) (* _index (Variables|Default|GetSpacing)) "Local") (Spline|GetRotationatDistanceAlongSpline (Variables|Default|GetSpline) (* _index (Variables|Default|GetSpacing)) "Local"))))
      (Utilities|Array|Add (Variables|Default|GetSplineMeshes) _returnvalue))))
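; Cinematic intro camera actor that plays a level sequence and then hands the view over to the twin aircraft rig's camera.
; LookThroughCinematicCamera makes it the view target, plays the sequence, waits a set delay, then uses a timeline to lerp its root transform toward the rig camera.
; When the blend finishes, the rig takes camera possession and the mission intro banner widget is added to the viewport.
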(event Custom|LookThroughCinematicCamera
  (bind _levelsequence (Variables|Default|GetLevelSequence))
  (Game|Player|SetViewTargetwithBlend (Game|GetPlayerController 0) self 0.0 "VTBlend_Linear" 0.0 false)
  (Utilities|IsValid _levelsequence
    (:Is%20Valid
      (Sequencer|Player|Play (Variables|/Script/LevelSequence.LevelSequenceActor|GetSequencePlayer _levelsequence) :!class /Script/MovieScene.MovieSceneSequencePlayer)
      (Utilities|FlowControl|Delay (Variables|Default|GetDelayForTransferCamera))
      (bind _outactors (Actor|GetAllActorsOfClass "/Game/Gameplay/Blueprints/BP_TwinAircraftRig.BP_TwinAircraftRig_C"))
      (Variables|Default|SetTwinRig (Utilities|Array|Get(acopy) _outactors))
      (Variables|Default|SetCameraSequencerExitTransform (Transformation|GetActorTransform self))
      (bind _lerp (Timeline|Lerp PlayFromStart)
        (:Update
          (Transformation|SetWorldTransform (Variables|Default|GetDefaultSceneRoot self) (Math|Transform|Lerp(Transform) (Variables|Default|GetCameraSequencerExitTransform) (Transformation|GetWorldTransform (Variables|/Game/Gameplay/Blueprints/BP_TwinAircraftRig.BP_TwinAircraftRig_C|GetCamera (Variables|Default|GetTwinRig))) _lerp) false false))
        (:Finished
          (Default|PossessTwinRigCamera (Variables|Default|GetTwinRig))
          (bind _returnvalue (UserInterface|CreateWidget "/Game/Gamemodes/WID_MissionIntro.WID_MissionIntro_C"))
          (Default|SetMissionBanner _returnvalue)
          (UserInterface|Viewport|AddtoViewport _returnvalue 0))))))

(fn ConstructionScript)
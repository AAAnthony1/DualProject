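; LIB_CommonFunctions is a Blueprint library of shared gameplay helpers for value wrapping and player colors.
; Integer and float functions wrap an input around a range, returning the minimum when it exceeds the maximum and the maximum when it falls below the minimum.
; The wrap snaps to the opposite bound and discards any overshoot.
; GetPlayerColors returns fixed Slate colors, blue for player one and orange for player two.
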(fn SetIntegerWithinLoopingRange
  (params (IntInput :type Integer) (IntMinValue :type Integer) (IntMaxValue :type Integer))
  (Math|Integer|CompareInt IntInput IntMinValue
    (:>
      (Math|Integer|CompareInt IntInput IntMaxValue
        (:>
          (LocalVariables|SetIntHandled IntMinValue))
        (:==
          (LocalVariables|SetIntHandled IntInput :!label _label))
        (:<
          (goto _label))))
    (:==
      (goto _label))
    (:<
      (LocalVariables|SetIntHandled IntMaxValue)))
  (return (LocalVariables|GetIntHandled)))

(fn SetFloatWithinLoopingRange
  (params (FloatInput :type Float%20%28single-precision%29) (FloatMinValue :type Float%20%28single-precision%29) (FloatMaxValue :type Float%20%28single-precision%29))
  (Math|Float|CompareFloat FloatInput FloatMinValue
    (:>
      (Math|Float|CompareFloat FloatInput FloatMaxValue
        (:>
          (LocalVariables|SetFloatHandled FloatMinValue))
        (:==
          (LocalVariables|SetFloatHandled FloatInput :!label _label))
        (:<
          (goto _label))))
    (:==
      (goto _label))
    (:<
      (LocalVariables|SetFloatHandled FloatMaxValue)))
  (return (LocalVariables|GetFloatHandled)))

(fn GetPlayerColors
  (return (Utilities|Struct|MakeSlateColor "(R=0.000000,G=0.564712,B=1.000000,A=1.000000)") (Utilities|Struct|MakeSlateColor "(R=1.000000,G=0.283149,B=0.000000,A=1.000000)")))
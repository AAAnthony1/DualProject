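; Four-part sliding reactor door for the Battleship boss, opened and closed through the ChangeDoorState event.
; The MoveDoorParts timeline plays from the start to open and reverses from the end to close.
; Its Sides track slides the left and right meshes apart on Y, while its BottomAndTop track moves the bottom and top meshes apart on Z.
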(event Custom|ChangeDoorState
  (params (Open :type Boolean))
  (if Open
    (bind (_direction _bottomandtop _sides) (Timeline|MoveDoorParts PlayFromStart)
      (:Update
        (Transformation|SetRelativeLocation (Variables|Default|GetSM_BattleshipReactorDoorSideLeft) (Math|Vector|MakeVector 0.0 (* _sides -7e+02) 0.0) false false)
        (Transformation|SetRelativeLocation (Variables|Default|GetSM_BattleshipReactorDoorSideRight) (Math|Vector|MakeVector 0.0 (* _sides 7e+02) 0.0) false false)
        (Transformation|SetRelativeLocation (Variables|Default|GetSM_BattleshipReactorDoorBottom) (Math|Vector|MakeVector 0.0 0.0 (* _bottomandtop -7.5e+02)) false false)
        (Transformation|SetRelativeLocation (Variables|Default|GetSM_BattleshipReactorDoorTop) (Math|Vector|MakeVector 0.0 0.0 (* _bottomandtop 7.5e+02)) false false)))
    (else
      (Timeline|MoveDoorParts ReverseFromEnd))))

(fn ConstructionScript)
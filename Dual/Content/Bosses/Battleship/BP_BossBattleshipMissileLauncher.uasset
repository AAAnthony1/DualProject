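; Battleship boss missile launcher that acts as a destructible part of the boss.
; On play it takes the damageable component from a child actor and binds to its hit and destroyed events.
; Hits are converted to a health fraction and broadcast, and destruction awards score for the launcher's unit type.
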(event Custom|Hit
  (params (CurrentHitpoints :type Integer))
  (Default|CallHitHealthPercent (/ (Math|Conversions|ToFloat(Integer) CurrentHitpoints) (Math|Conversions|ToFloat(Integer) (Variables|/Game/Units/Blueprints/BP_DamageableComponent.BP_DamageableComponent_C|GetTotalHitpoints (Variables|Default|GetLauncher))))))

(event Custom|MissileLauncherDestroyed
  (params (HullComponent :type BP%20Damageable%20Component%20Object%20Reference))
  (Utilities|UnitDestroyedAwardScore "NewEnumerator32" self))

(event EventBeginPlay
  (bind _asbp_damageable_component (Utilities|Casting|CastToBP_DamageableComponent (Variables|/Script/Engine.ChildActorComponent|GetChildActor (Variables|Default|GetBP_DamageableComponent))))
  (bind _output_get (Variables|Default|SetLauncher _asbp_damageable_component))
  (EventDispatchers|BindEventtoHit _output_get (delegate Custom|Hit))
  (EventDispatchers|BindEventtoDamageableComponentDestroyed _asbp_damageable_component (delegate Custom|MissileLauncherDestroyed)))

(fn ConstructionScript)
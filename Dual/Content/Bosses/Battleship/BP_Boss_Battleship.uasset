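; Battleship boss actor that runs a two-stage fight: an orbit chase, then a reactor attack.
; When triggered, the chase shows a health bar averaging twelve turrets and four missile launchers, while randomly timed left/right evasion sequences play.
; Once those weapons are destroyed, it polls until evasion ends, calls the rear door open, and awaits reactor entry.
; The bar then tracks two pylons' pooled hitpoints; a separate event explodes and hides the boss.
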(event Custom|DestroyTheBoss
  ;[1 1 1] Destroy Boss
  (Utilities|DestroyBoss))

(event Custom|Turret12Percent
  (params (HealthPercent :type Float%20%28single-precision%29))
  (Variables|Default|SetTurret12HealthPercent HealthPercent)
  (CallFunction|CalculateBattleshipRearWeaponsHealth))

(event Custom|BindEnteredReactorTrigger
  (EventDispatchers|BindEventtoTriggered (Variables|Default|GetTriggerEnteredReactor) (delegate Custom|EnteredReactors)))

(event Custom|Launcher03Percent
  (params (HitHealthPercent :type Float%20%28single-precision%29))
  (Variables|Default|SetLauncher03HealthPercent HitHealthPercent)
  (CallFunction|CalculateBattleshipRearWeaponsHealth))

(event Custom|Launcher04Percent
  (params (HitHealthPercent :type Float%20%28single-precision%29))
  (Variables|Default|SetLauncher04HealthPercent HitHealthPercent)
  (CallFunction|CalculateBattleshipRearWeaponsHealth))

(event Custom|CalculateBattleshipRearWeaponsHealth
  (bind _output_get (Variables|Default|SetAllRearWeaponsCombinedPercent (/ (+ (Variables|Default|GetTurret01HealthPercent) (Variables|Default|GetTurret02HealthPercent) (Variables|Default|GetTurret03HealthPercent) (Variables|Default|GetTurret04HealthPercent) (Variables|Default|GetTurret05HealthPercent) (Variables|Default|GetTurret06HealthPercent) (Variables|Default|GetTurret07HealthPercent) (Variables|Default|GetTurret08HealthPercent) (Variables|Default|GetTurret09HealthPercent) (Variables|Default|GetTurret10HealthPercent) (Variables|Default|GetTurret11HealthPercent) (Variables|Default|GetTurret12HealthPercent) (Variables|Default|GetLauncher01HealthPercent) (Variables|Default|GetLauncher02HealthPercent) (Variables|Default|GetLauncher03HealthPercent) (Variables|Default|GetLauncher04HealthPercent)) 16.0)))
  (Utilities|FlowControl|Sequence
    (:then_0
      (Default|UpdateBossHealth (Variables|Default|GetWID_BossHealthBar) _output_get))
    (:then_1
      (Math|Float|CompareFloat _output_get 0.0
        (:==
          _)
        (:<
          _))
      (Utilities|FlowControl|DoOnce false
        (:Completed
          (Variables|Default|SetOrbitChasePhase false)
          (Utilities|FlowControl|Delay 1.0)
          (Widget|RemovefromParent (Variables|Default|GetWID_BossHealthBar))
          (if (Variables|Default|GetOrbitChaseEvading)
            (Utilities|FlowControl|Delay 0.5)
            (CallFunction|CallOpenDoorAgain)
            (else
              (Default|CallOpenRearDoor)
              (CallFunction|BindEnteredReactorTrigger))))))))

(event Custom|Turret11Percent
  (params (HealthPercent :type Float%20%28single-precision%29))
  (Variables|Default|SetTurret11HealthPercent HealthPercent)
  (CallFunction|CalculateBattleshipRearWeaponsHealth))

(event Custom|ForeReactorHit
  (params (CurrentHitpoints :type Integer))
  ;[1 1 1] Track Reactor Health
  (Variables|Default|SetForeReactorCurrentHealth CurrentHitpoints)
  (CallFunction|UpdateBossHealthBar))

(event Custom|OrbitEvasive
  (bind _orbitevaderight (Variables|Default|GetOrbitEvadeRight))
  (bind _orbitevadeleft (Variables|Default|GetOrbitEvadeLeft))
  (bind _sequenceplayer (Variables|/Script/LevelSequence.LevelSequenceActor|GetSequencePlayer _orbitevadeleft))
  (bind _sequenceplayer_2 (Variables|/Script/LevelSequence.LevelSequenceActor|GetSequencePlayer _orbitevaderight))
  (if (Variables|Default|GetOrbitChasePhase)
    (Utilities|FlowControl|Delay (Math|Random|RandomFloatinRange 0.0 8.0))
    (if (Variables|Default|GetOrbitChasePhase)
      (Variables|Default|SetOrbitChaseEvading true)
      (Utilities|FlowControl|Sequence
        (:then_0
          (goto _label Reset))
        (:then_1
          (Utilities|FlowControl|MultiGate true false -1 :!label _label
            (:Out%200
              (Components|Timeline|SetPlaybackPosition _sequenceplayer 0.0)
              (Sequencer|Player|Play _sequenceplayer :!class /Script/MovieScene.MovieSceneSequencePlayer))
            (:Out%201
              (Components|Timeline|SetPlaybackPosition _sequenceplayer_2 0.0)
              (Sequencer|Player|Play _sequenceplayer_2 :!class /Script/MovieScene.MovieSceneSequencePlayer))))
        (:then_2
          (Utilities|FlowControl|Delay 2e+01)
          (Variables|Default|SetOrbitChaseEvading false)
          (CallFunction|OrbitEvasive))))))

(event Custom|AftReactorHit
  (params (CurrentHitpoints :type Integer))
  ;[1 1 1] Track Reactor Health
  (Variables|Default|SetAftReactorCurrentHealth CurrentHitpoints)
  (CallFunction|UpdateBossHealthBar))

(event Custom|Turret09Percent
  (params (HealthPercent :type Float%20%28single-precision%29))
  (Variables|Default|SetTurret09HealthPercent HealthPercent)
  (CallFunction|CalculateBattleshipRearWeaponsHealth))

(event Custom|Turret10Percent
  (params (HealthPercent :type Float%20%28single-precision%29))
  (Variables|Default|SetTurret10HealthPercent HealthPercent)
  (CallFunction|CalculateBattleshipRearWeaponsHealth))

(event Custom|CallOpenDoorAgain
  (if (Variables|Default|GetOrbitChaseEvading)
    (Utilities|FlowControl|Delay 0.5)
    (CallFunction|CallOpenDoorAgain)
    (else
      (Default|CallOpenRearDoor)
      (CallFunction|BindEnteredReactorTrigger))))

(event Custom|Turret01Percent
  (params (HealthPercent :type Float%20%28single-precision%29))
  (Variables|Default|SetTurret01HealthPercent HealthPercent)
  (CallFunction|CalculateBattleshipRearWeaponsHealth))

(event Custom|Turret02Percent
  (params (HealthPercent :type Float%20%28single-precision%29))
  (Variables|Default|SetTurret02HealthPercent HealthPercent)
  (CallFunction|CalculateBattleshipRearWeaponsHealth))

(event Custom|Turret03Percent
  (params (HealthPercent :type Float%20%28single-precision%29))
  (Variables|Default|SetTurret03HealthPercent HealthPercent)
  (CallFunction|CalculateBattleshipRearWeaponsHealth))

(event Custom|Turret04Percent
  (params (HealthPercent :type Float%20%28single-precision%29))
  (Variables|Default|SetTurret04HealthPercent HealthPercent)
  (CallFunction|CalculateBattleshipRearWeaponsHealth))

(event Custom|UpdateBossHealthBar
  ;[1 1 1] Track Reactor Health
  (Default|UpdateBossHealth (Variables|Default|GetWID_BossHealthBar) (/ (Math|Conversions|ToFloat(Integer) (+ (Variables|Default|GetForeReactorCurrentHealth) (Variables|Default|GetAftReactorCurrentHealth))) (Math|Conversions|ToFloat(Integer) (Variables|Default|GetReactorTotalHitPool)))))

(event Custom|FollowingBattleship
  (Variables|Default|SetOrbitChasePhase true)
  (Utilities|FlowControl|Sequence
    (:then_0
      (bind _returnvalue (UserInterface|CreateWidget "/Game/Bosses/Common/WID_BossHealthBar.WID_BossHealthBar_C"))
      (bind _output_get (Variables|Default|SetWID_BossHealthBar _returnvalue))
      (UserInterface|Viewport|AddtoViewport _output_get 0))
    (:then_1
      (CallFunction|OrbitEvasive))))

(event Custom|Launcher02Percent
  (params (HitHealthPercent :type Float%20%28single-precision%29))
  (Variables|Default|SetLauncher02HealthPercent HitHealthPercent)
  (CallFunction|CalculateBattleshipRearWeaponsHealth))

(event Custom|Launcher01Percent
  (params (HitHealthPercent :type Float%20%28single-precision%29))
  (Variables|Default|SetLauncher01HealthPercent HitHealthPercent)
  (CallFunction|CalculateBattleshipRearWeaponsHealth))

(event Custom|Turret05Percent
  (params (HealthPercent :type Float%20%28single-precision%29))
  (Variables|Default|SetTurret05HealthPercent HealthPercent)
  (CallFunction|CalculateBattleshipRearWeaponsHealth))

(event Custom|Turret06Percent
  (params (HealthPercent :type Float%20%28single-precision%29))
  (Variables|Default|SetTurret06HealthPercent HealthPercent)
  (CallFunction|CalculateBattleshipRearWeaponsHealth))

(event Custom|Turret07Percent
  (params (HealthPercent :type Float%20%28single-precision%29))
  (Variables|Default|SetTurret07HealthPercent HealthPercent)
  (CallFunction|CalculateBattleshipRearWeaponsHealth))

(event Custom|Turret08Percent
  (params (HealthPercent :type Float%20%28single-precision%29))
  (Variables|Default|SetTurret08HealthPercent HealthPercent)
  (CallFunction|CalculateBattleshipRearWeaponsHealth))

(event Custom|EnteredReactors
  (bind _wid_bosshealthbar (Variables|Default|GetWID_BossHealthBar))
  ;[1 1 1] Track Reactor Health
  (bind _asbp_boss_battleship_reactor_pylon (Utilities|Casting|CastToBP_Boss_Battleship_ReactorPylon (Variables|/Script/Engine.ChildActorComponent|GetChildActor (Variables|Default|GetReactorPylon_Fore))))
  (EventDispatchers|BindEventtoReactorTakenHit _asbp_boss_battleship_reactor_pylon (delegate Custom|ForeReactorHit))
  (Variables|Default|SetForeReactorCurrentHealth (Variables|/Game/Bosses/Battleship/BP_Boss_Battleship_ReactorPylon.BP_Boss_Battleship_ReactorPylon_C|GetTotalHitpoints _asbp_boss_battleship_reactor_pylon))
  (Variables|Default|SetReactorTotalHitPool (Variables|/Game/Bosses/Battleship/BP_Boss_Battleship_ReactorPylon.BP_Boss_Battleship_ReactorPylon_C|GetTotalHitpoints _asbp_boss_battleship_reactor_pylon))
  (bind _asbp_boss_battleship_reactor_pylon_2 (Utilities|Casting|CastToBP_Boss_Battleship_ReactorPylon (Variables|/Script/Engine.ChildActorComponent|GetChildActor (Variables|Default|GetReactorPylon_Aft))))
  (EventDispatchers|BindEventtoReactorTakenHit _asbp_boss_battleship_reactor_pylon_2 (delegate Custom|AftReactorHit))
  (Variables|Default|SetAftReactorCurrentHealth (Variables|/Game/Bosses/Battleship/BP_Boss_Battleship_ReactorPylon.BP_Boss_Battleship_ReactorPylon_C|GetTotalHitpoints _asbp_boss_battleship_reactor_pylon_2))
  (Variables|Default|SetReactorTotalHitPool (+ (Variables|/Game/Bosses/Battleship/BP_Boss_Battleship_ReactorPylon.BP_Boss_Battleship_ReactorPylon_C|GetTotalHitpoints _asbp_boss_battleship_reactor_pylon_2) (Variables|Default|GetReactorTotalHitPool)))
  (Default|UpdateBossHealth _wid_bosshealthbar 1.0)
  (UserInterface|Viewport|AddtoViewport _wid_bosshealthbar 0))

(event EventBeginPlay
  (EventDispatchers|BindEventtoTriggered (Variables|Default|GetTriggerFollowingBattleship) (delegate Custom|FollowingBattleship))
  (Utilities|FlowControl|Sequence
    (:then_0
      (bind _asbp_boss_battleship_turret (Utilities|Casting|CastToBP_Boss_Battleship_Turret (Variables|/Script/Engine.ChildActorComponent|GetChildActor (Variables|Default|GetTurret01))))
      (EventDispatchers|BindEventtoHitHealthPercent _asbp_boss_battleship_turret (delegate Custom|Turret01Percent)))
    (:then_1
      (bind _asbp_boss_battleship_turret_2 (Utilities|Casting|CastToBP_Boss_Battleship_Turret (Variables|/Script/Engine.ChildActorComponent|GetChildActor (Variables|Default|GetTurret02))))
      (EventDispatchers|BindEventtoHitHealthPercent _asbp_boss_battleship_turret_2 (delegate Custom|Turret02Percent)))
    (:then_2
      (bind _asbp_boss_battleship_turret_3 (Utilities|Casting|CastToBP_Boss_Battleship_Turret (Variables|/Script/Engine.ChildActorComponent|GetChildActor (Variables|Default|GetTurret03))))
      (EventDispatchers|BindEventtoHitHealthPercent _asbp_boss_battleship_turret_3 (delegate Custom|Turret03Percent)))
    (:then_3
      (bind _asbp_boss_battleship_turret_4 (Utilities|Casting|CastToBP_Boss_Battleship_Turret (Variables|/Script/Engine.ChildActorComponent|GetChildActor (Variables|Default|GetTurret04))))
      (EventDispatchers|BindEventtoHitHealthPercent _asbp_boss_battleship_turret_4 (delegate Custom|Turret04Percent)))
    (:then_4
      (bind _asbp_boss_battleship_turret_5 (Utilities|Casting|CastToBP_Boss_Battleship_Turret (Variables|/Script/Engine.ChildActorComponent|GetChildActor (Variables|Default|GetTurret05))))
      (EventDispatchers|BindEventtoHitHealthPercent _asbp_boss_battleship_turret_5 (delegate Custom|Turret05Percent)))
    (:then_5
      (bind _asbp_boss_battleship_turret_6 (Utilities|Casting|CastToBP_Boss_Battleship_Turret (Variables|/Script/Engine.ChildActorComponent|GetChildActor (Variables|Default|GetTurret06))))
      (EventDispatchers|BindEventtoHitHealthPercent _asbp_boss_battleship_turret_6 (delegate Custom|Turret06Percent)))
    (:then_6
      (bind _asbp_boss_battleship_turret_7 (Utilities|Casting|CastToBP_Boss_Battleship_Turret (Variables|/Script/Engine.ChildActorComponent|GetChildActor (Variables|Default|GetTurret07))))
      (EventDispatchers|BindEventtoHitHealthPercent _asbp_boss_battleship_turret_7 (delegate Custom|Turret07Percent)))
    (:then_7
      (bind _asbp_boss_battleship_turret_8 (Utilities|Casting|CastToBP_Boss_Battleship_Turret (Variables|/Script/Engine.ChildActorComponent|GetChildActor (Variables|Default|GetTurret08))))
      (EventDispatchers|BindEventtoHitHealthPercent _asbp_boss_battleship_turret_8 (delegate Custom|Turret08Percent)))
    (:then_8
      (bind _asbp_boss_battleship_turret_9 (Utilities|Casting|CastToBP_Boss_Battleship_Turret (Variables|/Script/Engine.ChildActorComponent|GetChildActor (Variables|Default|GetTurret09))))
      (EventDispatchers|BindEventtoHitHealthPercent _asbp_boss_battleship_turret_9 (delegate Custom|Turret09Percent)))
    (:then_9
      (bind _asbp_boss_battleship_turret_10 (Utilities|Casting|CastToBP_Boss_Battleship_Turret (Variables|/Script/Engine.ChildActorComponent|GetChildActor (Variables|Default|GetTurret10))))
      (EventDispatchers|BindEventtoHitHealthPercent _asbp_boss_battleship_turret_10 (delegate Custom|Turret10Percent)))
    (:then_10
      (bind _asbp_boss_battleship_turret_11 (Utilities|Casting|CastToBP_Boss_Battleship_Turret (Variables|/Script/Engine.ChildActorComponent|GetChildActor (Variables|Default|GetTurret11))))
      (EventDispatchers|BindEventtoHitHealthPercent _asbp_boss_battleship_turret_11 (delegate Custom|Turret11Percent)))
    (:then_11
      (bind _asbp_boss_battleship_turret_12 (Utilities|Casting|CastToBP_Boss_Battleship_Turret (Variables|/Script/Engine.ChildActorComponent|GetChildActor (Variables|Default|GetTurret12))))
      (EventDispatchers|BindEventtoHitHealthPercent _asbp_boss_battleship_turret_12 (delegate Custom|Turret12Percent)))
    (:then_12
      (bind _asbp_boss_battleship_missile_launcher (Utilities|Casting|CastToBP_BossBattleshipMissileLauncher (Variables|/Script/Engine.ChildActorComponent|GetChildActor (Variables|Default|GetLauncher01))))
      (EventDispatchers|BindEventtoHitHealthPercent _asbp_boss_battleship_missile_launcher (delegate Custom|Launcher01Percent)))
    (:then_13
      (bind _asbp_boss_battleship_missile_launcher_2 (Utilities|Casting|CastToBP_BossBattleshipMissileLauncher (Variables|/Script/Engine.ChildActorComponent|GetChildActor (Variables|Default|GetLauncher02))))
      (EventDispatchers|BindEventtoHitHealthPercent _asbp_boss_battleship_missile_launcher_2 (delegate Custom|Launcher02Percent)))
    (:then_14
      (bind _asbp_boss_battleship_missile_launcher_3 (Utilities|Casting|CastToBP_BossBattleshipMissileLauncher (Variables|/Script/Engine.ChildActorComponent|GetChildActor (Variables|Default|GetLauncher03))))
      (EventDispatchers|BindEventtoHitHealthPercent _asbp_boss_battleship_missile_launcher_3 (delegate Custom|Launcher03Percent)))
    (:then_15
      (bind _asbp_boss_battleship_missile_launcher_4 (Utilities|Casting|CastToBP_BossBattleshipMissileLauncher (Variables|/Script/Engine.ChildActorComponent|GetChildActor (Variables|Default|GetLauncher04))))
      (EventDispatchers|BindEventtoHitHealthPercent _asbp_boss_battleship_missile_launcher_4 (delegate Custom|Launcher04Percent)))))

(fn ConstructionScript)
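; Battleship boss turret actor whose body and barrel are separate damageable child actors that act as one shared health pool.
; On BeginPlay it binds to both parts' hit and destroyed events, and a hit on either copies its hitpoints to the other and broadcasts the health percentage, based on the body's total.
; Destruction of either part removes the whole turret after a short delay, guarded to run once.
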(event Custom|BodyHit
  (params (CurrentHitpoints :type Integer))
  (Default|OverrideCurrentHealth (Variables|Default|GetTurretBarrel) CurrentHitpoints)
  (Default|CallHitHealthPercent (/ (Math|Conversions|ToFloat(Integer) CurrentHitpoints) (Math|Conversions|ToFloat(Integer) (Variables|Default|GetTotalHealth)))))

(event Custom|BodyDestroyed
  (params (HullComponent :type BP%20Damageable%20Component%20Object%20Reference))
  (CallFunction|TurretDestroyed))

(event Custom|BarrelDestroyed
  (params (HullComponent :type BP%20Damageable%20Component%20Object%20Reference))
  (CallFunction|TurretDestroyed))

(event Custom|TurretDestroyed
  (Utilities|FlowControl|DoOnce false
    (:Completed
      (Utilities|FlowControl|Delay 2.0)
      (Actor|DestroyActor))))

(event Custom|BarrelHit
  (params (CurrentHitpoints :type Integer))
  (Default|OverrideCurrentHealth (Variables|Default|GetTurretBody) CurrentHitpoints)
  (Default|CallHitHealthPercent (/ (Math|Conversions|ToFloat(Integer) CurrentHitpoints) (Math|Conversions|ToFloat(Integer) (Variables|Default|GetTotalHealth)))))

(event EventBeginPlay
  (bind _asbp_damageable_component (Utilities|Casting|CastToBP_DamageableComponent (Variables|/Script/Engine.ChildActorComponent|GetChildActor (Variables|Default|GetBP_DamageableComponent_TurretBody))))
  (Variables|Default|SetTurretBody _asbp_damageable_component)
  (Variables|Default|SetTotalHealth (Variables|/Game/Units/Blueprints/BP_DamageableComponent.BP_DamageableComponent_C|GetTotalHitpoints _asbp_damageable_component))
  (EventDispatchers|BindEventtoHit _asbp_damageable_component (delegate Custom|BodyHit))
  (EventDispatchers|BindEventtoDestroyed _asbp_damageable_component (delegate Custom|BodyDestroyed))
  (bind _asbp_damageable_component_2 (Utilities|Casting|CastToBP_DamageableComponent (Variables|/Script/Engine.ChildActorComponent|GetChildActor (Variables|Default|GetBP_DamageableComponent_TurretBarrel))))
  (Variables|Default|SetTurretBarrel _asbp_damageable_component_2)
  (EventDispatchers|BindEventtoHit _asbp_damageable_component_2 (delegate Custom|BarrelHit))
  (EventDispatchers|BindEventtoDestroyed _asbp_damageable_component_2 (delegate Custom|BarrelDestroyed)))

(fn ConstructionScript)
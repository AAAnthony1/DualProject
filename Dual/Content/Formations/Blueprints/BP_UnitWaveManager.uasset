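; BP_UnitWaveManager spawns a wave of unit formations at its spline once a linked Trigger fires.
; It walks the Formations array in order, using an entry delay per formation and an instance delay before each repeated spawn.
; Each spawned formation is told to move along the spline, at either a shared consistent speed or its own configured speed.
; Sequencing runs through chained events and delays with counters instead of a loop.
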(event Custom|ContinueSpawningFormations
  (bind _formations (Variables|Default|GetFormations))
  (bind _formationtospawn (Variables|Default|GetFormationToSpawn))
  (bind _item (Utilities|Array|Get(acopy) _formations _formationtospawn))
  (bind (_formation _entrydelay _speed _instances _instancedelay) (Utilities|Struct|BreakSTRUCT_FormationWaveData _item))
  (Utilities|FlowControl|Delay _entrydelay)
  (Variables|Default|SetInstanceHandled 1)
  (Variables|Default|SetTotalInstances _instances)
  (Utilities|FlowControl|Delay _instancedelay)
  (bind _returnvalue (Game|SpawnActorfromClass _formation (Transformation|GetWorldTransform (Variables|Default|GetSpline)) "Undefined" 0 0))
  (if (Variables|Default|GetConsistentSpeed)
    (Variables|Default|SetFormationSpeed (Variables|Default|GetConsistentSpeedValue))
    (else
      (Variables|Default|SetFormationSpeed _speed)))
  (Default|MoveFormationAlongSpline _returnvalue self (Variables|Default|GetFormationSpeed))
  (Math|Integer|CompareInt (Variables|Default|GetInstanceHandled) (Variables|Default|GetTotalInstances)
    (:==
      (bind _result (Math|Integer|IncrementInt (Variables|Default|GetFormationToSpawn))
        (:%20%20
          (Math|Integer|CompareInt _result (Variables|Default|GetTotalFormationsInWave)
            (:<
              (CallFunction|ContinueSpawningFormations))))))
    (:<
      (Math|Integer|IncrementInt (Variables|Default|GetInstanceHandled)
        (:%20%20
          (CallFunction|ContinueSpawningInstances))))))

(event Custom|ContinueSpawningInstances
  (bind _formations (Variables|Default|GetFormations))
  (bind _formationtospawn (Variables|Default|GetFormationToSpawn))
  (bind _item (Utilities|Array|Get(acopy) _formations _formationtospawn))
  (bind (_formation _entrydelay _speed _instances _instancedelay) (Utilities|Struct|BreakSTRUCT_FormationWaveData _item))
  (Utilities|FlowControl|Delay _instancedelay)
  (bind _returnvalue (Game|SpawnActorfromClass _formation (Transformation|GetWorldTransform (Variables|Default|GetSpline)) "Undefined" 0 0))
  (if (Variables|Default|GetConsistentSpeed)
    (Variables|Default|SetFormationSpeed (Variables|Default|GetConsistentSpeedValue))
    (else
      (Variables|Default|SetFormationSpeed _speed)))
  (Default|MoveFormationAlongSpline _returnvalue self (Variables|Default|GetFormationSpeed))
  (Math|Integer|CompareInt (Variables|Default|GetInstanceHandled) (Variables|Default|GetTotalInstances)
    (:==
      (bind _result (Math|Integer|IncrementInt (Variables|Default|GetFormationToSpawn))
        (:%20%20
          (Math|Integer|CompareInt _result (Variables|Default|GetTotalFormationsInWave)
            (:<
              (CallFunction|ContinueSpawningFormations))))))
    (:<
      (Math|Integer|IncrementInt (Variables|Default|GetInstanceHandled)
        (:%20%20
          (CallFunction|ContinueSpawningInstances))))))

(event Custom|BeginSpawningFormation
  (bind _formations (Variables|Default|GetFormations))
  (bind _formationtospawn (Variables|Default|GetFormationToSpawn))
  (bind _item (Utilities|Array|Get(acopy) _formations _formationtospawn))
  (bind (_formation _entrydelay _speed _instances _instancedelay) (Utilities|Struct|BreakSTRUCT_FormationWaveData _item))
  (Variables|Default|SetTotalFormationsInWave (Utilities|Array|Length _formations))
  (Utilities|FlowControl|Delay _entrydelay)
  (Variables|Default|SetInstanceHandled 1)
  (Variables|Default|SetTotalInstances _instances)
  (Utilities|FlowControl|Delay _instancedelay)
  (bind _returnvalue (Game|SpawnActorfromClass _formation (Transformation|GetWorldTransform (Variables|Default|GetSpline)) "Undefined" 0 0))
  (if (Variables|Default|GetConsistentSpeed)
    (Variables|Default|SetFormationSpeed (Variables|Default|GetConsistentSpeedValue))
    (else
      (Variables|Default|SetFormationSpeed _speed)))
  (Default|MoveFormationAlongSpline _returnvalue self (Variables|Default|GetFormationSpeed))
  (Math|Integer|CompareInt (Variables|Default|GetInstanceHandled) (Variables|Default|GetTotalInstances)
    (:==
      (bind _result (Math|Integer|IncrementInt (Variables|Default|GetFormationToSpawn))
        (:%20%20
          (Math|Integer|CompareInt _result (Variables|Default|GetTotalFormationsInWave)
            (:<
              (CallFunction|ContinueSpawningFormations))))))
    (:<
      (Math|Integer|IncrementInt (Variables|Default|GetInstanceHandled)
        (:%20%20
          (CallFunction|ContinueSpawningInstances))))))

(event EventBeginPlay
  (bind _trigger (Variables|Default|GetTrigger))
  (Utilities|IsValid _trigger
    (:Is%20Valid
      (EventDispatchers|BindEventtoTriggered _trigger (delegate Custom|BeginSpawningFormation)))))

(fn ConstructionScript)
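; BP_Spawner spawns a configured unit when its Trigger fires or Spawn is called, and can destroy it via CullUnits.
; Unit data supplies the Blueprint class to spawn and a preview mesh added by the construction script.
; The spawned unit attaches to SpawnLocation.
; For warp-ins, SpawnLocation jumps far back along local X, then a timeline animates it, carrying the unit along.
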(event Custom|CullUnits
  (params (AwardScore :type Boolean))
  (Actor|DestroyActor (Variables|Default|GetSpawnedUnit)))

(event Custom|Spawn
  (params (WarpIn :type Boolean))
  (bind _output_get (Variables|Default|SetWarpedIn WarpIn))
  (if _output_get
    (Transformation|SetRelativeLocation (Variables|Default|GetSpawnLocation) "-100000.000000, 0, 0" false false))
  (bind _unitdata (Utilities|GetUnitData (Variables|Default|GetUnitToSpawn))
    (:Done
      (bind _returnvalue (Game|SpawnActorfromClass (.UnitBlueprintClass (Utilities|Struct|BreakSTRUCT_UnitData _unitdata)) (Transformation|GetWorldTransform (Variables|Default|GetSpawnLocation)) "Undefined" 0 0))
      (Variables|Default|SetSpawnedUnit _returnvalue)
      (Transformation|AttachComponentToComponent (Variables|Default|GetSpawnedUnit) (Variables|Default|GetSpawnLocation) "None" "SnapToTarget" "SnapToTarget" "KeepWorld" true)
      (if (Variables|Default|GetWarpedIn)
        (bind _newtrack_0 (Timeline|WarpIn PlayFromStart)
          (:Update
            (Transformation|SetRelativeLocation (Variables|Default|GetSpawnLocation) (Math|Vector|MakeVector _newtrack_0 0.0 0.0) false false)))))))

(event Custom|SpawnViaTrigger
  (bind _output_get (Variables|Default|SetWarpedIn (stale Custom|Spawn WarpIn)))
  (if _output_get
    (Transformation|SetRelativeLocation (Variables|Default|GetSpawnLocation) "-100000.000000, 0, 0" false false))
  (bind _unitdata (Utilities|GetUnitData (Variables|Default|GetUnitToSpawn))
    (:Done
      (bind _returnvalue (Game|SpawnActorfromClass (.UnitBlueprintClass (Utilities|Struct|BreakSTRUCT_UnitData _unitdata)) (Transformation|GetWorldTransform (Variables|Default|GetSpawnLocation)) "Undefined" 0 0))
      (Variables|Default|SetSpawnedUnit _returnvalue)
      (Transformation|AttachComponentToComponent (Variables|Default|GetSpawnedUnit) (Variables|Default|GetSpawnLocation) "None" "SnapToTarget" "SnapToTarget" "KeepWorld" true)
      (if (Variables|Default|GetWarpedIn)
        (bind _newtrack_0 (Timeline|WarpIn PlayFromStart)
          (:Update
            (Transformation|SetRelativeLocation (Variables|Default|GetSpawnLocation) (Math|Vector|MakeVector _newtrack_0 0.0 0.0) false false)))))))

(event EventBeginPlay
  (EventDispatchers|BindEventtoTriggered (Variables|Default|GetTrigger) (delegate Custom|SpawnViaTrigger)))

(fn ConstructionScript
  (bind _unitdata (Utilities|GetUnitData (Variables|Default|GetUnitToSpawn))
    (:Done
      (bind _returnvalue (AddComponent|AddStaticMeshComponent false))
      (Components|StaticMesh|SetStaticMesh _returnvalue (.UnitPreviewMesh (Utilities|Struct|BreakSTRUCT_UnitData _unitdata))))))
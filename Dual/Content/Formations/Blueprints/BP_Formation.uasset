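; BP_Formation is a formation actor that groups BP_Spawner child actors and moves along a wave manager's spline.
; MoveFormationAlongSpline starts the spline movement at the given speed, then tells each spawner in its child actor components to spawn, passing the WarpIn flag.
; When the movement reaches the path end, it calls CullUnits on every child spawner.
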(event Custom|MoveFormationAlongSpline
  (params (WaveManager :type BP%20Unit%20Wave%20Manager%20Object%20Reference) (Speed :type Float%20%28single-precision%29) (WarpIn :type Boolean))
  (Variables|Default|SetWarpIn WarpIn)
  (Utilities|FlowControl|Sequence
    (:then_0
      (Utilities|MoveAlongSpline 0 (Variables|/Game/Formations/Blueprints/BP_UnitWaveManager.BP_UnitWaveManager_C|GetSpline WaveManager) Speed
        (:ReachedPathEnd
          (for _array_element (Actor|GetAllChildActors true)
            (bind _asbp_spawner (Utilities|Casting|CastToBP_Spawner _array_element))
            (Default|CullUnits _asbp_spawner false)))))
    (:then_1
      (for _array_element_2 (Components|GetChildrenComponents (Variables|Default|GetDefaultSceneRoot) true)
        (bind _aschild_actor_component (Utilities|Casting|CastToChildActorComponent _array_element_2))
        (bind _asbp_spawner_2 (Utilities|Casting|CastToBP_Spawner (Variables|/Script/Engine.ChildActorComponent|GetChildActor _aschild_actor_component)))
        (Default|Spawn _asbp_spawner_2 (Variables|Default|GetWarpIn))))))

(fn ConstructionScript)
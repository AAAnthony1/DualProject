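; Superweapon pickup that adds its superweapon to the inventory of an overlapping player ship that is not at capacity.
; Collection fires once, playing a pickup sound and a delayed second cue before the actor destroys itself.
; A looping 30 Hz timer spins the icon mesh.
; The construction script tints border and icon through dynamic materials, with all handled color options wired to purple and the other three colors left disconnected.
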(event OnComponentBeginOverlap(Sphere)
  (params (OverlappedComponent :type Primitive%20Component%20Object%20Reference) (OtherActor :type Actor%20Object%20Reference) (OtherComp :type Primitive%20Component%20Object%20Reference) (OtherBodyIndex :type Integer) (bFromSweep :type Boolean) (SweepResult :type Hit%20Result%20Structure%20%28by%20ref%29))
  (bind _asbp_playership (Utilities|Casting|CastToBP_Playership OtherActor))
  (if (not (Variables|/Game/Players/Blueprints/BP_Playership.BP_Playership_C|GetSuperweaponsAtCapacity _asbp_playership))
    (Utilities|FlowControl|DoOnce false
      (:Completed
        (Default|AddSuperWeapontoInventory _asbp_playership (Variables|Default|GetSuperweapon))
        (Audio|PlaySound2D "/Game/Audio/SoundEffects/SC_SuperweaponPickup.SC_SuperweaponPickup")
        (Utilities|FlowControl|Delay 0.5)
        (Audio|PlaySound2D (Variables|Default|GetSoundCue))
        (Actor|DestroyActor)))))

(event Custom|Rotate
  (Transformation|AddWorldRotation (Variables|Default|GetSM_SuperweaponIcon) "0,10.000000, 0" false false))

(event EventBeginPlay
  (Utilities|Time|SetTimerbyEvent (delegate Custom|Rotate) (/ 1.0 3e+01) true))

(fn ConstructionScript
  (bind _color (Variables|Default|GetColor))
  (if (Utilities|Enum|Equal(Enum) _color "NewEnumerator0")
    (Variables|Default|SetIconColor "(R=0.250000,G=0.000000,B=1.000000,A=1.000000)" :!label _label)
    (bind _returnvalue (Rendering|Material|CreateDynamicMaterialInstance (Variables|Default|GetSM_SuperweaponBorder) 0 "/Game/Pickups/Superweapons/M_SuperweaponPickup.M_SuperweaponPickup" :!class /Script/Engine.PrimitiveComponent))
    (Rendering|Material|SetVectorParameterValue _returnvalue "Color" (Variables|Default|GetIconColor) :!class /Script/Engine.MaterialInstanceDynamic)
    (bind _returnvalue_2 (Rendering|Material|CreateDynamicMaterialInstance (Variables|Default|GetSM_SuperweaponIcon) 0 "/Game/Pickups/Superweapons/M_SuperweaponPickup.M_SuperweaponPickup" :!class /Script/Engine.PrimitiveComponent))
    (Rendering|Material|SetVectorParameterValue _returnvalue_2 "Color" (Variables|Default|GetIconColor) :!class /Script/Engine.MaterialInstanceDynamic)
    (elif (Utilities|Enum|Equal(Enum) _color "NewEnumerator1")
      (goto _label)
      (elif (Utilities|Enum|Equal(Enum) _color "NewEnumerator2")
        (goto _label)
        (elif (Utilities|Enum|Equal(Enum) _color "NewEnumerator3")
          (goto _label))))))
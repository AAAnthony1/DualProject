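; Health pickup that heals an overlapping BP_Playership through negative damage, plays a sound and destroys itself.
; The construction script gives six wedge meshes dynamic materials, whose "Filled" parameter displays the award.
; With Cycling on, a self-calling delayed event lights wedges in turn, updates HealthAwarded and clears them after the last, so the reward depends on timing.
; Otherwise, construction fills wedges to match a fixed HealthAwarded.
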(event OnComponentBeginOverlap(Sphere)
  (params (OverlappedComponent :type Primitive%20Component%20Object%20Reference) (OtherActor :type Actor%20Object%20Reference) (OtherComp :type Primitive%20Component%20Object%20Reference) (OtherBodyIndex :type Integer) (bFromSweep :type Boolean) (SweepResult :type Hit%20Result%20Structure%20%28by%20ref%29))
  ;[1 1 1] Award Health when collected
  (bind _asbp_playership (Utilities|Casting|CastToBP_Playership OtherActor))
  (Default|TakeDamage _asbp_playership (* (Variables|Default|GetHealthAwarded) -1))
  (Audio|PlaySound2D "/Game/Audio/SoundEffects/SC_HealthPickup.SC_HealthPickup")
  (Actor|DestroyActor))

(event Custom|ContinueCycling
  (Math|Integer|CompareInt (Variables|Default|GetBlockProcessed) 5
    (:>
      (Variables|Default|SetBlockProcessed 0)
      (for _array_element (Variables|Default|GetMaterialsArray)
        (Rendering|Material|SetScalarParameterValue _array_element "Filled" 0.0 :!class /Script/Engine.MaterialInstanceDynamic)))
    (:==
      _)
    (:<
      _))
  (Rendering|Material|SetScalarParameterValue (Utilities|Array|Get(acopy) (Variables|Default|GetMaterialsArray) (Variables|Default|GetBlockProcessed)) "Filled" 1.0 :!class /Script/Engine.MaterialInstanceDynamic)
  (bind _result (Math|Integer|IncrementInt (Variables|Default|GetBlockProcessed))
    (:%20%20
      (Variables|Default|SetHealthAwarded (+ _result 1))
      (Utilities|FlowControl|Delay (/ 1.0 6.0))
      (CallFunction|ContinueCycling))))

(event EventBeginPlay
  (if (Variables|Default|GetCycling)
    (Math|Integer|CompareInt (Variables|Default|GetBlockProcessed) 5
      (:>
        (Variables|Default|SetBlockProcessed 0)
        (for _array_element (Variables|Default|GetMaterialsArray)
          (Rendering|Material|SetScalarParameterValue _array_element "Filled" 0.0 :!class /Script/Engine.MaterialInstanceDynamic)))
      (:==
        _)
      (:<
        _))
    (Rendering|Material|SetScalarParameterValue (Utilities|Array|Get(acopy) (Variables|Default|GetMaterialsArray) (Variables|Default|GetBlockProcessed)) "Filled" 1.0 :!class /Script/Engine.MaterialInstanceDynamic)
    (bind _result (Math|Integer|IncrementInt (Variables|Default|GetBlockProcessed))
      (:%20%20
        (Variables|Default|SetHealthAwarded (+ _result 1))
        (Utilities|FlowControl|Delay (/ 1.0 6.0))
        (CallFunction|ContinueCycling)))))

(fn ConstructionScript
  (bind _materialsarray (Variables|Default|GetMaterialsArray))
  (Utilities|FlowControl|Sequence
    (:then_0
      (bind _returnvalue (Rendering|Material|CreateDynamicMaterialInstance (Variables|Default|GetSM_HealthWedge1) 0 "/Game/Pickups/Health/M_PickupHealth.M_PickupHealth" :!class /Script/Engine.PrimitiveComponent))
      (bind _output_get (Variables|Default|SetWedge1Material _returnvalue))
      (Utilities|Array|Add _materialsarray _output_get))
    (:then_1
      (bind _returnvalue_2 (Rendering|Material|CreateDynamicMaterialInstance (Variables|Default|GetSM_HealthWedge2) 0 "/Game/Pickups/Health/M_PickupHealth.M_PickupHealth" :!class /Script/Engine.PrimitiveComponent))
      (bind _output_get_2 (Variables|Default|SetWedge2Material _returnvalue_2))
      (Utilities|Array|Add _materialsarray _output_get_2))
    (:then_2
      (bind _returnvalue_3 (Rendering|Material|CreateDynamicMaterialInstance (Variables|Default|GetSM_HealthWedge3) 0 "/Game/Pickups/Health/M_PickupHealth.M_PickupHealth" :!class /Script/Engine.PrimitiveComponent))
      (bind _output_get_3 (Variables|Default|SetWedge3Material _returnvalue_3))
      (Utilities|Array|Add _materialsarray _output_get_3))
    (:then_3
      (bind _returnvalue_4 (Rendering|Material|CreateDynamicMaterialInstance (Variables|Default|GetSM_HealthWedge4) 0 "/Game/Pickups/Health/M_PickupHealth.M_PickupHealth" :!class /Script/Engine.PrimitiveComponent))
      (bind _output_get_4 (Variables|Default|SetWedge4Material _returnvalue_4))
      (Utilities|Array|Add _materialsarray _output_get_4))
    (:then_4
      (bind _returnvalue_5 (Rendering|Material|CreateDynamicMaterialInstance (Variables|Default|GetSM_HealthWedge5) 0 "/Game/Pickups/Health/M_PickupHealth.M_PickupHealth" :!class /Script/Engine.PrimitiveComponent))
      (bind _output_get_5 (Variables|Default|SetWedge5Material _returnvalue_5))
      (Utilities|Array|Add _materialsarray _output_get_5))
    (:then_5
      (bind _returnvalue_6 (Rendering|Material|CreateDynamicMaterialInstance (Variables|Default|GetSM_HealthWedge6) 0 "/Game/Pickups/Health/M_PickupHealth.M_PickupHealth" :!class /Script/Engine.PrimitiveComponent))
      (bind _output_get_6 (Variables|Default|SetWedge6Material _returnvalue_6))
      (Utilities|Array|Add _materialsarray _output_get_6)
      (if (not (Variables|Default|GetCycling))
        (Math|Integer|CompareInt (Variables|Default|GetBlockProcessed) (Variables|Default|GetHealthAwarded) :!label _label
          (:<
            (Rendering|Material|SetScalarParameterValue (Utilities|Array|Get(acopy) (Variables|Default|GetMaterialsArray) (Variables|Default|GetBlockProcessed)) "Filled" 1.0 :!class /Script/Engine.MaterialInstanceDynamic)
            (Math|Integer|IncrementInt (Variables|Default|GetBlockProcessed)
              (:%20%20
                (goto _label)))))))))
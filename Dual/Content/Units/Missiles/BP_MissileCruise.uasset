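; BP_MissileCruise is a cruise missile unit Blueprint that registers and assigns ownership to its damageable hull components.
; On BeginPlay it scans all descendants of the root for Child Actor Components whose actors are BP_DamageableComponent and collects them in AllHullComponents.
; It then sets each component's owner faction struct with both the Players and Colonial flags off.
; No flight, targeting or detonation logic appears in its graphs.
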(event Custom|CreateComponentArray
  (for _array_element (Components|GetChildrenComponents (Variables|Default|GetDefaultSceneRoot) true)
    (bind _aschild_actor_component (Utilities|Casting|CastToChildActorComponent _array_element))
    (bind _asbp_damageable_component (Utilities|Casting|CastToBP_DamageableComponent (Variables|/Script/Engine.ChildActorComponent|GetChildActor _aschild_actor_component)))
    (Utilities|Array|Add (Variables|Default|GetAllHullComponents) _asbp_damageable_component))
  (for _array_element_2 (Variables|Default|GetAllHullComponents)
    (Variables|/Game/Units/Blueprints/BP_DamageableComponent.BP_DamageableComponent_C|SetComponentOwner _array_element_2 (Utilities|Struct|MakeSTRUCT_Factions false false true))))

(event EventBeginPlay
  (CallFunction|CreateComponentArray))

(fn ConstructionScript)
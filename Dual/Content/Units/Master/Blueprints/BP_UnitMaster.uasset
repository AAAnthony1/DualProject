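; BP_UnitMaster, by its name the master unit Blueprint, represents a destructible unit that awards campaign score.
; On BeginPlay it loads its UnitData through GetUnitData using UnitType.
; A hit on the fighter mesh spawns an explosion, adds UnitCreditValue to the score via GAMEMODE_Campaign and destroys the actor.
; DestroyUnit removes it without the explosion, optionally awarding score; both scoring paths destroy it only if the game mode cast succeeds.
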(event OnComponentHit(SM_BasicFighter)
  (params (HitComponent :type Primitive%20Component%20Object%20Reference) (OtherActor :type Actor%20Object%20Reference) (OtherComp :type Primitive%20Component%20Object%20Reference) (NormalImpulse :type Vector :default "0, 0, 0") (Hit :type Hit%20Result%20Structure%20%28by%20ref%29))
  (bind _defaultsceneroot (Variables|Default|GetDefaultSceneRoot))
  (bind _returnvalue (Transformation|GetWorldTransform _defaultsceneroot))
  (bind (_location _rotation) (Math|Transform|BreakTransform _returnvalue))
  (Effects|SpawnEmitteratLocation "/Game/StarterContent/Particles/P_Explosion.P_Explosion" _location _rotation)
  (bind _asgamemode_campaign (Utilities|Casting|CastToGAMEMODE_Campaign (Game|GetGameMode)))
  (Default|UpdateScore _asgamemode_campaign (Utilities|Struct|BreakSTRUCT_UnitData (Variables|Default|GetUnitData)))
  (Actor|DestroyActor))

(event Custom|DestroyUnit
  (params (AwardScore :type Boolean))
  (if AwardScore
    (bind _asgamemode_campaign (Utilities|Casting|CastToGAMEMODE_Campaign (Game|GetGameMode)))
    (Default|UpdateScore _asgamemode_campaign (Utilities|Struct|BreakSTRUCT_UnitData (Variables|Default|GetUnitData))))
  (Actor|DestroyActor))

(event EventBeginPlay
  (bind _unitdata (Utilities|GetUnitData (Variables|Default|GetUnitType))
    (:Done
      (Variables|Default|SetUnitData _unitdata))))

(fn ConstructionScript)
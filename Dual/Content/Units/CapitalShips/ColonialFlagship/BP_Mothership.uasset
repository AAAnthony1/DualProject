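; BP_Mothership is the colonial flagship capital ship, which can start hidden and warp into the scene.
; On BeginPlay, an InitiallyHidden flag sets the visibility of its damageable mesh component.
; WarpIn plays a Warp timeline that reveals the component once, then drives the ShipControl component's relative X location to slide the ship into place.
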(event Custom|WarpIn
  (bind _warp (Timeline|Warp PlayFromStart)
    (:Update
      (Utilities|FlowControl|Sequence
        (:then_0
          (Utilities|FlowControl|DoOnce false
            (:Completed
              (Rendering|SetVisibility (Variables|Default|GetBP_DamageableComponent) true false))))
        (:then_1
          (Transformation|SetRelativeLocation (Variables|Default|GetShipControl) (Math|Vector|MakeVector _warp 0.0 0.0) false false))))))

(event EventBeginPlay
  (bind _bp_damageablecomponent (Variables|Default|GetBP_DamageableComponent))
  (if (Variables|Default|GetInitiallyHidden)
    (Rendering|SetVisibility _bp_damageablecomponent false false)
    (else
      (Rendering|SetVisibility _bp_damageablecomponent true false))))

(fn ConstructionScript)
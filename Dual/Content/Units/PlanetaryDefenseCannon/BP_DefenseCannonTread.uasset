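; Tread piece of the Planetary Defense Cannon unit that displays a wheel number on side-mounted text tags.
; The construction script reads the WheelLocation enum and hides either the left or right tag for the handled locations.
; SetWheelNumberTag writes the given number to both tags as single-digit, ungrouped text, so whichever tag is visible shows it.
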(event Custom|SetWheelNumberTag
  (params (NumberTag :type Integer))
  (Rendering|Components|TextRender|SetText (Variables|Default|GetNumberTagLeft) (Utilities|Text|ToText(Integer) NumberTag false false 1 1)))

(fn ConstructionScript
  (bind _wheellocation (Variables|Default|GetWheelLocation))
  (if (Utilities|Enum|Equal(Enum) _wheellocation "NewEnumerator1")
    (Rendering|SetVisibility (Variables|Default|GetNumberTagRight) false false :!label _label)
    (elif (Utilities|Enum|Equal(Enum) _wheellocation "NewEnumerator3")
      (goto _label)
      (elif (Utilities|Enum|Equal(Enum) _wheellocation "NewEnumerator2")
        (Rendering|SetVisibility (Variables|Default|GetNumberTagLeft) false false :!label _label_2)
        (elif (Utilities|Enum|Equal(Enum) _wheellocation "NewEnumerator4")
          (goto _label_2))))))
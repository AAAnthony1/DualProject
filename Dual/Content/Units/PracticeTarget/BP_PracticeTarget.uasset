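; Practice target unit that fades in as a hologram, becomes a damageable hull, and removes itself when destroyed.
; BeginPlay gets the hull from a child actor, assigns its non-player, non-colonial faction, disables collision and binds its destroyed event.
; ShowTarget runs a timeline driving the holographic mesh's yaw and dynamic material opacity, then swaps to the hull and enables its collision.
; Hull destruction destroys the actor after a short delay.
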(event Custom|ShowTarget
  (bind _returnvalue (Rendering|Material|CreateDynamicMaterialInstance (Variables|Default|GetSM_PracticeTarget) 0 "/Game/Units/PracticeTarget/M_PracticeTargetHolographic.M_PracticeTargetHolographic" :!class /Script/Engine.PrimitiveComponent))
  (bind _output_get (Variables|Default|SetHolographicMaterial _returnvalue))
  (Rendering|Material|SetScalarParameterValue _output_get "HolographicTargetOpacity" 0.0 :!class /Script/Engine.MaterialInstanceDynamic)
  (Development|SetHiddeninGame (Variables|Default|GetSM_PracticeTarget) false false)
  (bind _targetfade (Timeline|TargetFadeIn PlayFromStart)
    (:Update
      (Transformation|SetRelativeRotation (Variables|Default|GetSM_PracticeTarget) (Math|Rotator|MakeRotator 0.0 0.0 (* _targetfade 1.8e+02)) false false)
      (Rendering|Material|SetScalarParameterValue (Variables|Default|GetHolographicMaterial) "HolographicTargetOpacity" (* _targetfade 1.8e+02) :!class /Script/Engine.MaterialInstanceDynamic))
    (:Finished
      (Rendering|SetVisibility (Variables|Default|GetSM_PracticeTarget) false false)
      (Rendering|SetVisibility (Variables|Default|GetBP_HullComponent) true false)
      (Default|SetComponentCollision (Variables|Default|GetHullComponent) true))))

(event Custom|Destroyed
  (params (HullComponent :type BP%20Damageable%20Component%20Object%20Reference))
  (Utilities|FlowControl|Delay 1.0)
  (Actor|DestroyActor))

(event EventBeginPlay
  (bind _asbp_damageable_component (Utilities|Casting|CastToBP_DamageableComponent (Variables|/Script/Engine.ChildActorComponent|GetChildActor (Variables|Default|GetBP_HullComponent))))
  (bind _output_get (Variables|Default|SetHullComponent _asbp_damageable_component))
  (Variables|/Game/Units/Blueprints/BP_DamageableComponent.BP_DamageableComponent_C|SetComponentOwner _output_get (Utilities|Struct|MakeSTRUCT_Factions false false true))
  (Collision|SetActorEnableCollision false)
  (EventDispatchers|BindEventtoDestroyed (Variables|Default|GetHullComponent) (delegate Custom|Destroyed))
  (Default|SetComponentCollision (Variables|Default|GetHullComponent) false))

(fn ConstructionScript
  (|CallParentFunction))
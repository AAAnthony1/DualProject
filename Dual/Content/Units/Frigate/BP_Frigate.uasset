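; BP_Frigate is a frigate unit assembled from child-actor BP_DamageableComponent pieces, with destruction that cascades between them.
; On BeginPlay it collects all pieces, sets their owner faction and binds the Destroyed events of key hull sections and reactors.
; Losing the forward or engine hull destroys the pieces attached beneath its mesh.
; Losing the central hull destroys every piece, as does losing both reactors, counted through a non-looping MultiGate.
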(event Custom|CreateComponentArray
  (for _array_element (Components|GetChildrenComponents (Variables|Default|GetDefaultSceneRoot) true)
    (bind _aschild_actor_component (Utilities|Casting|CastToChildActorComponent _array_element))
    (bind _asbp_damageable_component (Utilities|Casting|CastToBP_DamageableComponent (Variables|/Script/Engine.ChildActorComponent|GetChildActor _aschild_actor_component)))
    (Utilities|Array|Add (Variables|Default|GetAllHullComponents) _asbp_damageable_component))
  (for _array_element_2 (Variables|Default|GetAllHullComponents)
    (Variables|/Game/Units/Blueprints/BP_DamageableComponent.BP_DamageableComponent_C|SetComponentOwner _array_element_2 (Utilities|Struct|MakeSTRUCT_Factions false false true))))

(event Custom|CustomEvent_0
  (params (HullComponent :type BP%20Damageable%20Component%20Object%20Reference))
  (for _array_element (Components|GetChildrenComponents (Variables|/Game/Units/Blueprints/BP_DamageableComponent.BP_DamageableComponent_C|GetStaticMeshPiece HullComponent) true)
    (bind _aschild_actor_component (Utilities|Casting|CastToChildActorComponent _array_element))
    (bind _asbp_damageable_component (Utilities|Casting|CastToBP_DamageableComponent (Variables|/Script/Engine.ChildActorComponent|GetChildActor _aschild_actor_component)))
    (Default|DestroyHullComponent _asbp_damageable_component true)))

(event Custom|ReactorDestroyed
  (params (HullComponent :type BP%20Damageable%20Component%20Object%20Reference))
  (Utilities|FlowControl|MultiGate false false -1
    (:Out%201
      (for _array_element (Components|GetChildrenComponents (Variables|Default|GetDefaultSceneRoot) true)
        (bind _aschild_actor_component (Utilities|Casting|CastToChildActorComponent _array_element))
        (bind _asbp_damageable_component (Utilities|Casting|CastToBP_DamageableComponent (Variables|/Script/Engine.ChildActorComponent|GetChildActor _aschild_actor_component)))
        (Default|DestroyHullComponent _asbp_damageable_component true)))))

(event Custom|CentreDestroyed
  (params (HullComponent :type BP%20Damageable%20Component%20Object%20Reference))
  (for _array_element (Components|GetChildrenComponents (Variables|Default|GetDefaultSceneRoot) true)
    (bind _aschild_actor_component (Utilities|Casting|CastToChildActorComponent _array_element))
    (bind _asbp_damageable_component (Utilities|Casting|CastToBP_DamageableComponent (Variables|/Script/Engine.ChildActorComponent|GetChildActor _aschild_actor_component)))
    (Default|DestroyHullComponent _asbp_damageable_component true)))

(event EventBeginPlay
  (CallFunction|CreateComponentArray)
  (Utilities|FlowControl|Sequence
    (:then_0
      (bind _asbp_damageable_component (Utilities|Casting|CastToBP_DamageableComponent (Variables|/Script/Engine.ChildActorComponent|GetChildActor (Variables|Default|GetReactorBow))))
      (EventDispatchers|BindEventtoDestroyed _asbp_damageable_component (delegate Custom|ReactorDestroyed)))
    (:then_1
      (bind _asbp_damageable_component_2 (Utilities|Casting|CastToBP_DamageableComponent (Variables|/Script/Engine.ChildActorComponent|GetChildActor (Variables|Default|GetReactorStern))))
      (EventDispatchers|BindEventtoDestroyed _asbp_damageable_component_2 (delegate Custom|ReactorDestroyed)))
    (:then_2
      (bind _asbp_damageable_component_3 (Utilities|Casting|CastToBP_DamageableComponent (Variables|/Script/Engine.ChildActorComponent|GetChildActor (Variables|Default|GetHullCentral))))
      (EventDispatchers|BindEventtoDestroyed _asbp_damageable_component_3 (delegate Custom|CentreDestroyed)))
    (:then_3
      (bind _asbp_damageable_component_4 (Utilities|Casting|CastToBP_DamageableComponent (Variables|/Script/Engine.ChildActorComponent|GetChildActor (Variables|Default|GetHullForward))))
      (EventDispatchers|BindEventtoDestroyed _asbp_damageable_component_4 (delegate Custom|CustomEvent_0)))
    (:then_4
      (bind _asbp_damageable_component_5 (Utilities|Casting|CastToBP_DamageableComponent (Variables|/Script/Engine.ChildActorComponent|GetChildActor (Variables|Default|GetHullEngine))))
      (EventDispatchers|BindEventtoDestroyed _asbp_damageable_component_5 (delegate Custom|CustomEvent_0)))))

(fn ConstructionScript)
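; Turret lander unit that continuously spins its hull core and awards score when that core is destroyed.
; A looping 60 Hz timer started on BeginPlay rotates the HullCore in yaw, with no use of Tick.
; It binds to the destroyed event of the core's BP_DamageableComponent child actor, then kills all child components before awarding score for the unit.
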(event Custom|CoreDestroyed
  (params (HullComponent :type BP%20Damageable%20Component%20Object%20Reference))
  (Utilities|UnitKillChildComponents (Components|GetChildrenComponents (Variables|Default|GetDefaultSceneRoot) true)
    (:Done
      (Utilities|UnitDestroyedAwardScore "NewEnumerator30" self))))

(event Custom|StartSpinning
  (Utilities|Time|SetTimerbyEvent (delegate Custom|Spin) (/ 1.0 6e+01) true))

(event Custom|Spin
  (Transformation|AddRelativeRotation (Variables|Default|GetHullCore) (Math|Rotator|MakeRotator 0.0 0.0 2.0) false false))

(event EventBeginPlay
  (CallFunction|StartSpinning)
  (bind _asbp_damageable_component (Utilities|Casting|CastToBP_DamageableComponent (Variables|/Script/Engine.ChildActorComponent|GetChildActor (Variables|Default|GetHullCore))))
  (EventDispatchers|BindEventtoDamageableComponentDestroyed _asbp_damageable_component (delegate Custom|CoreDestroyed)))

(fn ConstructionScript)
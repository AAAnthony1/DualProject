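; BP_HullComponentTurret is a hull component turret that automatically attacks Player One's BP_Playership.
; On BeginPlay it finds that ship, stores it as the target, starts a looping fire timer and prints a display name.
; Tick rotates the turret mesh toward the target's hull.
; Each shot spawns a BP_WeaponPulse aimed from the weapon origin, sets its damage and valid factions, and tints it red through a dynamic material.
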(event Custom|StartFiring
  (Utilities|Time|SetTimerbyEvent (delegate Custom|Fire) 0.5 true))

(event Custom|Fire
  (bind _returnvalue (Game|SpawnActorfromClass "/Game/Weaponry/Master/Blueprints/BP_WeaponPulse.BP_WeaponPulse_C" (Math|Transform|MakeTransform (Transformation|GetWorldLocation (Variables|Default|GetWeaponOrigin)) (Math|Rotator|FindLookatRotation (Transformation|GetWorldLocation (Variables|Default|GetWeaponOrigin)) (Transformation|GetWorldLocation (Variables|/Game/Players/Blueprints/BP_Playership.BP_Playership_C|GetHullComponent (Variables|Default|GetTargetBody))))) "Undefined" 0 0))
  (Default|ProjectileSetHitInfo _returnvalue 1 (Utilities|Struct|MakeSTRUCT_Factions true true false true))
  (bind _returnvalue_2 (Rendering|Material|CreateDynamicMaterialInstance (Variables|/Game/Weaponry/Master/Blueprints/BP_WeaponProjectile.BP_WeaponProjectile_C|GetSM_BlasterBoltSingle _returnvalue) 0 "/Game/Weaponry/Blasters/Materials/M_BlasterBoltMaterial.M_BlasterBoltMaterial" :!class /Script/Engine.PrimitiveComponent))
  (Rendering|Material|SetVectorParameterValue _returnvalue_2 "Color" "(R=1.000000,G=0.028078,B=0.000000,A=1.000000)" :!class /Script/Engine.MaterialInstanceDynamic))

(event EventBeginPlay
  (|CallParentFunction)
  (bind _outactors (Actor|GetAllActorsOfClass "/Game/Players/Blueprints/BP_Playership.BP_Playership_C"))
  (for _array_element _outactors
    (switch Utilities|FlowControl|Switch|SwitchonENUM_PlayerNumber (Variables|/Game/Players/Blueprints/BP_Playership.BP_Playership_C|GetPlayer _array_element)
      (:NewEnumerator0
        (Variables|Default|SetTargetBody _array_element)
        (CallFunction|StartFiring)
        (Development|PrintString (Utilities|GetDisplayName 0))))))

(event EventTick
  (params (DeltaSeconds :type Float%20%28single-precision%29))
  (bind _staticmeshpiece (Variables|Default|GetStaticMeshPiece))
  (Transformation|SetWorldRotation _staticmeshpiece (Math|Rotator|FindLookatRotation (Transformation|GetWorldLocation _staticmeshpiece) (Transformation|GetWorldLocation (Variables|/Game/Players/Blueprints/BP_Playership.BP_Playership_C|GetHullComponent (Variables|Default|GetTargetBody)))) false false))

(fn ConstructionScript
  (|CallParentFunction))
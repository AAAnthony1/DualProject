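; Turret that tracks and fires pulse projectiles at one BP_PlayerFighter, picked at random on BeginPlay, with meshes set in construction.
; A tracking-rate timer checks range, eases casing yaw and clamped barrel pitch onto the target via a timeline, and lerps back to rest when out of range.
; A fire-rate timer spawns shots from alternating barrels, aimed at the target's current position, when within firing range and not a Dummy.
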(event Custom|CustomTickEvent
  (bind _returnvalue (Transformation|GetActorLocation))
  (bind _target (Variables|Default|GetTarget))
  (bind _returnvalue_2 (Transformation|GetActorLocation _target))
  (bind _returnvalue_3 (- _returnvalue _returnvalue_2))
  (bind _returnvalue_4 (Math|Vector|VectorLength _returnvalue_3))
  ;[1 1 1] Custom Tick - Determine if player is within range
  (CallFunction|TrackWeaponsFire)
  (if (Variables|Turret|GetDebug)
    (Development|PrintString (Utilities|String|Append "Distance to Target" (Utilities|String|ToString(Float) _returnvalue_4))))
  (if (<= _returnvalue_4 (Variables|Turret|GetTurretRange))
    (Variables|Default|SetTargetInRange true)
    (Variables|Default|SetWoke true)
    (else
      (Variables|Default|SetTargetInRange false)))
  (if (Variables|Default|GetTargetInRange)
    (CallFunction|TrackPlayer)
    (elif (Variables|Default|GetWoke)
      (CallFunction|Resetto0))))

(event Custom|FireWeapon
  (bind _barrel1 (Variables|Default|GetBarrel1))
  (bind _barrel2 (Variables|Default|GetBarrel2))
  (bind _returnvalue (Transformation|GetWorldLocation _barrel2))
  (bind _returnvalue_2 (Transformation|GetWorldLocation _barrel1))
  ;[1 1 1] Fire Weapon - Need to override and copy this functionality for enemy weapons
  (Utilities|FlowControl|FlipFlop
    (:A
      (bind _returnvalue_3 (Game|SpawnActorfromClass "/Game/Weaponry/Master/Blueprints/BP_WeaponPulse.BP_WeaponPulse_C" (Math|Transform|MakeTransform _returnvalue_2 (Variables|/Script/Engine.SceneComponent|GetRelativeRotation _barrel1)) "Undefined" 0 0))
      (Variables|/Script/Engine.MovementComponent|SetVelocity (Variables|/Game/Weaponry/Master/Blueprints/BP_WeaponProjectile.BP_WeaponProjectile_C|GetProjectileMovement _returnvalue_3) (- (Transformation|GetActorLocation (Variables|Default|GetTarget)) _returnvalue_2))
      (Transformation|SetWorldScale3D (Variables|/Game/Weaponry/Master/Blueprints/BP_WeaponProjectile.BP_WeaponProjectile_C|GetSM_BlasterBoltSingle _returnvalue_3) "0.250000,0.250000,0.250000"))
    (:B
      (bind _returnvalue_4 (Game|SpawnActorfromClass "/Game/Weaponry/Master/Blueprints/BP_WeaponPulse.BP_WeaponPulse_C" (Math|Transform|MakeTransform _returnvalue (Variables|/Script/Engine.SceneComponent|GetRelativeRotation _barrel2)) "Undefined" 0 0))
      (Variables|/Script/Engine.MovementComponent|SetVelocity (Variables|/Game/Weaponry/Master/Blueprints/BP_WeaponProjectile.BP_WeaponProjectile_C|GetProjectileMovement _returnvalue_4) (- (Transformation|GetActorLocation (Variables|Default|GetTarget)) _returnvalue))
      (Transformation|SetWorldScale3D (Variables|/Game/Weaponry/Master/Blueprints/BP_WeaponProjectile.BP_WeaponProjectile_C|GetSM_BlasterBoltSingle _returnvalue_4) "0.250000,0.250000,0.250000"))))

(event Custom|ResetActivate
  ;[1 1 1] Track Player Location for turret tracking
  (Utilities|FlowControl|DoOnce false) ; enters at Reset
)

(event Custom|TrackWeaponsFire
  ;[1 1 1] Track Player location for weapons fire
  (if (<= (Math|Vector|VectorLength (- (Transformation|GetActorLocation) (Transformation|GetActorLocation (Variables|Default|GetTarget)))) (Variables|Turret|GetFiringRange))
    (Variables|Default|SetTargetInFiringRange true)
    (else
      (Variables|Default|SetTargetInFiringRange false))))

(event Custom|FireWeaponTick
  (if (not (Variables|Turret|GetDummy))
    (if (Variables|Default|GetTargetInFiringRange)
      (CallFunction|FireWeapon))))

(event Custom|CustomTick
  (CallFunction|CustomTickEvent))

(event Custom|ResetTo0
  ;[1 1 1] Rotate Meshes to Base Yaw and Pitch
  (Utilities|FlowControl|DoOnce false :!label _label
    (:Completed
      (bind _alpha (Timeline|Lerp PlayFromStart)
        (:Update
          (Transformation|SetRelativeRotation (Variables|Default|GetSM_PyramidTurretCasing) (Math|Rotator|Lerp(Rotator) (Variables|/Script/Engine.SceneComponent|GetRelativeRotation (Variables|Default|GetSM_PyramidTurretCasing)) (Variables|Default|GetInitialBaseRot) _alpha true) false false)
          (Transformation|SetRelativeRotation (Variables|Default|GetSM_PyramidTurretBarrels) (Math|Rotator|Lerp(Rotator) (Variables|/Script/Engine.SceneComponent|GetRelativeRotation (Variables|Default|GetSM_PyramidTurretBarrels)) (Variables|Default|GetInitialCannonPitch) _alpha true) false false))
        (:Finished
          (Variables|Default|SetWoke false)
          (Variables|Default|SetAlphaVar 0.0)
          (CallFunction|ResetActivate)
          (goto _label Reset))))))

(event Custom|TrackPlayer
  (bind _returnvalue (Transformation|GetActorLocation))
  (bind _target (Variables|Default|GetTarget))
  (bind _returnvalue_2 (Transformation|GetActorLocation _target))
  (bind _returnvalue_3 (Math|Rotator|FindLookatRotation _returnvalue _returnvalue_2))
  (bind (_roll _pitch _yaw) (Math|Rotator|BreakRotator _returnvalue_3))
  ;[1 1 1] Track Player Location for turret tracking
  (Variables|Default|SetLookAtPitch (Math|Rotator|MakeRotator 0.0 (Math|Float|Clamp(Float) _pitch 0.0 55.0) 0.0))
  (Variables|Default|SetLookAtYaw (Math|Rotator|MakeRotator 0.0 0.0 _yaw))
  (if (== (Variables|Default|GetAlphaVar) 1.0)
    (Transformation|SetRelativeRotation (Variables|Default|GetSM_PyramidTurretCasing) (Variables|Default|GetLookAtYaw) false false)
    (Transformation|SetRelativeRotation (Variables|Default|GetSM_PyramidTurretBarrels) (Variables|Default|GetLookAtPitch) false false)
    (else
      (Transformation|SetRelativeRotation (Variables|Default|GetSM_PyramidTurretCasing) (Math|Rotator|Lerp(Rotator) (Variables|/Script/Engine.SceneComponent|GetRelativeRotation (Variables|Default|GetSM_PyramidTurretCasing)) (Variables|Default|GetLookAtYaw) (Variables|Default|GetAlphaVar) true) false false)
      (Transformation|SetRelativeRotation (Variables|Default|GetSM_PyramidTurretBarrels) (Math|Rotator|Lerp(Rotator) (Variables|/Script/Engine.SceneComponent|GetRelativeRotation (Variables|Default|GetSM_PyramidTurretBarrels)) (Variables|Default|GetLookAtPitch) (Variables|Default|GetAlphaVar) true) false false)
      (Utilities|FlowControl|DoOnce false
        (:Completed
          (bind _alpha (Timeline|Activate PlayFromStart)
            (:Update
              (Variables|Default|SetAlphaVar _alpha))))))))

(event EventBeginPlay
  (|CallParentFunction)
  (Utilities|Time|SetTimerbyEvent (delegate Custom|CustomTick) (/ 1.0 (Variables|Turret|GetTrackingRate)) true)
  (Utilities|Time|SetTimerbyEvent (delegate Custom|FireWeaponTick) (/ 1.0 (Variables|Turret|GetFireRate)) true)
  ;[1 1 1] Cache Initial Rotations
  (Variables|Default|SetInitialBaseRot (Math|Rotator|MakeRotator 0.0 0.0 (.Yaw (Math|Rotator|BreakRotator (Variables|/Script/Engine.SceneComponent|GetRelativeRotation (Variables|Default|GetSM_PyramidTurretCasing))))))
  (Variables|Default|SetInitialCannonPitch (Math|Rotator|MakeRotator 0.0 (.Pitch (Math|Rotator|BreakRotator (Variables|/Script/Engine.SceneComponent|GetRelativeRotation (Variables|Default|GetSM_PyramidTurretBarrels)))) 0.0))
  ;[1 1 1] Cache Player References
  (bind _outactors (Actor|GetAllActorsOfClass "/Game/Players/Blueprints/BP_PlayerFighter.BP_PlayerFighter_C"))
  (bind _output_get (Variables|Default|SetPlayers _outactors))
  (for _array_element _output_get
    (switch Utilities|FlowControl|Switch|SwitchonENUM_PlayerNumber (Variables|/Game/Players/Blueprints/BP_PlayerFighter.BP_PlayerFighter_C|GetPlayer _array_element)
      (:NewEnumerator0
        (Variables|Default|SetPlayer1 _array_element))
      (:NewEnumerator1
        (Variables|Default|SetPlayer2 _array_element))))
  (Variables|Default|SetTarget (Utilities|Array|Get(acopy) (Variables|Default|GetPlayers) (Math|Random|RandomInteger (Utilities|Array|Length (Variables|Default|GetPlayers))))))

(fn ConstructionScript
  (|CallParentFunction)
  (Components|StaticMesh|SetStaticMesh (Variables|Default|GetSM_PyramidTurretBase) (Variables|Turret|GetTurretBase))
  (Components|StaticMesh|SetStaticMesh (Variables|Default|GetSM_PyramidTurretCasing) (Variables|Turret|GetTurretCasing))
  (Components|StaticMesh|SetStaticMesh (Variables|Default|GetSM_PyramidTurretBarrels) (Variables|Turret|GetTurretBarrels)))
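; BP_HullComponent is a destructible hull-piece actor with a configurable mesh, hitpoints, faction owner and score.
; Weapon-interface hits from valid targeting factions deduct attack power, flash the material red and fire Hit or Destroyed dispatchers.
; Destruction updates campaign score, disables collision, spawns a size-scaled explosion, drifts and dissolves the mesh through swapped burn materials, then destroys the actor.
; DestroyHullComponent triggers this sequence externally, with optional score.
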(event OnComponentHit(StaticMeshPiece)
  (params (HitComponent :type Primitive%20Component%20Object%20Reference) (OtherActor :type Actor%20Object%20Reference) (OtherComp :type Primitive%20Component%20Object%20Reference) (NormalImpulse :type Vector :default "0, 0, 0") (Hit :type Hit%20Result%20Structure%20%28by%20ref%29))
  (bind _staticmeshpiece (Variables|Default|GetStaticMeshPiece))
  (bind _returnvalue (Transformation|GetWorldTransform _staticmeshpiece))
  (bind (_location _rotation) (Math|Transform|BreakTransform _returnvalue))
  ;[1 1 1] Check hits and deduct health
  (if (not (Variables|Default|GetInvincible))
    (if (Utilities|DoesObjectImplementInterface OtherActor "/Game/Weaponry/BPI_WeaponsInterface.BPI_WeaponsInterface_C")
      (bind (_attackpower _validtargetslist) (Class|BPIWeaponsInterface|ProjectileGetHitInfo(Message) OtherActor))
      (Utilities|CheckValidTarget (Variables|Default|GetComponentOwner) _validtargetslist
        (:ValidTarget
          (Utilities|FlowControl|Sequence
            (:then_0
              ;[1 1 1] Flash Red When Hit
              (bind _newtrack_0 (Timeline|Timeline_0 PlayFromStart)
                (:Update
                  (Rendering|Material|SetScalarParameterValue (Variables|Default|GetHullMaterial) "Damaged" _newtrack_0 :!class /Script/Engine.MaterialInstanceDynamic))))
            (:then_1
              (bind _output_get (Variables|Default|SetCurrentHitpoints (- (Variables|Default|GetCurrentHitpoints) _attackpower)))
              (Math|Integer|CompareInt _output_get 0
                (:>
                  (Default|CallHit :!label _label))
                (:==
                  (Utilities|FlowControl|DoOnce false :!label _label_2
                    (:Completed
                      (Utilities|FlowControl|Sequence
                        (:then_0
                          (goto _label))
                        (:then_1
                          (Default|CallDestroyed self)
                          ;[1 1 1] Should Component give Score
                          (bind _asgamemode_campaign (Utilities|Casting|CastToGAMEMODE_Campaign (Game|GetGameMode)))
                          (Default|UpdateScore _asgamemode_campaign (Variables|Default|GetScore))
                          (Utilities|FlowControl|Sequence
                            (:then_0
                              ;[1 1 1] Disable Collision
                              (Collision|SetCollisionEnabled (Variables|Default|GetStaticMeshPiece) "NoCollision"))
                            (:then_1
                              ;[1 1 1] Create Explosion VFX
                              (bind _returnvalue_2 (Effects|SpawnEmitteratLocation "/Game/StarterContent/Particles/P_Explosion.P_Explosion" _location _rotation))
                              (switch Utilities|FlowControl|Switch|SwitchonENUM_ComponentSize (Variables|Default|GetComponentSize)
                                (:NewEnumerator0
                                  (Transformation|SetWorldScale3D _returnvalue_2 "15.000000,15.000000,15.000000"))
                                (:NewEnumerator1
                                  (Transformation|SetWorldScale3D _returnvalue_2 "30.000000,30.000000,30.000000"))
                                (:NewEnumerator2
                                  (Transformation|SetWorldScale3D _returnvalue_2 "50.000000,50.000000,50.000000"))))
                            (:then_2
                              (bind _drift_scale (Timeline|Drift PlayFromStart)
                                (:Update
                                  (Transformation|AddWorldOffset (Variables|Default|GetStaticMeshPiece) (Math|Vector|MakeVector 0.0 0.0 _drift_scale) false false))))
                            (:then_3
                              ;[1 1 1] Replace All Materials with Dissolve and start dissolving
                              (Math|Integer|CompareInt (Variables|Default|GetMaterialToHandle) (Rendering|Material|GetNumMaterials (Variables|Default|GetStaticMeshPiece))
                                (:>
                                  (bind (_direction _opacitya _opacityb _opacityc) (Timeline|Dissolve PlayFromStart)
                                    (:Update
                                      (for _array_element (Variables|Default|GetMaterials)
                                        (Utilities|FlowControl|Sequence
                                          (:then_0
                                            (Rendering|Material|SetScalarParameterValue _array_element "OpacityA" _opacitya :!class /Script/Engine.MaterialInstanceDynamic))
                                          (:then_1
                                            (Rendering|Material|SetScalarParameterValue _array_element "OpacityB" _opacityb :!class /Script/Engine.MaterialInstanceDynamic))
                                          (:then_2
                                            (Rendering|Material|SetScalarParameterValue _array_element "OpacityC" _opacityc :!class /Script/Engine.MaterialInstanceDynamic)))))))
                                (:==
                                  (bind _returnvalue_3 (Rendering|Material|CreateDynamicMaterialInstance (Variables|Default|GetStaticMeshPiece) (Variables|Default|GetMaterialToHandle) "/Game/Units/Materials/M_HullBurn.M_HullBurn" :!class /Script/Engine.PrimitiveComponent :!label _label_3))
                                  (Utilities|Array|Add (Variables|Default|GetMaterials) _returnvalue_3)
                                  (Math|Integer|IncrementInt (Variables|Default|GetMaterialToHandle)
                                    (:%20%20
                                      (CallFunction|NextMaterial))))
                                (:<
                                  (goto _label_3))))
                            (:then_4
                              ;[1 1 1] Destroy Hull Component
                              (Utilities|FlowControl|Delay 2.0)
                              (Actor|DestroyActor))))))))
                (:<
                  (goto _label_2))))))))))

(event Custom|DestroyHullComponent
  (params (AwardScore :type Boolean))
  (bind _staticmeshpiece (Variables|Default|GetStaticMeshPiece))
  (bind _returnvalue (Transformation|GetWorldTransform _staticmeshpiece))
  (bind (_location _rotation) (Math|Transform|BreakTransform _returnvalue))
  ;[1 1 1] Should Component give Score
  (if AwardScore
    (bind _asgamemode_campaign (Utilities|Casting|CastToGAMEMODE_Campaign (Game|GetGameMode)))
    (Default|UpdateScore _asgamemode_campaign (Variables|Default|GetScore)))
  (Utilities|FlowControl|Sequence
    (:then_0
      ;[1 1 1] Disable Collision
      (Collision|SetCollisionEnabled (Variables|Default|GetStaticMeshPiece) "NoCollision"))
    (:then_1
      ;[1 1 1] Create Explosion VFX
      (bind _returnvalue_2 (Effects|SpawnEmitteratLocation "/Game/StarterContent/Particles/P_Explosion.P_Explosion" _location _rotation))
      (switch Utilities|FlowControl|Switch|SwitchonENUM_ComponentSize (Variables|Default|GetComponentSize)
        (:NewEnumerator0
          (Transformation|SetWorldScale3D _returnvalue_2 "15.000000,15.000000,15.000000"))
        (:NewEnumerator1
          (Transformation|SetWorldScale3D _returnvalue_2 "30.000000,30.000000,30.000000"))
        (:NewEnumerator2
          (Transformation|SetWorldScale3D _returnvalue_2 "50.000000,50.000000,50.000000"))))
    (:then_2
      (bind _drift_scale (Timeline|Drift PlayFromStart)
        (:Update
          (Transformation|AddWorldOffset (Variables|Default|GetStaticMeshPiece) (Math|Vector|MakeVector 0.0 0.0 _drift_scale) false false))))
    (:then_3
      ;[1 1 1] Replace All Materials with Dissolve and start dissolving
      (Math|Integer|CompareInt (Variables|Default|GetMaterialToHandle) (Rendering|Material|GetNumMaterials (Variables|Default|GetStaticMeshPiece))
        (:>
          (bind (_direction _opacitya _opacityb _opacityc) (Timeline|Dissolve PlayFromStart)
            (:Update
              (for _array_element (Variables|Default|GetMaterials)
                (Utilities|FlowControl|Sequence
                  (:then_0
                    (Rendering|Material|SetScalarParameterValue _array_element "OpacityA" _opacitya :!class /Script/Engine.MaterialInstanceDynamic))
                  (:then_1
                    (Rendering|Material|SetScalarParameterValue _array_element "OpacityB" _opacityb :!class /Script/Engine.MaterialInstanceDynamic))
                  (:then_2
                    (Rendering|Material|SetScalarParameterValue _array_element "OpacityC" _opacityc :!class /Script/Engine.MaterialInstanceDynamic)))))))
        (:==
          (bind _returnvalue_3 (Rendering|Material|CreateDynamicMaterialInstance (Variables|Default|GetStaticMeshPiece) (Variables|Default|GetMaterialToHandle) "/Game/Units/Materials/M_HullBurn.M_HullBurn" :!class /Script/Engine.PrimitiveComponent :!label _label))
          (Utilities|Array|Add (Variables|Default|GetMaterials) _returnvalue_3)
          (Math|Integer|IncrementInt (Variables|Default|GetMaterialToHandle)
            (:%20%20
              (CallFunction|NextMaterial))))
        (:<
          (goto _label))))
    (:then_4
      ;[1 1 1] Destroy Hull Component
      (Utilities|FlowControl|Delay 2.0)
      (Actor|DestroyActor))))

(event Custom|SetPlayerComponentHitpoints
  (params (TotalHitpoints :type Integer))
  (Variables|Default|SetTotalHitpoints TotalHitpoints)
  (Variables|Default|SetCurrentHitpoints (Variables|Default|GetTotalHitpoints)))

(event Custom|NextMaterial
  ;[1 1 1] Replace All Materials with Dissolve and start dissolving
  (Math|Integer|CompareInt (Variables|Default|GetMaterialToHandle) (Rendering|Material|GetNumMaterials (Variables|Default|GetStaticMeshPiece))
    (:>
      (bind (_direction _opacitya _opacityb _opacityc) (Timeline|Dissolve PlayFromStart)
        (:Update
          (for _array_element (Variables|Default|GetMaterials)
            (Utilities|FlowControl|Sequence
              (:then_0
                (Rendering|Material|SetScalarParameterValue _array_element "OpacityA" _opacitya :!class /Script/Engine.MaterialInstanceDynamic))
              (:then_1
                (Rendering|Material|SetScalarParameterValue _array_element "OpacityB" _opacityb :!class /Script/Engine.MaterialInstanceDynamic))
              (:then_2
                (Rendering|Material|SetScalarParameterValue _array_element "OpacityC" _opacityc :!class /Script/Engine.MaterialInstanceDynamic)))))))
    (:==
      (bind _returnvalue (Rendering|Material|CreateDynamicMaterialInstance (Variables|Default|GetStaticMeshPiece) (Variables|Default|GetMaterialToHandle) "/Game/Units/Materials/M_HullBurn.M_HullBurn" :!class /Script/Engine.PrimitiveComponent :!label _label))
      (Utilities|Array|Add (Variables|Default|GetMaterials) _returnvalue)
      (Math|Integer|IncrementInt (Variables|Default|GetMaterialToHandle)
        (:%20%20
          (CallFunction|NextMaterial))))
    (:<
      (goto _label))))

(event EventBeginPlay
  (Utilities|FlowControl|Sequence
    (:then_0
      (bind _returnvalue (Rendering|Material|CreateDynamicMaterialInstance (Variables|Default|GetStaticMeshPiece) 0 "/Game/Units/Materials/M_Hull.M_Hull" :!class /Script/Engine.PrimitiveComponent))
      (Variables|Default|SetHullMaterial _returnvalue))
    (:then_1
      (Variables|Default|SetCurrentHitpoints (Variables|Default|GetTotalHitpoints)))))

(fn ConstructionScript
  (bind _staticmesh (Variables|Default|GetStaticMesh))
  (Utilities|IsValid _staticmesh
    (:Is%20Valid
      (Components|StaticMesh|SetStaticMesh (Variables|Default|GetStaticMeshPiece) _staticmesh))))

(fn ProjectileGetHitInfo
  (return 0 ""))
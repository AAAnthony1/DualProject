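; BP_CommunicationsManager plays character dialogue lines through an on-screen communications widget.
; It creates the widget at BeginPlay; PlayDialogue then looks up the speaker's defaults in the character portraits data table.
; A chain of events resolves allegiance, emotion and channel state, substituting the character default when the line holds a specific enum value.
; The resolved line goes to the widget's PlayConversation, followed by a duration-based delay with nothing after it.
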(event Custom|PlayDialogue
  (params (DialogueData :type STRUCT%20Dialogue%20Data%20Structure))
  ;[1 1 1] Get Character Default Data
  (bind _output_get (Variables|Default|SetDialogueData DialogueData))
  (bind _returnvalue (Utilities|GetDataTableRow "/Game/Communications/DATA_CharacterPortraits.DATA_CharacterPortraits" (Utilities|String|StringToName (Utilities|String|EnumtoString (Utilities|Enum|LiteralenumENUM_Characters (Utilities|Struct|BreakSTRUCT_DialogueData _output_get)))))
    (:then
      (Variables|Default|SetCharacterDefaultData _returnvalue)
      (CallFunction|GetAlliegence))))

(event Custom|GetAlliegence
  (bind _dialoguedata (Variables|Default|GetDialogueData))
  (bind _alligence (Utilities|Struct|BreakSTRUCT_DialogueData _dialoguedata))
  ;[1 1 1] Get Alligence
  (if (Utilities|Enum|Equal(Enum) _alligence "NewEnumerator4")
    (Variables|Default|SetAlligence (Utilities|Struct|BreakSTRUCT_PortraitData (Variables|Default|GetCharacterDefaultData)))
    (else
      (Variables|Default|SetAlligence _alligence)))
  (CallFunction|GetEmotion))

(event Custom|GetEmotion
  (bind _dialoguedata (Variables|Default|GetDialogueData))
  (bind _emotion (Utilities|Struct|BreakSTRUCT_DialogueData _dialoguedata))
  ;[1 1 1] Get Emotion
  (if (Utilities|Enum|Equal(Enum) _emotion "NewEnumerator15")
    (Variables|Default|SetEmotion (Utilities|Struct|BreakSTRUCT_PortraitData (Variables|Default|GetCharacterDefaultData)))
    (else
      (Variables|Default|SetEmotion _emotion)))
  (CallFunction|GetChannelState))

(event Custom|GetChannelState
  (bind _dialoguedata (Variables|Default|GetDialogueData))
  (bind _state (Utilities|Struct|BreakSTRUCT_DialogueData _dialoguedata))
  ;[1 1 1] Get Channel State
  (if (Utilities|Enum|Equal(Enum) _state "NewEnumerator6")
    (Variables|Default|SetState (Utilities|Struct|BreakSTRUCT_PortraitData (Variables|Default|GetCharacterDefaultData)))
    (else
      (Variables|Default|SetState _state)))
  (CallFunction|UpdateCommunicationsWidget))

(event Custom|UpdateCommunicationsWidget
  (bind _dialoguedata (Variables|Default|GetDialogueData))
  (bind (_character _dialogue _duration _firstline _lastline) (Utilities|Struct|BreakSTRUCT_DialogueData _dialoguedata))
  ;[1 1 1] Populate Communications Widget
  (Default|PlayConversation (Variables|Default|GetWIDCommunications) (Utilities|Struct|MakeSTRUCT_DialogueData _character (Variables|Default|GetAlligence) (Variables|Default|GetEmotion) (Variables|Default|GetState) _dialogue _duration _firstline _lastline))
  (Utilities|FlowControl|Delay (- (.Duration (Utilities|Struct|BreakSTRUCT_DialogueData (Variables|Default|GetDialogueData))) 0.1)))

(event EventBeginPlay
  ;[1 1 1] Create Communications Widget
  (bind _returnvalue (UserInterface|CreateWidget "/Game/Communications/WID_Communications.WID_Communications_C"))
  (bind _output_get (Variables|Default|SetWIDCommunications _returnvalue))
  (UserInterface|Viewport|AddtoViewport _output_get 0))

(fn ConstructionScript)